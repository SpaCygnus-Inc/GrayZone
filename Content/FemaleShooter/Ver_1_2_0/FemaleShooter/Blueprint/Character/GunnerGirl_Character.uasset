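; Playable GunnerGirl character that maps keyboard, mouse and gamepad input to movement, camera and gun actions.
; GunnerGirlComponent performs the actions, while KeyPressHandler supplies continuous WASD events and CameraSwitcher cycles cameras.
; After a short delay, BeginPlay runs optional setup for those helpers and the demo UI behind hardcoded branches, then equips the gun.
; Component gun and strafe mode delegates drive indicators in the GunnerGirl_GameMode help UI.
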(event `Key|Gamepad_Special_Right`
  (params (Key :type "Key Structure"))
  ;[1 0.4538 0.404] Input - Toggle Demo UI
  (:`Pressed`
    (bind _asgunner_girl_game_mode (cast `/Game/FemaleShooter/Ver_1_2_0/FemaleShooter/Blueprint/GunnerGirl_GameMode` (`GameplayStatics.GetGameMode`) :!label _label))
    (`/Game/FemaleShooter/Ver_1_2_0/FemaleShooter/Blueprint/GunnerGirl_GameMode.Toggle_UI_Help` _asgunner_girl_game_mode)))

(event `self.ReceiveBeginPlay`
  ;[1 1 1] Event BeginPlay, Event Tick, and Basic Setup
  (`KismetSystemLibrary.Delay` 0.2)
  (`|ExecutionSequence`
    (:`then_0`
      (if true
        (`self.SetupInput_KeyPressHandler`)))
    (:`then_1`
      (if true
        (`self.SetupDemoUI`)))
    (:`then_2`
      (if true
        (`self.SetupCameraHandler`)))
    (:`then_3`
      (`/Game/FemaleShooter/Ver_1_2_0/FemaleShooter/Blueprint/Component/GunnerGirlComponent.EquipHolsterAndGun` (`self.GunnerGirlComponent`))
      (`/Game/FemaleShooter/Ver_1_2_0/FemaleShooter/Blueprint/Component/GunnerGirlComponent.EquipGun` (`self.GunnerGirlComponent`) true))))

(event `SetupDemoUI`
  ;[1 0.4538 0.404] Setup - Demo UI
  (`|ExecutionSequence`
    (:`then_0`
      (bind _asgunner_girl_game_mode (cast `/Game/FemaleShooter/Ver_1_2_0/FemaleShooter/Blueprint/GunnerGirl_GameMode` (`GameplayStatics.GetGameMode`)))
      (`/Game/FemaleShooter/Ver_1_2_0/FemaleShooter/Blueprint/GunnerGirl_GameMode.Setup_UI_Help` _asgunner_girl_game_mode))
    (:`then_1`
      (add `/Game/FemaleShooter/Ver_1_2_0/FemaleShooter/Blueprint/Component/GunnerGirlComponent.OnGunModeChanged` (`self.GunnerGirlComponent`) (delegate `OnGunModeChanged_Event_0`))
      (add `/Game/FemaleShooter/Ver_1_2_0/FemaleShooter/Blueprint/Component/GunnerGirlComponent.OnStrafeModeChanged` (`self.GunnerGirlComponent`) (delegate `OnStrafeModeChanged_Event_0`)))))

(event `Key|Enter`
  (params (Key :type "Key Structure"))
  ;[1 0.4538 0.404] Input - Toggle Demo UI
  (:`Pressed`
    (goto _label)))

(event `self.ReceiveTick`
  (params (DeltaSeconds :type "Float (single-precision)"))
  ;[1 1 1] Event BeginPlay, Event Tick, and Basic Setup
)

(event `OnStrafeModeChanged_Event_0`
  (params (IsActive :type Boolean))
  ;[1 0.4538 0.404] Setup - Demo UI
  (if IsActive
    (`self.Enable_StrafeMode_UI`)
    (else
      (`self.Disable_StrafeMode_UI`))))

(event `OnGunModeChanged_Event_0`
  (params (IsActive :type Boolean))
  ;[1 0.4538 0.404] Setup - Demo UI
  (if IsActive
    (`self.EnableGunModeIndicator`)
    (else
      (`self.DisableGunModeIndicator`))))

(event `EnableGunModeIndicator`
  ;[1 0.4538 0.404] Setup - Demo UI
  (bind _asgunner_girl_game_mode (cast `/Game/FemaleShooter/Ver_1_2_0/FemaleShooter/Blueprint/GunnerGirl_GameMode` (`GameplayStatics.GetGameMode`)))
  (`/Game/FemaleShooter/Ver_1_2_0/FemaleShooter/Blueprint/UI/UI_Help.GunModeEnabled` (`/Game/FemaleShooter/Ver_1_2_0/FemaleShooter/Blueprint/GunnerGirl_GameMode.UI_Help` _asgunner_girl_game_mode)))

(event `Enable_StrafeMode_UI`
  ;[1 0.4538 0.404] Setup - Demo UI
  (bind _asgunner_girl_game_mode (cast `/Game/FemaleShooter/Ver_1_2_0/FemaleShooter/Blueprint/GunnerGirl_GameMode` (`GameplayStatics.GetGameMode`)))
  (`/Game/FemaleShooter/Ver_1_2_0/FemaleShooter/Blueprint/UI/UI_Help.StrafeModeEnabled` (`/Game/FemaleShooter/Ver_1_2_0/FemaleShooter/Blueprint/GunnerGirl_GameMode.UI_Help` _asgunner_girl_game_mode)))

(event `Key|Escape`
  (params (Key :type "Key Structure"))
  ;[1 0.4538 0.404] Input - Quit Program
  (:`Pressed`
    (`KismetSystemLibrary.QuitGame` null "Quit" :!label _label_2)))

(event `Key|Gamepad_Special_Left`
  (params (Key :type "Key Structure"))
  ;[1 0.4538 0.404] Input - Quit Program
  (:`Pressed`
    (goto _label_2)))

(event `DisableGunModeIndicator`
  ;[1 0.4538 0.404] Setup - Demo UI
  (bind _asgunner_girl_game_mode (cast `/Game/FemaleShooter/Ver_1_2_0/FemaleShooter/Blueprint/GunnerGirl_GameMode` (`GameplayStatics.GetGameMode`)))
  (`/Game/FemaleShooter/Ver_1_2_0/FemaleShooter/Blueprint/UI/UI_Help.GunModeDisabled` (`/Game/FemaleShooter/Ver_1_2_0/FemaleShooter/Blueprint/GunnerGirl_GameMode.UI_Help` _asgunner_girl_game_mode)))

(event `Disable_StrafeMode_UI`
  ;[1 0.4538 0.404] Setup - Demo UI
  (bind _asgunner_girl_game_mode (cast `/Game/FemaleShooter/Ver_1_2_0/FemaleShooter/Blueprint/GunnerGirl_GameMode` (`GameplayStatics.GetGameMode`)))
  (`/Game/FemaleShooter/Ver_1_2_0/FemaleShooter/Blueprint/UI/UI_Help.StrafeModeDisabled` (`/Game/FemaleShooter/Ver_1_2_0/FemaleShooter/Blueprint/GunnerGirl_GameMode.UI_Help` _asgunner_girl_game_mode)))

(event `Key|Gamepad_RightThumbstick`
  (params (Key :type "Key Structure"))
  ;[1 0.72 0.3615] Input - Switch Camera
  (:`Pressed`
    (`/Game/FemaleShooter/Ver_1_2_0/FemaleShooter/Additional/CameraSwitcher/Blueprint/Component/CameraSwitcher.SwitchToNextCamera` (`self.CameraSwitcher`) "NewEnumerator2" 8.0 :!label _label_3)))

(event `SetupCameraHandler`
  ;[1 0.72 0.3615] Setup - Camera Handler
  (`/Game/FemaleShooter/Ver_1_2_0/FemaleShooter/Additional/CameraSwitcher/Blueprint/Component/CameraSwitcher.Setup` (`self.CameraSwitcher`) (`self.FollowCamera`)))

(event `Key|C`
  (params (Key :type "Key Structure"))
  ;[1 0.72 0.3615] Input - Switch Camera
  (:`Pressed`
    (goto _label_3)))

(event `Key|Gamepad_FaceButton_Top`
  (params (Key :type "Key Structure"))
  ;[0.3569 1 0.3843] Input - Strafe Mode
  (:`Pressed`
    (`/Game/FemaleShooter/Ver_1_2_0/FemaleShooter/Blueprint/Component/GunnerGirlComponent.ToggleStrafeMode` (`self.GunnerGirlComponent`) :!label _label_4)))

(event `InputAxisKey|Gamepad_RightX`
  (params (AxisValue :type "Float (single-precision)"))
  ;[0.3569 1 0.3843] Input - Camera Control
  (`/Game/FemaleShooter/Ver_1_2_0/FemaleShooter/Blueprint/Component/GunnerGirlComponent.Camera_TurnHorizontal` (`self.GunnerGirlComponent`) AxisValue 45.0 2.0 false))

(event `InputAxisKey|Gamepad_LeftY`
  (params (AxisValue :type "Float (single-precision)"))
  ;[0.3569 1 0.3843] Input - Movement (Gamepad)
  (`/Game/FemaleShooter/Ver_1_2_0/FemaleShooter/Blueprint/Component/GunnerGirlComponent.MoveForward` (`self.GunnerGirlComponent`) AxisValue))

(event `Key|LeftShift`
  (params (Key :type "Key Structure"))
  ;[0.3569 1 0.3843] Input - Walk
  (:`Pressed`
    (`/Game/FemaleShooter/Ver_1_2_0/FemaleShooter/Blueprint/Component/GunnerGirlComponent.Walk` (`self.GunnerGirlComponent`)))
  (:`Released`
    (`/Game/FemaleShooter/Ver_1_2_0/FemaleShooter/Blueprint/Component/GunnerGirlComponent.UnWalk` (`self.GunnerGirlComponent`))))

(event `Key|Gamepad_LeftTrigger`
  (params (Key :type "Key Structure"))
  ;[0.3569 1 0.3843] Input - Gun Equip + Unequip (Normal) (Gamepad)
  (:`Pressed`
    (`/Game/FemaleShooter/Ver_1_2_0/FemaleShooter/Blueprint/Component/GunnerGirlComponent.EquipGun` (`self.GunnerGirlComponent`) false))
  (:`Released`
    (`/Game/FemaleShooter/Ver_1_2_0/FemaleShooter/Blueprint/Component/GunnerGirlComponent.UnequipGun` (`self.GunnerGirlComponent`) false)))

(event `Key|Y`
  (params (Key :type "Key Structure"))
  ;[0.3569 1 0.3843] Input - Strafe Mode
  (:`Pressed`
    (goto _label_4)))

(event `InputAxisKey|Gamepad_LeftX`
  (params (AxisValue :type "Float (single-precision)"))
  ;[0.3569 1 0.3843] Input - Movement (Gamepad)
  (`/Game/FemaleShooter/Ver_1_2_0/FemaleShooter/Blueprint/Component/GunnerGirlComponent.MoveSideward` (`self.GunnerGirlComponent`) AxisValue))

(event `InputAxisKey|Gamepad_RightY`
  (params (AxisValue :type "Float (single-precision)"))
  ;[0.3569 1 0.3843] Input - Camera Control
  (`/Game/FemaleShooter/Ver_1_2_0/FemaleShooter/Blueprint/Component/GunnerGirlComponent.Camera_TurnVertical` (`self.GunnerGirlComponent`) AxisValue 45.0 2.0 true))

(event `InputAxisKey|MouseX`
  (params (AxisValue :type "Float (single-precision)"))
  ;[0.3569 1 0.3843] Input - Camera Control
  (`/Game/FemaleShooter/Ver_1_2_0/FemaleShooter/Blueprint/Component/GunnerGirlComponent.Camera_TurnHorizontal` (`self.GunnerGirlComponent`) AxisValue 45.0 1.5 false))

(event `Key|Gamepad_RightShoulder`
  (params (Key :type "Key Structure"))
  ;[0.3569 1 0.3843] Input - Crouch
  (:`Pressed`
    (`/Game/FemaleShooter/Ver_1_2_0/FemaleShooter/Blueprint/Component/GunnerGirlComponent.Crouch` (`self.GunnerGirlComponent`) :!label _label_5))
  (:`Released`
    (`/Game/FemaleShooter/Ver_1_2_0/FemaleShooter/Blueprint/Component/GunnerGirlComponent.UnCrouch` (`self.GunnerGirlComponent`) :!label _label_6)))

(event `Key|Gamepad_DPad_Up`
  (params (Key :type "Key Structure"))
  ;[0.3569 1 0.3843] Input - Gun Equip + Unequip (Gunspinning) (Gamepad)
  (:`Pressed`
    (`/Game/FemaleShooter/Ver_1_2_0/FemaleShooter/Blueprint/Component/GunnerGirlComponent.EquipGun` (`self.GunnerGirlComponent`) true)))

(event `Key|LeftAlt`
  (params (Key :type "Key Structure"))
  ;[0.3569 1 0.3843] Input - Crouch
  (:`Pressed`
    (goto _label_5))
  (:`Released`
    (goto _label_6)))

(event `SetupInput_KeyPressHandler`
  ;[0.3569 1 0.3843] Input - Movement (Keyboard)
  (`/Game/FemaleShooter/Ver_1_2_0/FemaleShooter/Blueprint/Component/KeyPressHandler.Setup` (`self.KeyPressHandler`) (`|MakeMap` "W" "W" "S" "S" "D" "D" "A" "A" :!type "Key Structure" :!valuetype "Name"))
  (add `/Game/FemaleShooter/Ver_1_2_0/FemaleShooter/Blueprint/Component/KeyPressHandler.OnKeyDown` (`self.KeyPressHandler`) (delegate `OnKeyDown`)))

(event `Key|Gamepad_DPad_Down`
  (params (Key :type "Key Structure"))
  ;[0.3569 1 0.3843] Input - Gun Equip + Unequip (Gunspinning) (Gamepad)
  (:`Pressed`
    (`/Game/FemaleShooter/Ver_1_2_0/FemaleShooter/Blueprint/Component/GunnerGirlComponent.UnequipGun` (`self.GunnerGirlComponent`) true)))

(event `Key|LeftControl`
  (params (Key :type "Key Structure"))
  ;[0.3569 1 0.3843] Input - Crouch
  (:`Pressed`
    (goto _label_5))
  (:`Released`
    (goto _label_6)))

(event `InputAxisKey|MouseY`
  (params (AxisValue :type "Float (single-precision)"))
  ;[0.3569 1 0.3843] Input - Camera Control
  (`/Game/FemaleShooter/Ver_1_2_0/FemaleShooter/Blueprint/Component/GunnerGirlComponent.Camera_TurnVertical` (`self.GunnerGirlComponent`) AxisValue 45.0 2.0 true))

(event `Key|One`
  (params (Key :type "Key Structure"))
  ;[0.3569 1 0.3843] Gun Equip / Unequip (Keyboard)
  (:`Pressed`
    (`/Game/FemaleShooter/Ver_1_2_0/FemaleShooter/Blueprint/Component/GunnerGirlComponent.ToggleEquipGun` (`self.GunnerGirlComponent`) false)))

(event `Key|Gamepad_FaceButton_Right`
  (params (Key :type "Key Structure"))
  ;[0.3569 1 0.3843] Input - Roll
  (:`Pressed`
    (`/Game/FemaleShooter/Ver_1_2_0/FemaleShooter/Blueprint/Component/GunnerGirlComponent.Roll` (`self.GunnerGirlComponent`) :!label _label_7)))

(event `Key|E`
  (params (Key :type "Key Structure"))
  ;[0.3569 1 0.3843] Input - Roll
  (:`Pressed`
    (goto _label_7)))

(event `Key|Two`
  (params (Key :type "Key Structure"))
  ;[0.3569 1 0.3843] Gun Equip / Unequip (Keyboard)
  (:`Pressed`
    (`/Game/FemaleShooter/Ver_1_2_0/FemaleShooter/Blueprint/Component/GunnerGirlComponent.ToggleEquipGun` (`self.GunnerGirlComponent`) true)))

(event `OnKeyDown`
  (params (Key :type "Key Structure") (KeyName :type Name))
  ;[0.3569 1 0.3843] Input - Movement (Keyboard)
  (switch `name` KeyName
    (:`W`
      (`/Game/FemaleShooter/Ver_1_2_0/FemaleShooter/Blueprint/Component/GunnerGirlComponent.MoveForward` (`self.GunnerGirlComponent`) 1.0))
    (:`S`
      (`/Game/FemaleShooter/Ver_1_2_0/FemaleShooter/Blueprint/Component/GunnerGirlComponent.MoveForward` (`self.GunnerGirlComponent`) -1.0))
    (:`A`
      (`/Game/FemaleShooter/Ver_1_2_0/FemaleShooter/Blueprint/Component/GunnerGirlComponent.MoveSideward` (`self.GunnerGirlComponent`) -1.0))
    (:`D`
      (`/Game/FemaleShooter/Ver_1_2_0/FemaleShooter/Blueprint/Component/GunnerGirlComponent.MoveSideward` (`self.GunnerGirlComponent`) 1.0))))

(event `Key|SpaceBar`
  (params (Key :type "Key Structure"))
  ;[0.3569 1 0.3843] Input - Jump/Double Jump/Somersault
  (:`Pressed`
    (`/Game/FemaleShooter/Ver_1_2_0/FemaleShooter/Blueprint/Component/GunnerGirlComponent.TriggerJump` (`self.GunnerGirlComponent`) true :!label _label_8))
  (:`Released`
    (`/Game/FemaleShooter/Ver_1_2_0/FemaleShooter/Blueprint/Component/GunnerGirlComponent.ClearJump` (`self.GunnerGirlComponent`) :!label _label_9)))

(event `Key|Gamepad_RightTrigger`
  (params (Key :type "Key Structure"))
  ;[0.3569 1 0.3843] Input - Shoot
  (:`Pressed`
    (`/Game/FemaleShooter/Ver_1_2_0/FemaleShooter/Blueprint/Component/GunnerGirlComponent.Shoot` (`self.GunnerGirlComponent`) :!label _label_10))
  (:`Released`
    (`/Game/FemaleShooter/Ver_1_2_0/FemaleShooter/Blueprint/Component/GunnerGirlComponent.UnShoot` (`self.GunnerGirlComponent`) :!label _label_11)))

(event `Key|LeftMouseButton`
  (params (Key :type "Key Structure"))
  ;[0.3569 1 0.3843] Input - Shoot
  (:`Pressed`
    (goto _label_10))
  (:`Released`
    (goto _label_11)))

(event `Key|Gamepad_FaceButton_Bottom`
  (params (Key :type "Key Structure"))
  ;[0.3569 1 0.3843] Input - Jump/Double Jump/Somersault
  (:`Pressed`
    (goto _label_8))
  (:`Released`
    (goto _label_9)))

(fn `UserConstructionScript`)