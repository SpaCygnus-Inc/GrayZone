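; Component for the GunnerGirl character that manages attached equipment actors in a name-keyed map.
; Spawning destroys any existing item under that name, then attaches the new actor to a mesh socket with its primitive collision disabled.
; Items can be re-attached, destroyed, retrieved (optionally as an I_Handgun_Actor) or replaced in place.
; Replacement reuses the old actor's transform and parent, treating the equipment name as the socket name.
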(fn `AttachEquipmentToSocket`
  (params (EquipmentName :type Name) (MeshComponent :type "SkeletalMeshComponent Object Reference") (MeshSocketName :type Name))
  (bind (_value _returnvalue) (`BlueprintMapLibrary.Map_Find` (`self.EquipmentList`) EquipmentName))
  (if _returnvalue
    (`SceneComponent.K2_AttachToComponent` (`Actor.RootComponent` _value) MeshComponent MeshSocketName "KeepRelative" "KeepRelative" "KeepRelative" true)))

(fn `DestroyEquipment`
  (params (EquipmentName :type Name))
  (locals (TempEquipment :type "Actor Object Reference"))
  (bind (_value _returnvalue) (`BlueprintMapLibrary.Map_Find` (`self.EquipmentList`) EquipmentName))
  (if _returnvalue
    (bind _output_get (set `local.TempEquipment` _value))
    (`BlueprintMapLibrary.Map_Remove` (`self.EquipmentList`) EquipmentName)
    (`SceneComponent.K2_DetachFromComponent` (`Actor.RootComponent` _output_get) "KeepRelative" "KeepRelative" "KeepRelative" true)
    (`Actor.K2_DestroyActor` _output_get)))

(fn `ReplaceEquipment`
  (params (EquipmentName :type Name) (NewEquipmentClass :type "Actor Class Reference"))
  (returns (IsSuccessful :type Boolean))
  (locals (PreviousEquipment :type "Actor Object Reference"))
  (bind (_value _returnvalue) (`BlueprintMapLibrary.Map_Find` (`self.EquipmentList`) EquipmentName))
  (if _returnvalue
    (`|ExecutionSequence`
      (:`then_0`
        (set `local.PreviousEquipment` _value))
      (:`then_1`
        (bind _returnvalue_2 (`|SpawnActorFromClass` (`local.NewEquipmentClass`) (`Actor.GetTransform` (`local.PreviousEquipment`)) "AlwaysSpawn" "OverrideRootScale" null null))
        (`BlueprintMapLibrary.Map_Add` (`self.EquipmentList`) (`local.EquipmentName`) _returnvalue_2)
        (`PrimitiveComponent.SetCollisionEnabled` (`Actor.GetComponentByClass` _returnvalue_2 "/Script/Engine.PrimitiveComponent") "NoCollision")
        (`SceneComponent.K2_AttachToComponent` (`Actor.RootComponent` _returnvalue_2) (`SceneComponent.GetAttachParent` (`Actor.RootComponent` (`local.PreviousEquipment`))) (`local.EquipmentName`) "KeepWorld" "KeepWorld" "KeepWorld" true))
      (:`then_2`
        (`SceneComponent.K2_DetachFromComponent` (`Actor.RootComponent` (`local.PreviousEquipment`)) "KeepRelative" "KeepRelative" "KeepRelative" true)
        (`Actor.K2_DestroyActor` (`local.PreviousEquipment`)))
      (:`then_3`
        (return true)))
    (else
      (return false))))

(fn `RetrieveEquipment`
  (params (EquipmentName :type Name))
  (returns (Actor :type "Actor Object Reference"))
  (return (`BlueprintMapLibrary.Map_Find` (`self.EquipmentList`) EquipmentName)))

(fn `RetrieveHandgun`
  (params (EquipmentName :type Name))
  (returns (IsFound :type Boolean) (Actor :type "/Game/FemaleShooter/Ver_1_2_0/FemaleShooter/Blueprint/Interface/I_Handgun_Actor Interface"))
  (bind _asi_handgun_actor (cast `/Game/FemaleShooter/Ver_1_2_0/FemaleShooter/Blueprint/Interface/I_Handgun_Actor` (`BlueprintMapLibrary.Map_Find` (`self.EquipmentList`) EquipmentName))
    (:`then`
      (return true _asi_handgun_actor))
    (:`CastFailed`
      (return false null))))

(fn `SpawnEquipmentToSocket`
  (params (EquipmentName :type Name) (EquipmentClass :type "Actor Class Reference") (MeshComponent :type "SkeletalMeshComponent Object Reference") (MeshSocketName :type Name))
  (if (`KismetSystemLibrary.IsValidClass` EquipmentClass)
    (`self.DestroyEquipment` EquipmentName)
    (bind _returnvalue (`|SpawnActorFromClass` EquipmentClass (`KismetMathLibrary.MakeTransform` (0.0 0.0 0.0)) "AlwaysSpawn" "OverrideRootScale" null null))
    (`BlueprintMapLibrary.Map_Add` (`self.EquipmentList`) EquipmentName _returnvalue)
    (`PrimitiveComponent.SetCollisionEnabled` (`Actor.GetComponentByClass` _returnvalue "/Script/Engine.PrimitiveComponent") "NoCollision")
    (`SceneComponent.K2_AttachToComponent` (`Actor.RootComponent` _returnvalue) (`local.MeshComponent`) MeshSocketName "KeepRelative" "KeepRelative" "KeepRelative" true)))