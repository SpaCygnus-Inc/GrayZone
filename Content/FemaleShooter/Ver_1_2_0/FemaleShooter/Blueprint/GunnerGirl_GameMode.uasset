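; Game mode for the GunnerGirl female shooter that owns the on-screen help widget.
; Setup_UI_Help creates a UI_Help widget, stores it and adds it to the viewport, only if no valid instance exists yet.
; Toggle_UI_Help forwards to that widget's ToggleUI when it is valid.
; BeginPlay and Tick are empty, and nothing in this file calls either custom event.
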(event `self.ReceiveBeginPlay`)

(event `Setup_UI_Help`
  (`/Engine/EditorBlueprintResources/StandardMacros.IsValid` (`self.UI_Help`)
    (:`Is Not Valid`
      (bind _returnvalue (`|CreateWidget` "/Game/FemaleShooter/Ver_1_2_0/FemaleShooter/Blueprint/UI/UI_Help.UI_Help_C"))
      (set `self.UI_Help` _returnvalue)
      (`UserWidget.AddToViewport` (`self.UI_Help`) 0))))

(event `Toggle_UI_Help`
  (`/Engine/EditorBlueprintResources/StandardMacros.IsValid` (`self.UI_Help`)
    (:`Is Valid`
      (`/Game/FemaleShooter/Ver_1_2_0/FemaleShooter/Blueprint/UI/UI_Help.ToggleUI` (`self.UI_Help`)))))

(fn `UserConstructionScript`)