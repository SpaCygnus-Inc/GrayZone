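; GunnerGirlNotify is an animation notify that passes a message from an animation to the female shooter's GunnerGirlComponent.
; When it fires, it looks up that component on the mesh's owner and, if valid, calls GunnerGirlNotifyEvent with its Message, returning whether the component was found.
; The notify's display name is the Message converted to a string.
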(fn `GetNotifyName`
  (returns (ReturnValue :type String))
  (return (`KismetStringLibrary.Conv_NameToString` (`self.Message`))))

(fn `Received_Notify`
  (params (MeshComp :type "SkeletalMeshComponent Object Reference") (Animation :type "AnimSequenceBase Object Reference"))
  (returns (ReturnValue :type Boolean))
  (bind _returnvalue (`Actor.GetComponentByClass` (`ActorComponent.GetOwner` MeshComp) "/Game/FemaleShooter/Blueprint/Component/GunnerGirlComponent.GunnerGirlComponent_C"))
  (`/Engine/EditorBlueprintResources/StandardMacros.IsValid` _returnvalue
    (:`Is Valid`
      (`/Game/FemaleShooter/Blueprint/Component/GunnerGirlComponent.GunnerGirlNotifyEvent` _returnvalue (`self.Message`))
      (return true))
    (:`Is Not Valid`
      (return false))))