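; Playable gunner girl character Blueprint that maps keyboard, mouse and gamepad input to movement, camera and twin-gun actions.
; Work is delegated to components: GunnerGirlComponent for locomotion and flashlight, TwinGunHandler for weapons and shooting, CameraSwitcher for view and aim.
; After a short BeginPlay delay it sets these up and binds ItemCollector, whose found items dispatch by type to ammo, triggers, pickups, weapon swaps or shooting-pattern changes.
; Debug keys swap the skeletal mesh or quit.
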(event `self.ReceiveBeginPlay`
  ;[1 1 1] Event BeginPlay, Event Tick, and Basic Setup
  (`KismetSystemLibrary.Delay` 0.5) ; Delay required to ensure all the actors and components are initialized
  (`|ExecutionSequence`
    (:`then_0`
      (`/Game/FemaleShooter/Blueprint/Misc/ZenLib.SetupComponents` self))
    (:`then_1`
      (`self.SetupCameraHandler`)
      (`self.SetupItemCollector`))))

(event `Key|Three`
  (params (Key :type "Key Structure"))
  ;[1 1 1] Switch mesh during gameplay
  (:`Pressed`
    (`SkinnedMeshComponent.SetSkinnedAssetAndUpdate` (`self.Mesh`) "/Game/FemaleShooter/Asset/GunnerGirl/Mesh/SK_GunnerGirl.SK_GunnerGirl" true)))

(event `Key|Escape`
  (params (Key :type "Key Structure"))
  (bind _returnvalue (`self.GetComponentByClass` "/Game/FemaleShooter/Blueprint/Component/UIController.UIController_C"))
  ;[1 0.4538 0.404] Input - Quit Program
  (:`Pressed`
    (`/Engine/EditorBlueprintResources/StandardMacros.IsValid` _returnvalue :!label _label
      (:`Is Valid`
        (if (not (`/Game/FemaleShooter/Blueprint/Component/UIController.IsUIActive` _returnvalue))
          (`KismetSystemLibrary.QuitGame` null "Quit" :!label _label_2)))
      (:`Is Not Valid`
        (goto _label_2)))))

(event `Key|Gamepad_Special_Left`
  (params (Key :type "Key Structure"))
  ;[1 0.4538 0.404] Input - Quit Program
  (:`Pressed`
    (goto _label)))

(event `self.ReceiveTick`
  (params (DeltaSeconds :type "Float (single-precision)"))
  ;[1 1 1] Event BeginPlay, Event Tick, and Basic Setup
)

(event `Key|Four`
  (params (Key :type "Key Structure"))
  ;[1 1 1] Switch mesh during gameplay
  (:`Pressed`
    (`SkinnedMeshComponent.SetSkinnedAssetAndUpdate` (`self.Mesh`) "/Game/FemaleShooter/Asset/GunnerGirl/Mesh/SK_Mannequin.SK_Mannequin" true)))

(event `Key|Five`
  (params (Key :type "Key Structure"))
  ;[1 1 1] Switch mesh during gameplay
  (:`Pressed`
    (`SkinnedMeshComponent.SetSkinnedAssetAndUpdate` (`self.Mesh`) "/Game/FemaleShooter/Asset/GunnerGirl/Mesh/SK_Mannequin_Female.SK_Mannequin_Female" true)))

(event `Key|Gamepad_RightThumbstick`
  (params (Key :type "Key Structure"))
  ;[1 0.72 0.3615] Input - Switch Camera
  (:`Pressed`
    (`/Game/FemaleShooter/Blueprint/Component/CameraSwitcher.SwitchToNextCamera` (`self.CameraSwitcher`) "NewEnumerator2" 16.0 :!label _label_3)))

(event `SetupCameraHandler`
  (bind _cameraswitcher (`self.CameraSwitcher`))
  ;[1 0.7231 0.3613] Setup - Camera Handler
  (`/Game/FemaleShooter/Blueprint/Component/CameraSwitcher.Setup` _cameraswitcher (`self.FollowCamera`))
  (`/Game/FemaleShooter/Blueprint/Component/CameraSwitcher.RegisterAimCamera` _cameraswitcher (`|MakeArray` (`self.GunCamera`))))

(event `Key|RightMouseButton`
  (params (Key :type "Key Structure"))
  ;[1 0.7231 0.3613] Input - Aim (Keyboard)
  (:`Pressed`
    (`/Game/FemaleShooter/Blueprint/Component/CameraSwitcher.StartAim` (`self.CameraSwitcher`)))
  (:`Released`
    (`/Game/FemaleShooter/Blueprint/Component/CameraSwitcher.StopAim` (`self.CameraSwitcher`))))

(event `Key|V`
  (params (Key :type "Key Structure"))
  ;[1 0.72 0.3615] Input - Switch Camera
  (:`Pressed`
    (goto _label_3)))

(event `InputAxisKey|Gamepad_LeftTriggerAxis`
  (params (AxisValue :type "Float (single-precision)"))
  ;[1 0.7231 0.3613] Input - Aim (Gamepad)
  (`/Game/FemaleShooter/Blueprint/Component/CameraSwitcher.DynamicAim` (`self.CameraSwitcher`) AxisValue))

(event `Key|Gamepad_FaceButton_Top`
  (params (Key :type "Key Structure"))
  ;[0 0.6445 1] Input - Examine/Interact
  (:`Pressed`
    (`/Game/FemaleShooter/Blueprint/Component/ItemCollector.FindSimpleItem` (`self.ItemCollector`) :!label _label_4)))

(event `Key|Gamepad_LeftThumbstick`
  (params (Key :type "Key Structure"))
  ;[0.3569 1 0.3843] Input - Strafe Mode
  (:`Pressed`
    (`/Game/FemaleShooter/Blueprint/Component/GunnerGirlComponent.ToggleStrafeMode` (`self.GunnerGirlComponent`) :!label _label_5)))

(event `Key|Gamepad_DPad_Left`
  (params (Key :type "Key Structure"))
  ;[0.8714 0.2016 1] Input - Left Gun Shot Only
  (:`Pressed`
    (`/Game/FemaleShooter/Blueprint/Component/TwinGunHandler.LeftGunShotOnly` (`self.TwinGunHandler`) true :!label _label_6))
  (:`Released`
    (`/Game/FemaleShooter/Blueprint/Component/TwinGunHandler.LeftGunShotOnly` (`self.TwinGunHandler`) false :!label _label_7)))

(event `InputAxisKey|Gamepad_LeftY`
  (params (AxisValue :type "Float (single-precision)"))
  ;[0.3569 1 0.3843] Input - Movement (Gamepad)
  (`/Game/FemaleShooter/Blueprint/Component/GunnerGirlComponent.MoveForward` (`self.GunnerGirlComponent`) AxisValue))

(event `Key|Gamepad_LeftShoulder`
  (params (Key :type "Key Structure"))
  ;[0.8714 0.2016 1] Input - Gun Equip + Unequip (Normal) (Gamepad)
  (:`Pressed`
    (`/Game/FemaleShooter/Blueprint/Component/TwinGunHandler.ToggleEquipGun` (`self.TwinGunHandler`) false)))

(event `SetupItemCollector`
  ;[0 0.6445 1] Item Collector
  (add `/Game/FemaleShooter/Blueprint/Component/ItemCollector.OnSimpleItemFound` (`self.ItemCollector`) (delegate `OnSimpleItemFound_Event_0`)))

(event `InputAxisKey|Gamepad_RightX`
  (params (AxisValue :type "Float (single-precision)"))
  ;[0.3569 1 0.3843] Input - Camera Control (Gamepad)
  (`/Game/FemaleShooter/Blueprint/Component/GunnerGirlComponent.GamepadTurnHorizontal` (`self.GunnerGirlComponent`) AxisValue))

(event `Key|F`
  (params (Key :type "Key Structure"))
  ;[0 0.6445 1] Input - Examine/Interact
  (:`Pressed`
    (goto _label_4)))

(event `Key|Y`
  (params (Key :type "Key Structure"))
  ;[0.3569 1 0.3843] Input - Strafe Mode
  (:`Pressed`
    (goto _label_5)))

(event `Key|Z`
  (params (Key :type "Key Structure"))
  ;[0.8714 0.2016 1] Input - Left Gun Shot Only
  (:`Pressed`
    (goto _label_6))
  (:`Released`
    (goto _label_7)))

(event `Key|LeftShift`
  (params (Key :type "Key Structure"))
  ;[0.3569 1 0.3843] Input - Walk
  ; Requires GunnerGirlComponent MoveForward/MoveSideward
  (:`Pressed`
    (`/Game/FemaleShooter/Blueprint/Component/GunnerGirlComponent.Walk` (`self.GunnerGirlComponent`)))
  (:`Released`
    (`/Game/FemaleShooter/Blueprint/Component/GunnerGirlComponent.UnWalk` (`self.GunnerGirlComponent`))))

(event `OnSimpleItemFound_Event_0`
  (params (SimpleItem :type "/Game/FemaleShooter/Additional/SimpleItem/SimpleItem Object Reference") (ItemType :type Name))
  ;[0 0.6445 1] Item Collector
  (switch `name` ItemType
    (:`Ammo`
      (`self.ExamineAmmo` SimpleItem))
    (:`Trigger`
      (`self.ExamineTrigger` SimpleItem))
    (:`Flashlight`
      (`self.PickupFlashlight` SimpleItem))
    (:`WeaponSet`
      (`self.LoadNewWeaponSet` SimpleItem))
    (:`ShootingPatternChange`
      (`self.ChangeShootingPattern`))
    (:`Left Weapon Swap`
      (`self.LeftWeaponSwapActor` SimpleItem))
    (:`WeaponPickup`
      (`self.PickupWeaponSet` SimpleItem))
    (:`ReassembleCans`
      (`/Game/FemaleShooter/Additional/SimpleItem/SimpleItem.Trigger` SimpleItem :!label _label_8))
    (:`ToggleShootingRange`
      (goto _label_8))))

(event `InputAxisKey|Gamepad_LeftX`
  (params (AxisValue :type "Float (single-precision)"))
  ;[0.3569 1 0.3843] Input - Movement (Gamepad)
  (`/Game/FemaleShooter/Blueprint/Component/GunnerGirlComponent.MoveSideward` (`self.GunnerGirlComponent`) AxisValue))

(event `InputAxisKey|Gamepad_RightY`
  (params (AxisValue :type "Float (single-precision)"))
  ;[0.3569 1 0.3843] Input - Camera Control (Gamepad)
  (`/Game/FemaleShooter/Blueprint/Component/GunnerGirlComponent.GamepadTurnVertical` (`self.GunnerGirlComponent`) AxisValue))

(event `Key|Gamepad_RightShoulder`
  (params (Key :type "Key Structure"))
  ;[0.3569 1 0.3843] Input - Crouch
  (:`Pressed`
    (`/Game/FemaleShooter/Blueprint/Component/GunnerGirlComponent.Crouch` (`self.GunnerGirlComponent`) :!label _label_9))
  (:`Released`
    (`/Game/FemaleShooter/Blueprint/Component/GunnerGirlComponent.UnCrouch` (`self.GunnerGirlComponent`) :!label _label_10)))

(event `ExamineAmmo`
  (params (Item :type "/Game/FemaleShooter/Additional/SimpleItem/SimpleItem Object Reference"))
  ;[0 0.6445 1] Item Collector
  (bind _asammo_data (cast `/Game/FemaleShooter/Blueprint/Data/Ammo/AmmoData` (`/Game/FemaleShooter/Additional/SimpleItem/SimpleItem.ItemData` Item)))
  (`/Game/FemaleShooter/Blueprint/Component/TwinGunHandler.AssignAmmo` (`self.TwinGunHandler`) _asammo_data))

(event `Key|Gamepad_DPad_Up`
  (params (Key :type "Key Structure"))
  ;[0.8714 0.2016 1] Input - Gun Equip + Unequip (Gunspinning) (Gamepad)
  (:`Pressed`
    (`/Game/FemaleShooter/Blueprint/Component/TwinGunHandler.ToggleEquipGun` (`self.TwinGunHandler`) true)))

(event `Key|Gamepad_DPad_Right`
  (params (Key :type "Key Structure"))
  ;[0.8745 0.2 1] Input - Right Gun Shot Only
  (:`Pressed`
    (`/Game/FemaleShooter/Blueprint/Component/TwinGunHandler.RightGunShotOnly` (`self.TwinGunHandler`) true :!label _label_11))
  (:`Released`
    (`/Game/FemaleShooter/Blueprint/Component/TwinGunHandler.RightGunShotOnly` (`self.TwinGunHandler`) false :!label _label_12)))

(event `Key|LeftAlt`
  (params (Key :type "Key Structure"))
  ;[0.3569 1 0.3843] Input - Crouch
  (:`Pressed`
    (goto _label_9))
  (:`Released`
    (goto _label_10)))

(event `InputAxisKey|MouseX`
  (params (AxisValue :type "Float (single-precision)"))
  ;[0.3569 1 0.3843] Input - Camera Control (Mouse)
  (`/Game/FemaleShooter/Blueprint/Component/GunnerGirlComponent.MouseTurnHorizontal` (`self.GunnerGirlComponent`) AxisValue))

(event `self.KeyPressHandler.OnKeyboardMoveForward`
  (params (AxisValue :type "Float (single-precision)"))
  ;[0.3569 1 0.3843] Input - Movement (Keyboard)
  ; If using UE Third Person Template,
  ; these events can be replaced with InputAxis MoveForward and MoveRight
  (`/Game/FemaleShooter/Blueprint/Component/GunnerGirlComponent.MoveForward` (`self.GunnerGirlComponent`) AxisValue))

(event `Key|C`
  (params (Key :type "Key Structure"))
  ;[0.8745 0.2 1] Input - Right Gun Shot Only
  (:`Pressed`
    (goto _label_11))
  (:`Released`
    (goto _label_12)))

(event `Key|LeftControl`
  (params (Key :type "Key Structure"))
  ;[0.3569 1 0.3843] Input - Crouch
  (:`Pressed`
    (goto _label_9))
  (:`Released`
    (goto _label_10)))

(event `ExamineTrigger`
  (params (Item :type "/Game/FemaleShooter/Additional/SimpleItem/SimpleItem Object Reference"))
  (bind _itemtrigger (`/Game/FemaleShooter/Additional/SimpleItem/SimpleItem.ItemTrigger` Item))
  ;[0 0.6445 1] Item Collector
  (`/Engine/EditorBlueprintResources/StandardMacros.IsValid` _itemtrigger
    (:`Is Valid`
      (`/Game/FemaleShooter/Additional/SimpleItem/ItemTrigger.PressTrigger` _itemtrigger))))

(event `InputAxisKey|MouseY`
  (params (AxisValue :type "Float (single-precision)"))
  ;[0.3569 1 0.3843] Input - Camera Control (Mouse)
  (`/Game/FemaleShooter/Blueprint/Component/GunnerGirlComponent.MouseTurnVertical` (`self.GunnerGirlComponent`) AxisValue))

(event `self.KeyPressHandler.OnKeyboardMoveRight`
  (params (AxisValue :type "Float (single-precision)"))
  ;[0.3569 1 0.3843] Input - Movement (Keyboard)
  ; If using UE Third Person Template,
  ; these events can be replaced with InputAxis MoveForward and MoveRight
  (`/Game/FemaleShooter/Blueprint/Component/GunnerGirlComponent.MoveSideward` (`self.GunnerGirlComponent`) AxisValue))

(event `PickupFlashlight`
  (params (Item :type "/Game/FemaleShooter/Additional/SimpleItem/SimpleItem Object Reference"))
  ;[0 0.6445 1] Item Collector
  (`/Game/FemaleShooter/Blueprint/Component/GunnerGirlComponent.EquipFlashlight` (`self.GunnerGirlComponent`) true))

(event `Key|Gamepad_FaceButton_Right`
  (params (Key :type "Key Structure"))
  ;[0.3569 1 0.3843] Input - Roll
  (:`Pressed`
    (`/Game/FemaleShooter/Blueprint/Component/GunnerGirlComponent.Roll` (`self.GunnerGirlComponent`) :!label _label_13)))

(event `Key|One`
  (params (Key :type "Key Structure"))
  ;[0.8714 0.2016 1] Gun Equip / Unequip (Keyboard)
  (:`Pressed`
    (`/Game/FemaleShooter/Blueprint/Component/TwinGunHandler.ToggleEquipGun` (`self.TwinGunHandler`) false)))

(event `Key|E`
  (params (Key :type "Key Structure"))
  ;[0.3569 1 0.3843] Input - Roll
  (:`Pressed`
    (goto _label_13)))

(event `Key|Gamepad_FaceButton_Left`
  (params (Key :type "Key Structure"))
  ;[0.8745 0.2 1] Switch to next weapon
  ; (if there are more than 1 weapon equipped)
  (:`Pressed`
    (`/Game/FemaleShooter/Blueprint/Component/TwinGunHandler.SwitchToNextWeapon` (`self.TwinGunHandler`) :!label _label_14)))

(event `Key|Two`
  (params (Key :type "Key Structure"))
  ;[0.8714 0.2016 1] Gun Equip / Unequip (Keyboard)
  (:`Pressed`
    (`/Game/FemaleShooter/Blueprint/Component/TwinGunHandler.ToggleEquipGun` (`self.TwinGunHandler`) true)))

(event `LoadNewWeaponSet`
  (params (Item :type "/Game/FemaleShooter/Additional/SimpleItem/SimpleItem Object Reference"))
  ;[0 0.6445 1] Item Collector
  (bind _asequipment_set (cast `/Game/FemaleShooter/Blueprint/Data/Equipment/EquipmentSet` (`/Game/FemaleShooter/Additional/SimpleItem/SimpleItem.ItemData` Item))
    (:`then`
      (`/Game/FemaleShooter/Blueprint/Component/TwinGunHandler.LoadEquipmentSet` (`self.TwinGunHandler`) _asequipment_set))
    (:`CastFailed`
      (`/Game/FemaleShooter/Blueprint/Component/TwinGunHandler.ClearAllEquipment` (`self.TwinGunHandler`)))))

(event `Key|R`
  (params (Key :type "Key Structure"))
  ;[0.8745 0.2 1] Switch to next weapon
  ; (if there are more than 1 weapon equipped)
  (:`Pressed`
    (goto _label_14)))

(event `ChangeShootingPattern`
  (bind _array (`|MakeArray` "/Game/FemaleShooter/Blueprint/Data/ShootingPattern/Shooting_Frantic.Shooting_Frantic" "/Game/FemaleShooter/Blueprint/Data/ShootingPattern/Shooting_OneTwo.Shooting_OneTwo" "/Game/FemaleShooter/Blueprint/Data/ShootingPattern/Shooting_OneTwoThree.Shooting_OneTwoThree" "/Game/FemaleShooter/Blueprint/Data/ShootingPattern/Shooting_SevenShots.Shooting_SevenShots" :!type "/Game/FemaleShooter/Blueprint/Data/ShootingPattern/ShootingPattern Object Reference"))
  ;[0 0.6445 1] Item Collector
  (bind _output_get (set `self.ShootingPatternCount` (mod (+ (`self.ShootingPatternCount`) 1) (`KismetArrayLibrary.Array_Length` _array))))
  (`/Game/FemaleShooter/Blueprint/Component/TwinGunHandler.AssignShootingPattern` (`self.TwinGunHandler`) (`|GetArrayItem` _array _output_get)))

(event `Key|Gamepad_RightTrigger`
  (params (Key :type "Key Structure"))
  ;[0.8714 0.2016 1] Input - Shoot
  (:`Pressed`
    (`/Game/FemaleShooter/Blueprint/Component/TwinGunHandler.StartShooting` (`self.TwinGunHandler`) :!label _label_15))
  (:`Released`
    (`/Game/FemaleShooter/Blueprint/Component/TwinGunHandler.StopShooting` (`self.TwinGunHandler`) :!label _label_16)))

(event `Key|SpaceBar`
  (params (Key :type "Key Structure"))
  ;[0.3564 1 0.3864] Input - Jump/Double Jump/Somersault
  (:`Pressed`
    (`/Game/FemaleShooter/Blueprint/Component/GunnerGirlComponent.TriggerJump` (`self.GunnerGirlComponent`) true :!label _label_17))
  (:`Released`
    (`/Game/FemaleShooter/Blueprint/Component/GunnerGirlComponent.ClearJump` (`self.GunnerGirlComponent`) :!label _label_18)))

(event `Key|LeftMouseButton`
  (params (Key :type "Key Structure"))
  ;[0.8714 0.2016 1] Input - Shoot
  (:`Pressed`
    (goto _label_15))
  (:`Released`
    (goto _label_16)))

(event `Key|Gamepad_FaceButton_Bottom`
  (params (Key :type "Key Structure"))
  ;[0.3564 1 0.3864] Input - Jump/Double Jump/Somersault
  (:`Pressed`
    (goto _label_17))
  (:`Released`
    (goto _label_18)))

(event `PickupWeaponSet`
  (params (Item :type "/Game/FemaleShooter/Additional/SimpleItem/SimpleItem Object Reference"))
  ;[0 0.6445 1] Item Collector
  (bind _asequipment_set (cast `/Game/FemaleShooter/Blueprint/Data/Equipment/EquipmentSet` (`/Game/FemaleShooter/Additional/SimpleItem/SimpleItem.ItemData` Item)))
  (`/Game/FemaleShooter/Blueprint/Component/TwinGunHandler.PickupEquipmentSet` (`self.TwinGunHandler`) _asequipment_set))

(event `Key|Gamepad_DPad_Down`
  (params (Key :type "Key Structure"))
  ;[0.3564 1 0.3864] Input - Toggle Flashlight
  (:`Pressed`
    (`/Game/FemaleShooter/Blueprint/Component/GunnerGirlComponent.ToggleFlashLight` (`self.GunnerGirlComponent`) :!label _label_19)))

(event `LeftWeaponSwapActor`
  (params (Item :type "/Game/FemaleShooter/Additional/SimpleItem/SimpleItem Object Reference"))
  ;[0 0.6445 1] Item Collector
  (bind _displayedactor (`/Game/FemaleShooter/Additional/SimpleItem/SimpleItem.GetDisplayedActor` Item))
  (`/Engine/EditorBlueprintResources/StandardMacros.IsValid` _displayedactor
    (:`Is Valid`
      (bind _removedequipmentactor (`/Game/FemaleShooter/Blueprint/Component/TwinGunHandler.PickupEquipmentActor` (`self.TwinGunHandler`) _displayedactor "LeftGun" "Holster_L" "Weapon_L" "NewEnumerator1"))
      (`/Game/FemaleShooter/Additional/SimpleItem/SimpleItem.ChangeDisplayedActor` Item _removedequipmentactor))
    (:`Is Not Valid`
      (bind _droppedequipmentactor (`/Game/FemaleShooter/Blueprint/Component/TwinGunHandler.DropEquipmentActor` (`self.TwinGunHandler`) "LeftGun" "NewEnumerator1"))
      (`/Game/FemaleShooter/Additional/SimpleItem/SimpleItem.ChangeDisplayedActor` Item _droppedequipmentactor))))

(event `Key|Q`
  (params (Key :type "Key Structure"))
  ;[0.3564 1 0.3864] Input - Toggle Flashlight
  (:`Pressed`
    (goto _label_19)))

(fn `UserConstructionScript`)