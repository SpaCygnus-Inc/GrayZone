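; EquipmentInstance tracks one piece of character equipment and moves its Actor between an equip socket and a storage socket on a skeletal mesh.
; UpdateData sets the class and socket names, while equip and storage events attach to the character's mesh and UpdateInstance reattaches from the saved state.
; A shared attach function disables collision on one primitive component, snaps the root to the socket, and records the parent mesh, socket and equipped flag.
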(event `UpdateData`
  (params (ActorClass :type "Actor Class Reference") (StorageSocketName :type Name) (EquipSocketName :type Name))
  (set `self.ActorClass` ActorClass)
  (set `self.StorageSocketName` StorageSocketName)
  (set `self.EquipSocketName` EquipSocketName))

(event `CharacterEquip`
  (params (Character :type "Character Object Reference"))
  (`self.AttachActorToSocket` (`Character.Mesh` Character) (`self.Actor`) (`self.EquipSocketName`)))

(event `CharacterStorage`
  (params (Character :type "Character Object Reference"))
  (`self.AttachActorToSocket` (`Character.Mesh` Character) (`self.Actor`) (`self.StorageSocketName`)))

(event `UpdateInstance`
  (`self.AttachActorToSocket` (`self.ParentMesh`) (`self.Actor`) (select `bool` (`self.IsEquipped`) :`false` (`self.StorageSocketName`) :`true` (`self.EquipSocketName`))))

(fn `AttachActorToSocket`
  (params (SkeletalMesh :type "SkeletalMeshComponent Object Reference") (Actor :type "Actor Object Reference") (SocketName :type Name))
  (set `self.ParentMesh` SkeletalMesh)
  (`|ExecutionSequence`
    (:`then_0`
      (`PrimitiveComponent.SetCollisionEnabled` (`Actor.GetComponentByClass` Actor "/Script/Engine.PrimitiveComponent") "NoCollision"))
    (:`then_1`
      (`SceneComponent.K2_AttachToComponent` (`Actor.RootComponent` Actor) (`self.ParentMesh`) SocketName "SnapToTarget" "SnapToTarget" "SnapToTarget" true))
    (:`then_2`
      (`/Engine/EditorBlueprintResources/StandardMacros.IsValid` self
        (:`Is Valid`
          (set `self.CurrentSocket` SocketName)
          (set `self.IsEquipped` (== SocketName (`self.EquipSocketName`))))))))