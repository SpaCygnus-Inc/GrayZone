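; Equipment manager that spawns, swaps and attaches equipment actors on a character's mesh, tracked by identifier.
; Set or list updates diff identifiers against current gear, then remove, update or generate items according to the equip option.
; Items snap to hold or storage sockets with collision disabled, and updates preserve equipped state.
; Spawning goes through a Spawner unless an actor is provided, removal destroys or detaches, and sets can adjust high-heel offsets.
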(event `Internal_UpdateEquipmentList`
  (params (EquipOption :type "/Game/FemaleShooter/Blueprint/Enum/EquipmentChangeOption Enum" :default "NewEnumerator0") (RemovalOption2 :type "/Game/FemaleShooter/Blueprint/Enum/EquipmentRemovalOption Enum" :default "NewEnumerator0") (IdentifierList :type "Array of Name") (EquipmentMap :type "Map of Name to /Game/FemaleShooter/Blueprint/Struct/EquipmentDataStruct Structure"))
  (bind _array (`|MakeArray`))
  (bind _keys (`BlueprintMapLibrary.Map_Keys` (`self.ActorDict`)))
  (bind (_existinglist _addedlist _removedlist) (`self.CompareIdentifiers` _keys IdentifierList))
  (`self.RemoveEquipments` (select `/Game/FemaleShooter/Blueprint/Enum/EquipmentChangeOption` EquipOption :`NewEnumerator0` _removedlist :`NewEnumerator2` _array :`NewEnumerator1` _array) RemovalOption2)
  (`self.UpdateEquipments` (select `/Game/FemaleShooter/Blueprint/Enum/EquipmentChangeOption` EquipOption :`NewEnumerator0` _existinglist :`NewEnumerator2` _existinglist :`NewEnumerator1` _array) EquipmentMap RemovalOption2)
  (`self.GenerateEquipments` (select `/Game/FemaleShooter/Blueprint/Enum/EquipmentChangeOption` EquipOption :`NewEnumerator0` _addedlist :`NewEnumerator2` _addedlist :`NewEnumerator1` _addedlist) EquipmentMap)
  (`self.OnEquipmentUpdated`))

(event `SetupCharacter`
  (params (Character :type "Character Object Reference") (Spawner :type "/Game/FemaleShooter/Blueprint/Interface/I_Spawner Interface"))
  (`self.Setup` Character (`Character.Mesh` Character) Spawner))

(event `UpdateHighHeels`
  (params (HeelsData :type "/Game/FemaleShooter/Blueprint/Struct/HighHeelSharedData Structure") (IsForced :type Boolean))
  (bind (_isapplysettings _heightoffset _rotationoffset) (break `/Game/FemaleShooter/Blueprint/Struct/HighHeelSharedData` HeelsData))
  (bind _returnvalue (`Actor.GetComponentByClass` (`self.Owner`) "/Game/FemaleShooter/Blueprint/Component/HighHeelComponent.HighHeelComponent_C"))
  (if (or _isapplysettings IsForced)
    (`/Engine/EditorBlueprintResources/StandardMacros.IsValid` _returnvalue
      (:`Is Valid`
        (set `/Game/FemaleShooter/Blueprint/Component/HighHeelComponent.HeightOffset` _heightoffset _returnvalue)
        (set `/Game/FemaleShooter/Blueprint/Component/HighHeelComponent.RotationOffset` _rotationoffset _returnvalue)))))

(event `Setup`
  (params (Owner :type "Actor Object Reference") (MeshComponent :type "SkeletalMeshComponent Object Reference") (Spawner :type "/Game/FemaleShooter/Blueprint/Interface/I_Spawner Interface"))
  (set `self.Owner` Owner)
  (set `self.MeshComponent` MeshComponent)
  (set `self.Spawner` Spawner))

(event `UpdateEquipmentList`
  (params (EquipmentList :type "Array of /Game/FemaleShooter/Blueprint/Struct/EquipmentDataStruct Structure") (EquipOption :type "/Game/FemaleShooter/Blueprint/Enum/EquipmentChangeOption Enum" :default "NewEnumerator0") (RemovalOption2 :type "/Game/FemaleShooter/Blueprint/Enum/EquipmentRemovalOption Enum" :default "NewEnumerator0"))
  (bind (_identifierlist _equipmentmap) (`self.ExtractIdentifierList` EquipmentList))
  (`self.Internal_UpdateEquipmentList` EquipOption RemovalOption2 _identifierlist _equipmentmap))

(event `LoadEquipmentSet`
  (params (EquipmentSet :type "/Game/FemaleShooter/Blueprint/Data/Equipment/EquipmentSet Object Reference"))
  (bind _equipmentset (`self.EquipmentSet`))
  (bind _output_get (set `self.EquipmentSet` EquipmentSet))
  (`/Engine/EditorBlueprintResources/StandardMacros.IsValid` _output_get
    (:`Is Valid`
      (`self.UpdateHighHeels` (`/Game/FemaleShooter/Blueprint/Data/Equipment/EquipmentSet.HighHeelsSettings` _equipmentset) true)
      (`self.UpdateEquipmentList` (`/Game/FemaleShooter/Blueprint/Data/Equipment/EquipmentSet.EquipmentList` _equipmentset) "NewEnumerator0" "NewEnumerator0"))))

(event `PickupEquipmentSet`
  (params (EquipmentSet :type "/Game/FemaleShooter/Blueprint/Data/Equipment/EquipmentSet Object Reference"))
  (`/Engine/EditorBlueprintResources/StandardMacros.IsValid` EquipmentSet
    (:`Is Valid`
      (`self.UpdateHighHeels` (`/Game/FemaleShooter/Blueprint/Data/Equipment/EquipmentSet.HighHeelsSettings` EquipmentSet))
      (`self.UpdateEquipmentList` (`/Game/FemaleShooter/Blueprint/Data/Equipment/EquipmentSet.EquipmentList` EquipmentSet) "NewEnumerator2" "NewEnumerator0"))))

(event `ClearEqupmentSet`
  (set `self.EquipmentSet` null)
  (`self.UpdateHighHeels` (make `/Game/FemaleShooter/Blueprint/Struct/HighHeelSharedData` false) true)
  (`self.UpdateEquipmentList` (`|MakeArray`) "NewEnumerator0" "NewEnumerator0"))

(event `RemoveCurrentEquipments`
  (params (RemovalOption2 :type "/Game/FemaleShooter/Blueprint/Enum/EquipmentRemovalOption Enum" :default "NewEnumerator0"))
  (bind _keys (`BlueprintMapLibrary.Map_Keys` (`self.ActorDict`)))
  (`self.RemoveEquipments` _keys RemovalOption2))

(event `RemoveEquipments`
  (params (EquipmentList :type "Array of Name (by ref)") (RemovalOption2 :type "/Game/FemaleShooter/Blueprint/Enum/EquipmentRemovalOption Enum" :default "NewEnumerator0"))
  (for _array_element EquipmentList
    (`self.RemoveEquipment` _array_element RemovalOption2)))

(event `GenerateEquipments`
  (params (IdentifierList :type "Array of Name") (EquipmentMap :type "Map of Name to /Game/FemaleShooter/Blueprint/Struct/EquipmentDataStruct Structure"))
  (for _array_element IdentifierList
    (`self.GenerateEquipment` (`BlueprintMapLibrary.Map_Find` EquipmentMap _array_element))))

(event `ReattachEquipment`
  (params (Identifier :type Name))
  (bind (_value _returnvalue) (`BlueprintMapLibrary.Map_Find` (`self.EquipStatusDict`) Identifier))
  (if _returnvalue
    (if _value
      (`self.HoldEquipment` Identifier)
      (else
        (`self.StoreEquipment` Identifier)))))

(event `UpdateEquipments`
  (params (IdentifierList :type "Array of Name") (EquipmentMap :type "Map of Name to /Game/FemaleShooter/Blueprint/Struct/EquipmentDataStruct Structure") (RemovalOption2 :type "/Game/FemaleShooter/Blueprint/Enum/EquipmentRemovalOption Enum" :default "NewEnumerator0"))
  (for _array_element IdentifierList
    (`self.UpdateEquipment` _array_element (`BlueprintMapLibrary.Map_Find` EquipmentMap _array_element) null RemovalOption2)))

(event `HoldEquipment`
  (params (Identifier :type Name))
  (`self.Internal_AttachEquipment` Identifier true (`.EquipSocketName_14_1771FD3740FEB9F0070E06B758E0A8D6` (break `/Game/FemaleShooter/Blueprint/Struct/EquipmentDataStruct` (`BlueprintMapLibrary.Map_Find` (`self.DataDict`) Identifier)))))

(event `StoreEquipment`
  (params (Identifier :type Name))
  (`self.Internal_AttachEquipment` Identifier false (`.StorageSocketName_12_48FBA803401A2B5E46E19AB65E2CAEFA` (break `/Game/FemaleShooter/Blueprint/Struct/EquipmentDataStruct` (`BlueprintMapLibrary.Map_Find` (`self.DataDict`) Identifier)))))

(event `Internal_AttachEquipment`
  (params (Identifier :type Name) (IsEquipped :type Boolean) (SocketName :type Name))
  (bind _meshcomponent (`self.MeshComponent`))
  (bind _value (`BlueprintMapLibrary.Map_Find` (`self.ActorDict`) Identifier))
  (`/Engine/EditorBlueprintResources/StandardMacros.IsValid` _meshcomponent
    (:`Is Valid`
      (`/Engine/EditorBlueprintResources/StandardMacros.IsValid` _value
        (:`Is Valid`
          (`|ExecutionSequence`
            (:`then_0`
              (`PrimitiveComponent.SetCollisionEnabled` (`Actor.GetComponentByClass` _value "/Script/Engine.PrimitiveComponent") "NoCollision"))
            (:`then_1`
              (`SceneComponent.K2_AttachToComponent` (`Actor.RootComponent` _value) _meshcomponent SocketName "SnapToTarget" "SnapToTarget" "SnapToTarget" true))
            (:`then_2`
              (`BlueprintMapLibrary.Map_Add` (`self.CurrentSocketDict`) Identifier SocketName)
              (`BlueprintMapLibrary.Map_Add` (`self.EquipStatusDict`) Identifier IsEquipped))))))))

(fn `CheckIdentifierStatus`
  (params (OldList :type "Array of Name") (NewList :type "Array of Name") (IsDebugPrint :type Boolean) (identifier :type Name))
  (returns (ExistingList :type "Array of Name") (AddedList :type "Array of Name") (RemovedList :type "Array of Name"))
  (locals (TempExistList :type "Array of Name") (TempAddedList :type "Array of Name") (TempRemovedList :type "Array of Name"))
  (for _array_element NewList
    (if (>= (`KismetArrayLibrary.Array_Find` OldList _array_element) 0)
      (`KismetArrayLibrary.Array_Add` (`local.TempExistList`) _array_element)
      (if IsDebugPrint
        (`KismetSystemLibrary.PrintString` null (`KismetStringLibrary.Concat_StrStr` "Found Existing: " (`KismetStringLibrary.Conv_NameToString` _array_element))))
      (else
        (`KismetArrayLibrary.Array_Add` (`local.TempAddedList`) _array_element)
        (if IsDebugPrint
          (`KismetSystemLibrary.PrintString` null (`KismetStringLibrary.Concat_StrStr` "Found Addition: " (`KismetStringLibrary.Conv_NameToString` _array_element)))))))
  (for _array_element_2 OldList
    (if (not (>= (`KismetArrayLibrary.Array_Find` (`local.TempExistList`) _array_element_2) 0))
      (`KismetArrayLibrary.Array_Add` (`local.TempRemovedList`) _array_element_2)
      (if IsDebugPrint
        (`KismetSystemLibrary.PrintString` null (`KismetStringLibrary.Concat_StrStr` "Found Removal" (`KismetStringLibrary.Conv_NameToString` _array_element_2))))))
  (return (`local.TempExistList`) (`local.TempAddedList`) (`local.TempRemovedList`)))

(fn `CompareIdentifiers`
  (params (OldList :type "Array of Name") (NewList :type "Array of Name") (IsDebugPrint :type Boolean))
  (returns (ExistingList :type "Array of Name") (AddedList :type "Array of Name") (RemovedList :type "Array of Name"))
  (locals (TempExistList :type "Array of Name") (TempAddedList :type "Array of Name") (TempRemovedList :type "Array of Name"))
  (for _array_element NewList
    (if (>= (`KismetArrayLibrary.Array_Find` OldList _array_element) 0)
      (`KismetArrayLibrary.Array_Add` (`local.TempExistList`) _array_element)
      (if IsDebugPrint
        (`KismetSystemLibrary.PrintString` null (`KismetStringLibrary.Concat_StrStr` "Found Existing: " (`KismetStringLibrary.Conv_NameToString` _array_element))))
      (else
        (`KismetArrayLibrary.Array_Add` (`local.TempAddedList`) _array_element)
        (if IsDebugPrint
          (`KismetSystemLibrary.PrintString` null (`KismetStringLibrary.Concat_StrStr` "Found Addition: " (`KismetStringLibrary.Conv_NameToString` _array_element)))))))
  (for _array_element_2 OldList
    (if (not (>= (`KismetArrayLibrary.Array_Find` (`local.TempExistList`) _array_element_2) 0))
      (`KismetArrayLibrary.Array_Add` (`local.TempRemovedList`) _array_element_2)
      (if IsDebugPrint
        (`KismetSystemLibrary.PrintString` null (`KismetStringLibrary.Concat_StrStr` "Found Removal" (`KismetStringLibrary.Conv_NameToString` _array_element_2))))))
  (return (`local.TempExistList`) (`local.TempAddedList`) (`local.TempRemovedList`)))

(fn `ExtractIdentifierList`
  (params (EquipmentDataList :type "Array of /Game/FemaleShooter/Blueprint/Struct/EquipmentDataStruct Structure"))
  (returns (IdentifierList :type "Array of Name") (EquipmentMap :type "Map of Name to /Game/FemaleShooter/Blueprint/Struct/EquipmentDataStruct Structure"))
  (locals (TempList :type "Array of Name") (TempEquipmentMap :type "Map of Name to /Game/FemaleShooter/Blueprint/Struct/EquipmentDataStruct Structure"))
  (for _array_element EquipmentDataList
    (bind _identifier (break `/Game/FemaleShooter/Blueprint/Struct/EquipmentDataStruct` _array_element))
    (`KismetArrayLibrary.Array_Add` (`local.TempList`) _identifier)
    (`BlueprintMapLibrary.Map_Add` (`local.TempEquipmentMap`) _identifier _array_element))
  (return (`local.TempList`) (`local.TempEquipmentMap`)))

(fn `GenerateEquipment`
  (params (EquipmentData :type "/Game/FemaleShooter/Blueprint/Struct/EquipmentDataStruct Structure") (ProvidedActor :type "Actor Object Reference") (IsEquipped :type Boolean) (IsDebugPrint :type Boolean))
  (returns (Identifier :type Name) (Actor :type "Actor Object Reference"))
  (locals (TempActor :type "Actor Object Reference"))
  (bind (_identifier _actorclass _storagesocketname _equipsocketname) (break `/Game/FemaleShooter/Blueprint/Struct/EquipmentDataStruct` EquipmentData))
  (bind _tempactor (`local.TempActor`))
  (bind _actordict (`self.ActorDict`))
  (`|ExecutionSequence`
    (:`then_0`
      (if IsDebugPrint
        (`KismetSystemLibrary.PrintString` null (`KismetStringLibrary.Concat_StrStr` "Equipment Generated: " (`KismetStringLibrary.Conv_NameToString` _identifier)))))
    (:`then_1`
      (if (`KismetSystemLibrary.IsValidClass` _actorclass)
        (`/Engine/EditorBlueprintResources/StandardMacros.IsValid` ProvidedActor
          (:`Is Valid`
            (set `local.TempActor` ProvidedActor))
          (:`Is Not Valid`
            (bind _actor (`/Game/FemaleShooter/Blueprint/Interface/I_Spawner.RequestSpawnActor` (`self.Spawner`) _actorclass (`KismetMathLibrary.MakeTransform` (0.0 0.0 0.0)) "Undefined"))
            (set `local.TempActor` _actor)))
        (`/Engine/EditorBlueprintResources/StandardMacros.IsValid` _tempactor
          (:`Is Valid`
            (`|ExecutionSequence`
              (:`then_0`
                (`PrimitiveComponent.SetCollisionEnabled` (`Actor.GetComponentByClass` _tempactor "/Script/Engine.PrimitiveComponent") "NoCollision")
                (`Actor.SetActorHiddenInGame` _tempactor false))
              (:`then_1`
                (`BlueprintMapLibrary.Map_Add` _actordict _identifier)
                (`BlueprintMapLibrary.Map_Remove` _actordict _identifier)
                (`BlueprintMapLibrary.Map_Add` (`self.ActorDict`) _identifier (`local.TempActor`))
                (`BlueprintMapLibrary.Map_Add` (`self.DataDict`) _identifier EquipmentData)
                (`BlueprintMapLibrary.Map_Add` (`self.CurrentSocketDict`) _storagesocketname _equipsocketname)
                (`BlueprintMapLibrary.Map_Add` (`self.EquipStatusDict`) _identifier IsEquipped))
              (:`then_2`
                (`self.ReattachEquipment` _identifier))
              (:`then_3`
                (return _identifier (`local.TempActor`)))))
          (:`Is Not Valid`
            (return "None" null)))
        (else
          (return "None" null))))))

(fn `GetEquipmentActor`
  (params (Identifier :type Name))
  (returns (Actor :type "Actor Object Reference"))
  (return (`BlueprintMapLibrary.Map_Find` (`self.ActorDict`) Identifier)))

(fn `IdentifierExist`
  (params (Identifier :type Name))
  (returns (IsExist :type Boolean))
  (return (`.ReturnValue` (`BlueprintMapLibrary.Map_Find` (`self.ActorDict`) Identifier))))

(fn `LoadEquipmentActor`
  (params (EquipmentActor :type "Actor Object Reference") (Identifier :type Name) (StorageSocketName :type Name) (EquipSocketName :type Name) (RemovalOption2 :type "/Game/FemaleShooter/Blueprint/Enum/EquipmentRemovalOption Enum" :default "NewEnumerator0"))
  (returns (RemovedEquipmentActor :type "Actor Object Reference"))
  (locals (DroppedActor :type "Actor Object Reference"))
  (bind _equipmentdatastruct (make `/Game/FemaleShooter/Blueprint/Struct/EquipmentDataStruct` Identifier (`GameplayStatics.GetObjectClass` EquipmentActor) StorageSocketName EquipSocketName))
  (`|ExecutionSequence`
    (:`then_0`
      (switch `/Game/FemaleShooter/Blueprint/Enum/EquipmentRemovalOption` RemovalOption2
        (:`NewEnumerator0`
          (set `local.DroppedActor` null))
        (:`NewEnumerator1`
          (set `local.DroppedActor` (`BlueprintMapLibrary.Map_Find` (`self.ActorDict`) Identifier)))))
    (:`then_1`
      (`/Engine/EditorBlueprintResources/StandardMacros.IsValid` (`BlueprintMapLibrary.Map_Find` (`self.ActorDict`) Identifier)
        (:`Is Valid`
          (`self.UpdateEquipment` Identifier _equipmentdatastruct EquipmentActor RemovalOption2))
        (:`Is Not Valid`
          (`self.GenerateEquipment` _equipmentdatastruct EquipmentActor)))
      (`self.OnEquipmentUpdated`)
      (return (`local.DroppedActor`)))))

(fn `RemoveEquipment`
  (params (Identifier :type Name) (RemovalOption2 :type "/Game/FemaleShooter/Blueprint/Enum/EquipmentRemovalOption Enum" :default "NewEnumerator0") (IsDebugPrint :type Boolean))
  (returns (Actor :type "Actor Object Reference"))
  (locals (PurgedActor :type "Actor Object Reference"))
  (bind _value (`BlueprintMapLibrary.Map_Find` (`self.ActorDict`) Identifier))
  (`|ExecutionSequence`
    (:`then_0`
      (if IsDebugPrint
        (`KismetSystemLibrary.PrintString` null (`KismetStringLibrary.Concat_StrStr` "Equipment Removed: " (`KismetStringLibrary.Conv_NameToString` Identifier)))))
    (:`then_1`
      (`/Engine/EditorBlueprintResources/StandardMacros.IsValid` _value
        (:`Is Valid`
          (set `local.PurgedActor` _value)
          (`|ExecutionSequence`
            (:`then_0`
              (`BlueprintMapLibrary.Map_Add` (`self.ActorDict`) Identifier)
              (`BlueprintMapLibrary.Map_Remove` (`self.ActorDict`) Identifier)
              (`BlueprintMapLibrary.Map_Remove` (`self.DataDict`) Identifier)
              (`BlueprintMapLibrary.Map_Remove` (`self.CurrentSocketDict`) Identifier)
              (`BlueprintMapLibrary.Map_Remove` (`self.EquipStatusDict`) Identifier))
            (:`then_1`
              (`Actor.K2_DetachFromActor` (`local.PurgedActor`) "KeepWorld" "KeepWorld" "KeepWorld"))
            (:`then_2`
              (switch `/Game/FemaleShooter/Blueprint/Enum/EquipmentRemovalOption` RemovalOption2
                (:`NewEnumerator0`
                  (`Actor.K2_DestroyActor` (`local.PurgedActor`))
                  (return null))
                (:`NewEnumerator1`
                  (return (`local.PurgedActor`)))))))
        (:`Is Not Valid`
          (return null))))))

(fn `UpdateEquipment`
  (params (EquipmentIdentifier :type Name) (EquipmentData :type "/Game/FemaleShooter/Blueprint/Struct/EquipmentDataStruct Structure") (ProvidedActor :type "Actor Object Reference") (RemovalOption2 :type "/Game/FemaleShooter/Blueprint/Enum/EquipmentRemovalOption Enum" :default "NewEnumerator0") (IsDebugPrint :type Boolean))
  (returns (Identifier :type Name) (Actor :type "Actor Object Reference"))
  (locals (TempActor :type "Actor Object Reference") (IsPreviouslyEquipped :type Boolean))
  (`|ExecutionSequence`
    (:`then_0`
      (if IsDebugPrint
        (`KismetSystemLibrary.PrintString` null (`KismetStringLibrary.Concat_StrStr` "Equipment Updated: " (`KismetStringLibrary.Conv_NameToString` EquipmentIdentifier)))))
    (:`then_1`
      (set `local.IsPreviouslyEquipped` (`BlueprintMapLibrary.Map_Find` (`self.EquipStatusDict`) EquipmentIdentifier))
      (`self.RemoveEquipment` EquipmentIdentifier RemovalOption2)
      (`self.GenerateEquipment` EquipmentData ProvidedActor (`local.IsPreviouslyEquipped`)))))