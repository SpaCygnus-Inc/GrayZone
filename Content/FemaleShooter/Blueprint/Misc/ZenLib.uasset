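; ZenLib is a utility function library for the FemaleShooter game, covering aiming, rotation math, attachment, component setup and display settings.
; Crosshair targeting deprojects the offset screen center and line-traces on Visibility, returning the hit or trace end.
; Rotator helpers add, subtract and wrap angles, while attach helpers disable primitive collision and snap objects to mesh sockets.
; Other helpers send a setup message to every actor component and apply screen mode and resolution without saving.
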(fn `AddRotation`
  (params (Rot1 :type "Rotator Structure") (Rot2 :type "Rotator Structure"))
  (returns (Result :type "Rotator Structure"))
  (return (`KismetMathLibrary.MakeRotator` (+ (.roll Rot1) (.roll Rot2)) (+ (.pitch Rot1) (.pitch Rot2)) (+ (.yaw Rot1) (.yaw Rot2)))))

(fn `AttachToCharacterSocket`
  (params (Character :type "Character Object Reference") (Object :type "Actor Object Reference") (SocketName :type Name))
  (`self.AttachToMeshSocket` (`Character.Mesh` Character) Object SocketName (`local.__WorldContext`)))

(fn `AttachToMeshSocket`
  (params (SkeletalMesh :type "SkeletalMeshComponent Object Reference") (Object :type "Actor Object Reference") (SocketName :type Name))
  (`|ExecutionSequence`
    (:`then_0`
      (`PrimitiveComponent.SetCollisionEnabled` (`Actor.GetComponentByClass` Object "/Script/Engine.PrimitiveComponent") "NoCollision"))
    (:`then_1`
      (`SceneComponent.K2_AttachToComponent` (`Actor.RootComponent` Object) SkeletalMesh SocketName "SnapToTarget" "SnapToTarget" "SnapToTarget" true))))

(fn `Clamp180`
  (params (Input :type "Float (double-precision)"))
  (returns (Output :type "Float (double-precision)"))
  (bind _output (`self.Clamp360` Input))
  (return (select `bool` (> _output 180.0) :`false` _output :`true` (- _output 360.0))))

(fn `Clamp360`
  (params (Input :type "Float (double-precision)"))
  (returns (Output :type "Float (double-precision)"))
  (return (mod (+ (mod Input 360.0) 360.0) 360.0)))

(fn `RetrieveCrosshairTarget`
  (params (ActiveCharacter :type "Character Object Reference") (CrosshairOffset :type "Vector2D Structure") (MaxDistance :type "Float (double-precision)") (IsDrawDebugLine :type Boolean))
  (returns (IsTargetFound :type Boolean) (HitResult :type "HitResult Structure") (TargetLocation :type "Vector Structure"))
  (`/Engine/EditorBlueprintResources/StandardMacros.IsValid` ActiveCharacter
    (:`Is Valid`
      (bind _asplayer_controller (cast `PlayerController` (`Pawn.GetController` ActiveCharacter))
        (:`then`
          (bind (_worldposition _worlddirection) (`GameplayStatics.DeprojectScreenToWorld` _asplayer_controller (+ (/ (`WidgetLayoutLibrary.GetViewportSize` ActiveCharacter) 2.0) (* CrosshairOffset (`WidgetLayoutLibrary.GetViewportScale` ActiveCharacter)))))
          (bind (_outhit _returnvalue) (`KismetSystemLibrary.LineTraceSingle` null _worldposition (+ _worldposition (* _worlddirection MaxDistance)) "TraceTypeQuery1" false (`|MakeArray` ActiveCharacter :!type "Actor Object Reference") (select `bool` IsDrawDebugLine :`true` "ForDuration" :!type "EDrawDebugTrace Enum")))
          (bind (_bblockinghit _binitialoverlap _time _distance _location _impactpoint _normal _impactnormal _physmat _hitactor _hitcomponent _hitbonename _hititem _faceindex _tracestart _traceend) (`GameplayStatics.BreakHitResult` _outhit))
          (return _returnvalue _outhit (select `bool` _returnvalue :`false` _traceend :`true` _location)))
        (:`CastFailed`
          (return false (struct) (0.0 0.0 0.0)))))))

(fn `SetupComponents`
  (params (Actor :type "Actor Object Reference"))
  (for _array_element (`Actor.K2_GetComponentsByClass` Actor "/Script/Engine.ActorComponent")
    (`/Engine/EditorBlueprintResources/StandardMacros.IsValid` _array_element
      (:`Is Valid`
        (message `/Game/FemaleShooter/Blueprint/Interface/I_SetupComponent.SetupComponent` _array_element)))))

(fn `SubtractRotation`
  (params (Rot1 :type "Rotator Structure") (Rot2 :type "Rotator Structure"))
  (returns (Result :type "Rotator Structure"))
  (return (`KismetMathLibrary.MakeRotator` (- (.roll Rot1) (.roll Rot2)) (- (.pitch Rot1) (.pitch Rot2)) (- (.yaw Rot1) (.yaw Rot2)))))

(fn `UpdateScreenDisplay`
  (params (ScreenMode :type "EWindowMode Enum" :default "Fullscreen") (ScreenResolution :type "IntPoint Structure"))
  (bind _returnvalue (`GameUserSettings.GetGameUserSettings`))
  (`GameUserSettings.SetFullscreenMode` _returnvalue ScreenMode)
  (`GameUserSettings.SetScreenResolution` _returnvalue ScreenResolution)
  (`GameUserSettings.ApplyResolutionSettings` _returnvalue false))