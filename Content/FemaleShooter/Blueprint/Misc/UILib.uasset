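; UILib is a function library for directional focus navigation across GunnerGirl UI widgets that implement the container and element interfaces.
; GetDefaultFocus builds a UIPointer from a container's focus data, tracking the active element and index.
; Above/Below functions step it through vertical containers and Left/Right through horizontal ones, wrapping when cyclical.
; Helpers build element lists from widget arrays, collect element widgets from a VerticalBox, and print pointers for debugging.
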(fn `FocusListFromVerticalBox`
  (params (VBox :type "VerticalBox Object Reference"))
  (returns (WidgetList :type "Array of Widget Object Reference"))
  (locals (TempWidgetList :type "Array of Widget Object Reference") (Widget :type "Widget Object Reference"))
  (`|ExecutionSequence`
    (:`then_0`
      (for _index (range (`PanelWidget.GetChildrenCount` VBox))
        (bind _output_get (set `local.Widget` (`PanelWidget.GetChildAt` VBox _index)))
        (cast `/Game/FemaleShooter/Blueprint/Interface/I_GunnerGirl_UIElement` _output_get)
        (`KismetArrayLibrary.Array_Add` (`local.TempWidgetList`) _output_get)))
    (:`then_1`
      (return (`local.TempWidgetList`)))))

(fn `GenerateElementList`
  (params (Container :type "/Game/FemaleShooter/Blueprint/Interface/I_GunnerGirl_UIContainer Interface") (WidgetList :type "Array of Widget Object Reference"))
  (returns (ElementList :type "Array of /Game/FemaleShooter/Blueprint/Interface/I_GunnerGirl_UIElement Interface"))
  (locals (TempElementList :type "Array of /Game/FemaleShooter/Blueprint/Interface/I_GunnerGirl_UIElement Interface"))
  (`|ExecutionSequence`
    (:`then_0`
      (for _array_element WidgetList
        (bind _asi_gunner_girl_uielement (cast `/Game/FemaleShooter/Blueprint/Interface/I_GunnerGirl_UIElement` _array_element))
        (`KismetArrayLibrary.Array_Add` (`local.TempElementList`) _asi_gunner_girl_uielement)))
    (:`then_1`
      (return (`local.TempElementList`)))))

(fn `GetDefaultFocus`
  (params (Widget :type "Widget Object Reference"))
  (returns (Pointer :type "/Game/FemaleShooter/Blueprint/Struct/UI/UI_Pointer Structure"))
  (bind _asi_gunner_girl_uicontainer (cast `/Game/FemaleShooter/Blueprint/Interface/I_GunnerGirl_UIContainer` Widget)
    (:`then`
      (bind (_focusedelement _isprocessed) (`/Game/FemaleShooter/Blueprint/Interface/I_GunnerGirl_UIContainer.GetDefaultFocus` _asi_gunner_girl_uicontainer))
      (bind (_uitype _iscyclical _elementlist) (`/Game/FemaleShooter/Blueprint/Interface/I_GunnerGirl_UIContainer.GetFocusData` _asi_gunner_girl_uicontainer))
      (if (> (`KismetArrayLibrary.Array_Length` _elementlist) 0)
        (bind _returnvalue (select `bool` _isprocessed :`true` (`KismetArrayLibrary.Array_Find` _elementlist _focusedelement)))
        (bind _output (`|GetArrayItem` _elementlist _returnvalue))
        (bind _widget (`/Game/FemaleShooter/Blueprint/Interface/I_GunnerGirl_UIElement.GetWidget` _output))
        (return (make `/Game/FemaleShooter/Blueprint/Struct/UI/UI_Pointer` true _asi_gunner_girl_uicontainer _output _returnvalue false Widget _widget))
        (else
          (return (make `/Game/FemaleShooter/Blueprint/Struct/UI/UI_Pointer` true _asi_gunner_girl_uicontainer null -1 false Widget)))))
    (:`CastFailed`
      (return))))

(fn `GetFocusAbove`
  (params (UIPointer :type "/Game/FemaleShooter/Blueprint/Struct/UI/UI_Pointer Structure"))
  (returns (ResultPointer :type "/Game/FemaleShooter/Blueprint/Struct/UI/UI_Pointer Structure"))
  (bind (_isvalid _container _activeelement _activeindex _ishud _containerwidget) (break `/Game/FemaleShooter/Blueprint/Struct/UI/UI_Pointer` UIPointer))
  (bind _returnvalue (+ _activeindex -1))
  (bind (_uitype _iscyclical _elementlist) (`/Game/FemaleShooter/Blueprint/Interface/I_GunnerGirl_UIContainer.GetFocusData` _container))
  (switch `/Game/FemaleShooter/Blueprint/Enum/GunnerGirl_UIContainerType` _uitype
    (:`NewEnumerator0`
      (bind _returnvalue_2 (`KismetArrayLibrary.Array_Length` _elementlist))
      (if (> _returnvalue_2 0)
        (bind _returnvalue_3 (select `bool` (>= _returnvalue 0) :`false` (select `bool` _iscyclical :`false` _activeindex :`true` (- _returnvalue_2 1)) :`true` _returnvalue))
        (bind _output (`|GetArrayItem` _elementlist _returnvalue_3))
        (bind _widget (`/Game/FemaleShooter/Blueprint/Interface/I_GunnerGirl_UIElement.GetWidget` _output))
        (return (make `/Game/FemaleShooter/Blueprint/Struct/UI/UI_Pointer` true _container _output _returnvalue_3 _ishud _containerwidget _widget))
        (else
          _)))
    (:`NewEnumerator1`
      _))
  (return UIPointer))

(fn `GetFocusBelow`
  (params (UIPointer :type "/Game/FemaleShooter/Blueprint/Struct/UI/UI_Pointer Structure"))
  (returns (ResultPointer :type "/Game/FemaleShooter/Blueprint/Struct/UI/UI_Pointer Structure"))
  (bind (_isvalid _container _activeelement _activeindex _ishud _containerwidget) (break `/Game/FemaleShooter/Blueprint/Struct/UI/UI_Pointer` UIPointer))
  (bind _returnvalue (+ _activeindex 1))
  (bind (_uitype _iscyclical _elementlist) (`/Game/FemaleShooter/Blueprint/Interface/I_GunnerGirl_UIContainer.GetFocusData` _container))
  (switch `/Game/FemaleShooter/Blueprint/Enum/GunnerGirl_UIContainerType` _uitype
    (:`NewEnumerator0`
      (bind _returnvalue_2 (`KismetArrayLibrary.Array_Length` _elementlist))
      (if (> _returnvalue_2 0)
        (bind _returnvalue_3 (select `bool` (< _returnvalue _returnvalue_2) :`false` (select `bool` _iscyclical :`false` _activeindex :`true` (mod _returnvalue _returnvalue_2)) :`true` _returnvalue))
        (bind _output (`|GetArrayItem` _elementlist _returnvalue_3))
        (bind _widget (`/Game/FemaleShooter/Blueprint/Interface/I_GunnerGirl_UIElement.GetWidget` _output))
        (return (make `/Game/FemaleShooter/Blueprint/Struct/UI/UI_Pointer` true _container _output _returnvalue_3 _ishud _containerwidget _widget))
        (else
          _)))
    (:`NewEnumerator1`
      _))
  (return UIPointer))

(fn `GetFocusLeft`
  (params (UIPointer :type "/Game/FemaleShooter/Blueprint/Struct/UI/UI_Pointer Structure"))
  (returns (ResultPointer :type "/Game/FemaleShooter/Blueprint/Struct/UI/UI_Pointer Structure"))
  (bind (_isvalid _container _activeelement _activeindex _ishud _containerwidget) (break `/Game/FemaleShooter/Blueprint/Struct/UI/UI_Pointer` UIPointer))
  (bind _returnvalue (+ _activeindex -1))
  (bind (_uitype _iscyclical _elementlist) (`/Game/FemaleShooter/Blueprint/Interface/I_GunnerGirl_UIContainer.GetFocusData` _container))
  (switch `/Game/FemaleShooter/Blueprint/Enum/GunnerGirl_UIContainerType` _uitype
    (:`NewEnumerator0`
      _)
    (:`NewEnumerator1`
      (bind _returnvalue_2 (`KismetArrayLibrary.Array_Length` _elementlist))
      (if (> _returnvalue_2 0)
        (bind _returnvalue_3 (select `bool` (>= _returnvalue 0) :`false` (select `bool` _iscyclical :`false` _activeindex :`true` (- _returnvalue_2 1)) :`true` _returnvalue))
        (bind _output (`|GetArrayItem` _elementlist _returnvalue_3))
        (bind _widget (`/Game/FemaleShooter/Blueprint/Interface/I_GunnerGirl_UIElement.GetWidget` _output))
        (return (make `/Game/FemaleShooter/Blueprint/Struct/UI/UI_Pointer` true _container _output _returnvalue_3 _ishud _containerwidget _widget))
        (else
          _))))
  (return UIPointer))

(fn `GetFocusRight`
  (params (UIPointer :type "/Game/FemaleShooter/Blueprint/Struct/UI/UI_Pointer Structure"))
  (returns (ResultPointer :type "/Game/FemaleShooter/Blueprint/Struct/UI/UI_Pointer Structure"))
  (bind (_isvalid _container _activeelement _activeindex _ishud _containerwidget) (break `/Game/FemaleShooter/Blueprint/Struct/UI/UI_Pointer` UIPointer))
  (bind _returnvalue (+ _activeindex 1))
  (bind (_uitype _iscyclical _elementlist) (`/Game/FemaleShooter/Blueprint/Interface/I_GunnerGirl_UIContainer.GetFocusData` _container))
  (switch `/Game/FemaleShooter/Blueprint/Enum/GunnerGirl_UIContainerType` _uitype
    (:`NewEnumerator0`
      _)
    (:`NewEnumerator1`
      (bind _returnvalue_2 (`KismetArrayLibrary.Array_Length` _elementlist))
      (if (> _returnvalue_2 0)
        (bind _returnvalue_3 (select `bool` (< _returnvalue _returnvalue_2) :`false` (select `bool` _iscyclical :`false` _activeindex :`true` (mod _returnvalue _returnvalue_2)) :`true` _returnvalue))
        (bind _output (`|GetArrayItem` _elementlist _returnvalue_3))
        (bind _widget (`/Game/FemaleShooter/Blueprint/Interface/I_GunnerGirl_UIElement.GetWidget` _output))
        (return (make `/Game/FemaleShooter/Blueprint/Struct/UI/UI_Pointer` true _container _output _returnvalue_3 _ishud _containerwidget _widget))
        (else
          _))))
  (return UIPointer))

(fn `PrintPointer`
  (params (Pointer :type "/Game/FemaleShooter/Blueprint/Struct/UI/UI_Pointer Structure"))
  (bind ((`IsValid_16_ACF86F7A4B06EBD3509B77A656CBC147` _isvalid) (`Container_12_64639091486C03090C093AB56C229993` _container) (`ActiveElement_14_DF9F291E43D503DEB36086B0401BB257` _activeelement) (`ActiveIndex_11_2A70059445FC11E5A7061EA9EBC20EAC` _activeindex) (`IsHUD_18_8BEFEBEC4741202BBF7F189FF3254FD4` _ishud)) (break `/Game/FemaleShooter/Blueprint/Struct/UI/UI_Pointer` Pointer))
  (bind _widget (`/Game/FemaleShooter/Blueprint/Interface/I_GunnerGirl_UIElement.GetWidget` _activeelement))
  (bind _widget_2 (`/Game/FemaleShooter/Blueprint/Interface/I_GunnerGirl_UIContainer.GetWidget` _container))
  (`KismetSystemLibrary.PrintString` null (`KismetStringLibrary.Concat_StrStr` "Pointer valid [" (`KismetStringLibrary.Conv_BoolToString` _isvalid) "], container [" (`KismetSystemLibrary.GetDisplayName` _widget_2) "], focused element [" (`KismetSystemLibrary.GetDisplayName` _widget) "], is HUD [" (`KismetStringLibrary.Conv_BoolToString` _ishud) "], active index [" (`KismetStringLibrary.Conv_IntToString` _activeindex) "]")))