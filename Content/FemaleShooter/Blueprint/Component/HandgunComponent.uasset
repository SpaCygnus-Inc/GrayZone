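; Handgun actor component for the female shooter that handles firing and a gun-twirl animation on a skeletal gun mesh found by name or passed to Setup.
; PerformShot spawns the muzzle flash, briefly shows the owner's point light, spawns a Bullet toward an optional adjusted target, and plays randomized gunshot sound.
; Bullet hit callbacks play impact sounds.
; Tick applies frame-rate-scaled roll around the trigger socket pivot, offsetting location while spinning.
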(event `TryAutoSetupGun`
  (`/Engine/EditorBlueprintResources/StandardMacros.IsValid` (`self.GunMeshComponent`)
    (:`Is Not Valid`
      (for _array_element (`Actor.K2_GetComponentsByClass` (`self.GetOwner`) "/Script/Engine.SkeletalMeshComponent")
        (if (`KismetStringLibrary.EqualEqual_StrStr` (`self.GunMeshName`) (`KismetSystemLibrary.GetObjectName` _array_element))
          (`self.Setup` _array_element (`self.MuzzleSocketName`) (`self.GunSpinSpeed`)))))))

(event `self.ReceiveBeginPlay`
  (`self.TryAutoSetupGun`))

(event `SyncSpinFromOutside`
  (params (IsSpinning :type Boolean))
  (set `self.IsGunSpinning` IsSpinning))

(event `self.ReceiveTick`
  (params (DeltaSeconds :type "Float (single-precision)"))
  (`self.UpdateSpin`))

(event `Setup`
  (params (GunMeshComponent :type "SkeletalMeshComponent Object Reference") (MuzzleSocket :type Name :default "MuzzleSocket") (GunSpinSpeed :type "Float (double-precision)" :default 30.0))
  (set `self.GunMeshComponent` GunMeshComponent)
  (set `self.MuzzleSocketName` MuzzleSocket)
  (set `self.GunSpinSpeed` GunSpinSpeed)
  (`self.UpdateSpinPivot`))

(event `GenerateMuzzleLight`
  (params (IsGenerateMuzzleLight :type Boolean))
  (set `self.IsGenerateMuzzleLight` IsGenerateMuzzleLight)
  (if (`self.IsGenerateMuzzleLight`)
    (`KismetSystemLibrary.K2_ClearAndInvalidateTimerHandle` (`self.MuzzleLightTimer`))
    (set `self.MuzzleLightTimer` (struct))
    (`SceneComponent.SetVisibility` (`Actor.GetComponentByClass` (`self.GetOwner`) "/Script/Engine.PointLightComponent") true false)
    (bind _returnvalue (`KismetSystemLibrary.K2_SetTimerDelegate` (delegate `EndMuzzleLight`) 0.05))
    (set `self.MuzzleLightTimer` _returnvalue)))

(event `ShowMuzzleFlash`
  (params (MuzzleFlashEffect :type "ParticleSystem Object Reference") (isGenerateMuzzleLight :type Boolean))
  (`GameplayStatics.SpawnEmitterAttached` MuzzleFlashEffect (`self.GunMeshComponent`) (`self.MuzzleSocketName`))
  (`self.GenerateMuzzleLight` isGenerateMuzzleLight))

(event `EndMuzzleLight`
  (`KismetSystemLibrary.K2_ClearAndInvalidateTimerHandle` (`self.MuzzleLightTimer`))
  (set `self.MuzzleLightTimer` (struct))
  (`SceneComponent.SetVisibility` (`Actor.GetComponentByClass` (`self.GetOwner`) "/Script/Engine.PointLightComponent") false false))

(event `StartGunSpin`
  (set `self.IsGunSpinning` true))

(event `ActivateGunSpin`
  (params (IsActive :type Boolean))
  (if IsActive
    (`self.StartGunSpin`)
    (else
      (`self.StopGunSpin`))))

(event `StopGunSpin`
  (set `self.IsGunSpinning` false))

(event `PerformShot`
  (params (AmmoData :type "/Game/FemaleShooter/Blueprint/Data/Ammo/AmmoData Object Reference") (IsAdjustedTarget :type Boolean) (AdjustedTargetLocation :type "Vector Structure") (IsGenerateMuzzleLight :type Boolean))
  (`|ExecutionSequence`
    (:`then_0`
      (`self.ShowMuzzleFlash` (`/Game/FemaleShooter/Blueprint/Data/Ammo/AmmoData.MuzzleFlashEffect` AmmoData) IsGenerateMuzzleLight))
    (:`then_1`
      (`self.ShootBullet` IsAdjustedTarget AdjustedTargetLocation (`/Game/FemaleShooter/Blueprint/Data/Ammo/AmmoData.BulletSpeed` AmmoData) (`/Game/FemaleShooter/Blueprint/Data/Ammo/AmmoData.Gravity` AmmoData) (`/Game/FemaleShooter/Blueprint/Data/Ammo/AmmoData.ImpactModifier` AmmoData) (`/Game/FemaleShooter/Blueprint/Data/Ammo/AmmoData.Lifetime` AmmoData) (`/Game/FemaleShooter/Blueprint/Data/Ammo/AmmoData.BulletMesh` AmmoData) (`/Game/FemaleShooter/Blueprint/Data/Ammo/AmmoData.TrailEffect` AmmoData) (`/Game/FemaleShooter/Blueprint/Data/Ammo/AmmoData.ImpactEffect` AmmoData)))
    (:`then_2`
      (`self.PlayGunshotSound`))))

(event `ShootBullet`
  (params (IsAdjustedTarget :type Boolean) (AdjustedTargetLocation :type "Vector Structure") (BulletSpeed :type "Float (double-precision)") (Gravity :type "Float (double-precision)") (BulletImpactModifier :type "Float (double-precision)" :default 1.0) (Lifetime :type "Float (double-precision)") (BulletMesh :type "StaticMesh Object Reference") (TrailEffect :type "ParticleSystem Object Reference") (ImpactEffect :type "ParticleSystem Object Reference"))
  (bind _returnvalue (`SceneComponent.GetSocketTransform` (`self.GunMeshComponent`) (`self.MuzzleSocketName`) "RTS_World"))
  (bind _location (.location _returnvalue))
  (bind _returnvalue_2 (`|SpawnActorFromClass` "/Game/FemaleShooter/Asset/Bullet/Bullet.Bullet_C" (select `bool` IsAdjustedTarget :`false` _returnvalue :`true` (`KismetMathLibrary.MakeTransform` _location (`KismetMathLibrary.FindLookAtRotation` _location AdjustedTargetLocation) (.scale _returnvalue))) "AlwaysSpawn" "OverrideRootScale" null BulletMesh TrailEffect ImpactEffect BulletSpeed Gravity BulletImpactModifier Lifetime null))
  (add `/Game/FemaleShooter/Asset/Bullet/Bullet.OnBulletHit` _returnvalue_2 (delegate `OnBulletHit_Event_0`)))

(event `OnBulletHit_Event_0`
  (params (HitResult :type "HitResult Structure"))
  (`self.ProcessBulletHitSound` HitResult))

(event `PlayGunshotSound`
  (`GameplayStatics.PlaySoundAtLocation` self (`self.SFX_Gunshot`) (.location (`SceneComponent.GetSocketTransform` (`self.GunMeshComponent`) (`self.MuzzleSocketName`) "RTS_World")) (struct) (`KismetMathLibrary.RandomFloatInRange` 0.8 1.2) (`KismetMathLibrary.RandomFloatInRange` 0.9 1.1) 0.0 "/Game/FemaleShooter/Audio/DefautlSoundAttenuation.DefautlSoundAttenuation" null null))

(event `ProcessBulletHitSound`
  (params (HitResult :type "HitResult Structure"))
  (`GameplayStatics.PlaySoundAtLocation` self (`self.SFX_BulletHit`) (`.ImpactPoint` (`GameplayStatics.BreakHitResult` HitResult)) (struct) (`KismetMathLibrary.RandomFloatInRange` 2.0 3.0) (`KismetMathLibrary.RandomFloatInRange` 0.9 1.1) 0.0 "/Game/FemaleShooter/Audio/DefautlSoundAttenuation.DefautlSoundAttenuation" null null))

(event `UpdateSpinPivot`
  (set `self.TriggerSpinLocation` (`self.RetrieveTriggerSpinLocation`)))

(event `UpdateSpin`
  (bind _gunmeshcomponent (`self.GunMeshComponent`))
  (bind _triggerspinlocation (`self.TriggerSpinLocation`))
  (bind _returnvalue (`KismetMathLibrary.MakeRotator` (* (`self.GunSpinAngle`) -1.0)))
  (`|ExecutionSequence`
    (:`then_0`
      (if (`self.IsGunSpinning`)
        (set `self.GunSpinAngle` (mod (+ (`self.GunSpinAngle`) (`self.FloatStep` (`self.GunSpinSpeed`))) 360.0))
        (else
          (set `self.GunSpinAngle` 0.0))))
    (:`then_1`
      (`SceneComponent.K2_SetRelativeRotation` _gunmeshcomponent _returnvalue false false)
      (`SceneComponent.K2_SetRelativeLocation` _gunmeshcomponent (+ _triggerspinlocation (`KismetMathLibrary.GreaterGreater_VectorRotator` (* _triggerspinlocation -1.0) _returnvalue)) false false))))

(fn `FloatStep`
  (params (Input :type "Float (double-precision)"))
  (returns (Output :type "Float (double-precision)"))
  (bind _returnvalue (`GameplayStatics.GetWorldDeltaSeconds`))
  (return (/ (* Input (`self.ExpectedFPS`)) (/ 1.0 (select `bool` (> _returnvalue 0.0) :`false` 1.0 :`true` _returnvalue)))))

(fn `RetrieveTriggerSpinLocation`
  (returns (TriggerSpinLocation :type "Vector Structure"))
  (bind _gunmeshcomponent (`self.GunMeshComponent`))
  (bind _triggerspinsocketname (`self.TriggerSpinSocketName`))
  (`/Engine/EditorBlueprintResources/StandardMacros.IsValid` _gunmeshcomponent
    (:`Is Valid`
      (if (`SceneComponent.DoesSocketExist` _gunmeshcomponent _triggerspinsocketname)
        (return (.location (`SceneComponent.GetSocketTransform` _gunmeshcomponent _triggerspinsocketname "RTS_Component")))
        (else
          _)))
    (:`Is Not Valid`
      _))
  (return (0.0 0.0 0.0)))