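; Health component that tracks an actor's current and maximum health and manages its attached health bar.
; Damage and healing feed one clamped update, which fires OnZeroHealth whenever the result is zero.
; On BeginPlay it spawns a health bar actor on a mesh socket with an offset, finding the mesh by component name if none is set.
; It also exposes a full reset, show/hide for the bar and a health percentage getter.
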(event `TryAutoSetup`
  (`/Engine/EditorBlueprintResources/StandardMacros.IsValid` (`self.Mesh`)
    (:`Is Not Valid`
      (for _array_element (`Actor.K2_GetComponentsByClass` (`self.GetOwner`) "/Script/Engine.PrimitiveComponent")
        (if (`KismetStringLibrary.EqualEqual_StrStr` (`KismetSystemLibrary.GetObjectName` _array_element) (`self.MeshName`))
          (set `self.Mesh` _array_element)
          (break))))))

(event `Setup`
  (params (Mesh :type "PrimitiveComponent Object Reference") (Socket :type Name))
  (set `self.Mesh` Mesh)
  (set `self.Socket` Socket))

(event `SetupUI`
  (bind _mesh (`self.Mesh`))
  (`self.TryAutoSetup`)
  (`/Engine/EditorBlueprintResources/StandardMacros.IsValid` _mesh
    (:`Is Valid`
      (bind _returnvalue (`|SpawnActorFromClass` "/Game/FemaleShooter/Blueprint/Misc/HealthBarActor.HealthBarActor_C" (`KismetMathLibrary.MakeTransform` (0.0 0.0 0.0)) "AlwaysSpawn" "OverrideRootScale" null null))
      (`Actor.K2_AttachToComponent` _returnvalue _mesh (`self.Socket`) "SnapToTarget" "SnapToTarget" "SnapToTarget" true)
      (`SceneComponent.K2_AddLocalOffset` (`/Game/FemaleShooter/Blueprint/Misc/HealthBarActor.DefaultSceneRoot` _returnvalue) (`self.Offset`) false false)
      (`/Game/FemaleShooter/Blueprint/Misc/HealthBarActor.Setup` _returnvalue (`self.GetOwner`))
      (set `self.UIActor` _returnvalue)
      (`self.UpdateUIVisibility` (`self.IsShowUI`)))))

(event `SetupHealth`
  (params (Health :type Integer) (HealthMax :type Integer :default 100))
  (set `self.Health` Health)
  (set `self.HealthMax` HealthMax))

(event `self.ReceiveBeginPlay`
  (`self.SetupHealth` (`self.Health`) (`self.HealthMax`))
  (`self.SetupUI`))

(event `ReceiveHealth`
  (params (Value :type Integer))
  (`self.UpdateHealthPoint` (+ (`self.Health`) Value)))

(event `UpdateHealthPoint`
  (params (Value :type Integer))
  (bind _output_get (set `self.Health` (`KismetMathLibrary.Clamp` Value 0 (`self.HealthMax`))))
  (if (<= _output_get 0)
    (`self.OnZeroHealth`)))

(event `ReceiveDamage`
  (params (Value :type Integer))
  (`self.UpdateHealthPoint` (- (`self.Health`) Value)))

(event `UpdateUIVisibility`
  (params (IsVisible :type Boolean))
  (`/Game/FemaleShooter/Blueprint/Misc/HealthBarActor.UpdateVisibility` (`self.UIActor`) IsVisible))

(event `HideUI`
  (`self.UpdateUIVisibility` false))

(event `ResetToFullHealth`
  (set `self.Health` (`self.HealthMax`)))

(event `ShowUI`
  (`self.UpdateUIVisibility` true))

(fn `GetHealthPercentage`
  (returns (HealthPercentage :type "Float (double-precision)"))
  (bind _healthmax (`self.HealthMax`))
  (if (> _healthmax 0)
    (return (/ (`KismetMathLibrary.Conv_IntToDouble` (`self.Health`)) (`KismetMathLibrary.Conv_IntToDouble` _healthmax)))
    (else
      (return 0.0))))