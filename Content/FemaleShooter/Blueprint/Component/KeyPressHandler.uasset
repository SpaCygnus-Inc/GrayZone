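; KeyPressHandler is a pawn component that turns held WASD keys into keyboard movement events.
; On BeginPlay it stores a key-to-name map and binds its own OnKeyDown dispatcher to ProcessKey.
; Each tick it polls the owning pawn's PlayerController for every mapped key, bypassing input bindings, and fires OnKeyDown for those held.
; ProcessKey converts the names into signed forward or right dispatcher calls, leaving the movement itself to listeners.
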(event `self.ReceiveBeginPlay`
  (`self.SetupInput_KeyPressHandler`))

(event `self.ReceiveTick`
  (params (DeltaSeconds :type "Float (single-precision)"))
  (`self.UpdateInput`))

(event `UpdateInput`
  (bind _playercontroller (`self.RetrievePlayerController`))
  (`/Engine/EditorBlueprintResources/StandardMacros.IsValid` _playercontroller
    (:`Is Valid`
      (bind _keys (`BlueprintMapLibrary.Map_Keys` (`self.Map_InputName`)))
      (for _array_element _keys
        (if (`PlayerController.IsInputKeyDown` _playercontroller _array_element)
          (`self.OnKeyDown` _array_element (`BlueprintMapLibrary.Map_Find` (`self.Map_InputName`) _array_element)))))))

(event `Setup`
  (params (KeyMap :type "Map of Key Structure to Name"))
  (set `self.Map_InputName` KeyMap))

(event `SetupInput_KeyPressHandler`
  ;[0.3569 1 0.3843] Input - Movement (Keyboard)
  (`self.Setup` (`|MakeMap` "W" "W" "S" "S" "D" "D" "A" "A" :!type "Key Structure" :!valuetype "Name"))
  (add `self.OnKeyDown` (delegate `ProcessKey`)))

(event `ProcessKey` :!signature `self.OnKeyDown`
  (params (Key :type "Key Structure") (KeyName :type Name))
  ;[0.3569 1 0.3843] Input - Movement (Keyboard)
  (switch `name` KeyName
    (:`W`
      (`self.OnKeyboardMoveForward` 1.0))
    (:`S`
      (`self.OnKeyboardMoveForward` -1.0))
    (:`A`
      (`self.OnKeyboardMoveRight` -1.0))
    (:`D`
      (`self.OnKeyboardMoveRight` 1.0))))

(fn `RetrievePlayerController`
  (returns (PlayerController :type "PlayerController Object Reference"))
  (bind _aspawn (cast `Pawn` (`self.GetOwner`)))
  (bind _asplayer_controller (cast `PlayerController` (`Pawn.GetController` _aspawn)))
  (return _asplayer_controller))