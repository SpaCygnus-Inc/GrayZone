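; Character component that manages equipment as EquipmentInstance objects in a dictionary keyed by identifier, each holding an actor plus storage and equip socket names.
; Loading an equipment set removes, updates or adds entries according to a change option, then applies high-heel offsets to any HighHeelComponent.
; Actors spawned from class have their primitive component collision disabled.
; Pickup registers an existing actor, while drop detaches and returns it.
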(event `self.ReceiveBeginPlay`)

(event `SetupCharacter`
  ;[1 1 1] Setup Character Reference
  (`/Engine/EditorBlueprintResources/StandardMacros.IsValid` (`self.Character`)
    (:`Is Not Valid`
      (bind _ascharacter (cast `Character` (`self.GetOwner`)))
      (set `self.Character` _ascharacter))))

(event `LoadEquipmentSet`
  (params (EquipmentSet :type "/Game/FemaleShooter/Blueprint/Data/Equipment/EquipmentSet Object Reference") (EquipmentChangeOption :type "/Game/FemaleShooter/Blueprint/Enum/EquipmentChangeOption Enum" :default "NewEnumerator0") (IsForced :type Boolean))
  ;[1 1 1] Equipment
  (`/Engine/EditorBlueprintResources/StandardMacros.IsValid` EquipmentSet
    (:`Is Valid`
      (`|ExecutionSequence`
        (:`then_0`
          (`self.RemoveUnusedEquipmentData` EquipmentSet EquipmentChangeOption))
        (:`then_1`
          (set `self.EquipmentSet` EquipmentSet))
        (:`then_2`
          (for _array_element (`/Game/FemaleShooter/Blueprint/Data/Equipment/EquipmentSet.EquipmentList` (`self.EquipmentSet`))
            (`self.UpdateEquipmentFromData` _array_element EquipmentChangeOption)))
        (:`then_3`
          (`self.TryApplyHighHeelsSettings` EquipmentSet))
        (:`then_4`
          (`self.OnEquipmentUpdated`))))))

(event `TryApplyHighHeelsSettings`
  (params (EquipmentSet :type "/Game/FemaleShooter/Blueprint/Data/Equipment/EquipmentSet Object Reference"))
  (bind (_isapplysettings _heightoffset _rotationoffset) (break `/Game/FemaleShooter/Blueprint/Struct/HighHeelSharedData` (`/Game/FemaleShooter/Blueprint/Data/Equipment/EquipmentSet.HighHeelsSettings` EquipmentSet)))
  (bind _returnvalue (`Actor.GetComponentByClass` (`self.GetOwner`) "/Game/FemaleShooter/Blueprint/Component/HighHeelComponent.HighHeelComponent_C"))
  ;[1 1 1] Try Implement High Heels Setting
  (`/Engine/EditorBlueprintResources/StandardMacros.IsValid` _returnvalue
    (:`Is Valid`
      (set `/Game/FemaleShooter/Blueprint/Component/HighHeelComponent.HeightOffset` _heightoffset _returnvalue)
      (set `/Game/FemaleShooter/Blueprint/Component/HighHeelComponent.RotationOffset` _rotationoffset _returnvalue))))

(fn `DropEquipmentActor`
  (params (Identifier :type Name))
  (returns (DroppedEquipmentActor :type "Actor Object Reference"))
  (locals (DroppedActor :type "Actor Object Reference"))
  (bind _equipmentdict (`self.EquipmentDict`))
  (bind (_value _returnvalue) (`BlueprintMapLibrary.Map_Find` _equipmentdict Identifier))
  (bind _actor (`/Game/FemaleShooter/Blueprint/Misc/EquipmentInstance.Actor` _value))
  (if _returnvalue
    (`Actor.K2_DetachFromActor` _actor "KeepWorld" "KeepWorld" "KeepWorld")
    (set `local.DroppedActor` _actor)
    (set `/Game/FemaleShooter/Blueprint/Misc/EquipmentInstance.Actor` null _value)
    (`BlueprintMapLibrary.Map_Remove` _equipmentdict Identifier)
    (return (`local.DroppedActor`))
    (else
      (return null))))

(fn `GenerateEquipmentActorFromClass`
  (params (ActorClass :type "Actor Class Reference"))
  (returns (Actor :type "Actor Object Reference"))
  (if (`KismetSystemLibrary.IsValidClass` ActorClass)
    (bind _returnvalue (`|SpawnActorFromClass` ActorClass (`KismetMathLibrary.MakeTransform` (0.0 0.0 0.0)) "AlwaysSpawn" "OverrideRootScale" null null))
    (`PrimitiveComponent.SetCollisionEnabled` (`Actor.GetComponentByClass` _returnvalue "/Script/Engine.PrimitiveComponent") "NoCollision")
    (return _returnvalue)
    (else
      (return null))))

(fn `GenerateEquipmentFromActor`
  (params (EquipmentData :type "/Game/FemaleShooter/Blueprint/Struct/EquipmentDataStruct Structure") (Actor :type "Actor Object Reference"))
  (returns (Equipment :type "/Game/FemaleShooter/Blueprint/Misc/EquipmentInstance Object Reference"))
  (bind (_identifier _actorclass _storagesocketname _equipsocketname) (break `/Game/FemaleShooter/Blueprint/Struct/EquipmentDataStruct` EquipmentData))
  (`/Engine/EditorBlueprintResources/StandardMacros.IsValid` Actor
    (:`Is Valid`
      (`self.SetupCharacter`)
      (bind _returnvalue (`|GenericCreateObject` "/Game/FemaleShooter/Blueprint/Misc/EquipmentInstance.EquipmentInstance_C" self _identifier Actor (`GameplayStatics.GetObjectClass` Actor) _storagesocketname _equipsocketname))
      (`/Game/FemaleShooter/Blueprint/Misc/EquipmentInstance.CharacterStorage` _returnvalue (`self.Character`))
      (`BlueprintMapLibrary.Map_Add` (`self.EquipmentDict`) (`/Game/FemaleShooter/Blueprint/Misc/EquipmentInstance.Identifier` _returnvalue) _returnvalue)
      (return _returnvalue))
    (:`Is Not Valid`
      (return null))))

(fn `GenerateEquipmentFromData`
  (params (EquipmentData :type "/Game/FemaleShooter/Blueprint/Struct/EquipmentDataStruct Structure"))
  (returns (Equipment :type "/Game/FemaleShooter/Blueprint/Misc/EquipmentInstance Object Reference"))
  (bind (_identifier _actorclass _storagesocketname _equipsocketname) (break `/Game/FemaleShooter/Blueprint/Struct/EquipmentDataStruct` EquipmentData))
  (`self.SetupCharacter`)
  (if (`KismetSystemLibrary.IsValidClass` _actorclass)
    (bind _actor (`self.GenerateEquipmentActorFromClass` _actorclass))
    (bind _returnvalue (`|GenericCreateObject` "/Game/FemaleShooter/Blueprint/Misc/EquipmentInstance.EquipmentInstance_C" self _identifier _actor _actorclass _storagesocketname _equipsocketname))
    (`/Game/FemaleShooter/Blueprint/Misc/EquipmentInstance.CharacterStorage` _returnvalue (`self.Character`))
    (`BlueprintMapLibrary.Map_Add` (`self.EquipmentDict`) (`/Game/FemaleShooter/Blueprint/Misc/EquipmentInstance.Identifier` _returnvalue) _returnvalue)
    (return _returnvalue)
    (else
      (return null))))

(fn `GetBatchedEquipments`
  (params (EquipmentNames :type "Array of Name"))
  (returns (EquipmentList :type "Array of /Game/FemaleShooter/Blueprint/Misc/EquipmentInstance Object Reference"))
  (locals (TempEquipmentList :type "Array of /Game/FemaleShooter/Blueprint/Misc/EquipmentInstance Object Reference"))
  (for (_array_element _array_index) EquipmentNames
    (`KismetArrayLibrary.Array_Set` (`local.TempEquipmentList`) _array_index (`BlueprintMapLibrary.Map_Find` (`self.EquipmentDict`) _array_element) true))
  (return (`local.TempEquipmentList`)))

(fn `GetEquipment`
  (params (EquipmentName :type Name))
  (returns (Equipment :type "/Game/FemaleShooter/Blueprint/Misc/EquipmentInstance Object Reference") (IsFound :type Boolean))
  (bind (_value _returnvalue) (`BlueprintMapLibrary.Map_Find` (`self.EquipmentDict`) EquipmentName))
  (return _value _returnvalue))

(fn `PickupEquipmentActor`
  (params (Actor :type "Actor Object Reference") (Identifier :type Name) (StorageSocketName :type Name) (EquipSocketName :type Name))
  (`/Engine/EditorBlueprintResources/StandardMacros.IsValid` Actor
    (:`Is Valid`
      (`self.UpdateEquipmentFromData` (make `/Game/FemaleShooter/Blueprint/Struct/EquipmentDataStruct` Identifier (`GameplayStatics.GetObjectClass` Actor) StorageSocketName EquipSocketName) "NewEnumerator2" Actor))))

(fn `RemoveUnusedEquipmentData`
  (params (ReferenceEquipmentSet :type "/Game/FemaleShooter/Blueprint/Data/Equipment/EquipmentSet Object Reference") (EquipmentChangeOption :type "/Game/FemaleShooter/Blueprint/Enum/EquipmentChangeOption Enum" :default "NewEnumerator0"))
  (locals (IsFound :type Boolean) (NewEquipmentSet :type "/Game/FemaleShooter/Blueprint/Data/Equipment/EquipmentSet Object Reference") (OldEquipmentSet :type "/Game/FemaleShooter/Blueprint/Data/Equipment/EquipmentSet Object Reference") (OldIdentifier :type Name) (NewIdentifier :type Name))
  (bind _equipmentdict (`self.EquipmentDict`))
  (bind _value (`BlueprintMapLibrary.Map_Find` _equipmentdict (`local.OldIdentifier`)))
  (bind _actor (`/Game/FemaleShooter/Blueprint/Misc/EquipmentInstance.Actor` _value))
  (switch `/Game/FemaleShooter/Blueprint/Enum/EquipmentChangeOption` EquipmentChangeOption
    (:`NewEnumerator0`
      (`|ExecutionSequence`
        (:`then_0`
          (set `local.OldEquipmentSet` (`self.EquipmentSet`))
          (set `local.NewEquipmentSet` ReferenceEquipmentSet))
        (:`then_1`
          (`/Engine/EditorBlueprintResources/StandardMacros.IsValid` (`local.OldEquipmentSet`)
            (:`Is Valid`
              (for _array_element (`/Game/FemaleShooter/Blueprint/Data/Equipment/EquipmentSet.EquipmentList` (`local.OldEquipmentSet`))
                (set `local.IsFound` false)
                (set `local.OldIdentifier` (`.Identifier_2_6416B9F1420E5404C109398FB0603114` (break `/Game/FemaleShooter/Blueprint/Struct/EquipmentDataStruct` _array_element)))
                (for _array_element_2 (`/Game/FemaleShooter/Blueprint/Data/Equipment/EquipmentSet.EquipmentList` (`local.NewEquipmentSet`))
                  (set `local.NewIdentifier` (`.Identifier_2_6416B9F1420E5404C109398FB0603114` (break `/Game/FemaleShooter/Blueprint/Struct/EquipmentDataStruct` _array_element_2)))
                  (if (== (`local.OldIdentifier`) (`local.NewIdentifier`))
                    (set `local.IsFound` true)
                    (break)))
                (if (not (`local.IsFound`))
                  (`Actor.K2_DetachFromActor` _actor "KeepWorld" "KeepWorld" "KeepWorld")
                  (`Actor.K2_DestroyActor` _actor)
                  (set `/Game/FemaleShooter/Blueprint/Misc/EquipmentInstance.Actor` null _value)
                  (`BlueprintMapLibrary.Map_Remove` _equipmentdict (`local.OldIdentifier`)))))))))))

(fn `UpdateEquipmentActor`
  (params (Equipment :type "/Game/FemaleShooter/Blueprint/Misc/EquipmentInstance Object Reference") (NewActor :type "Actor Object Reference"))
  (bind _actor (`/Game/FemaleShooter/Blueprint/Misc/EquipmentInstance.Actor` Equipment))
  (`self.SetupCharacter`)
  (`/Engine/EditorBlueprintResources/StandardMacros.IsValid` NewActor
    (:`Is Valid`
      (`|ExecutionSequence`
        (:`then_0`
          (`Actor.K2_DetachFromActor` _actor "KeepWorld" "KeepWorld" "KeepWorld")
          (`Actor.K2_DestroyActor` _actor))
        (:`then_1`
          (set `/Game/FemaleShooter/Blueprint/Misc/EquipmentInstance.Actor` NewActor Equipment)
          (`/Game/FemaleShooter/Blueprint/Misc/EquipmentInstance.UpdateInstance` Equipment))))))

(fn `UpdateEquipmentActorFromClass`
  (params (Equipment :type "/Game/FemaleShooter/Blueprint/Misc/EquipmentInstance Object Reference") (ActorClass :type "Actor Class Reference"))
  (bind _actor (`/Game/FemaleShooter/Blueprint/Misc/EquipmentInstance.Actor` Equipment))
  (`self.SetupCharacter`)
  (bind _actor_2 (`self.GenerateEquipmentActorFromClass` ActorClass))
  (`/Engine/EditorBlueprintResources/StandardMacros.IsValid` _actor_2
    (:`Is Valid`
      (`|ExecutionSequence`
        (:`then_0`
          (`Actor.K2_DetachFromActor` _actor "KeepWorld" "KeepWorld" "KeepWorld")
          (`Actor.K2_DestroyActor` _actor))
        (:`then_1`
          (set `/Game/FemaleShooter/Blueprint/Misc/EquipmentInstance.Actor` _actor_2 Equipment)
          (`/Game/FemaleShooter/Blueprint/Misc/EquipmentInstance.UpdateInstance` Equipment))))))

(fn `UpdateEquipmentFromData`
  (params (EquipmentData :type "/Game/FemaleShooter/Blueprint/Struct/EquipmentDataStruct Structure") (EquipmentChangeOption :type "/Game/FemaleShooter/Blueprint/Enum/EquipmentChangeOption Enum" :default "NewEnumerator0") (NewActor :type "Actor Object Reference"))
  (returns (Equipment :type "/Game/FemaleShooter/Blueprint/Misc/EquipmentInstance Object Reference"))
  (bind (_identifier _actorclass _storagesocketname _equipsocketname) (break `/Game/FemaleShooter/Blueprint/Struct/EquipmentDataStruct` EquipmentData))
  (bind (_value _returnvalue) (`BlueprintMapLibrary.Map_Find` (`self.EquipmentDict`) _identifier))
  (if (`KismetSystemLibrary.IsValidClass` _actorclass)
    (if _returnvalue
      (switch `/Game/FemaleShooter/Blueprint/Enum/EquipmentChangeOption` EquipmentChangeOption
        (:`NewEnumerator0`
          _)
        (:`NewEnumerator2`
          _)
        (:`NewEnumerator1`
          (return _value)))
      (`/Game/FemaleShooter/Blueprint/Misc/EquipmentInstance.UpdateData` _value _actorclass _storagesocketname _equipsocketname)
      (`/Engine/EditorBlueprintResources/StandardMacros.IsValid` NewActor
        (:`Is Valid`
          (`self.UpdateEquipmentActor` _value NewActor))
        (:`Is Not Valid`
          (`self.UpdateEquipmentActorFromClass` _value _actorclass)))
      (return _value)
      (else
        (`/Engine/EditorBlueprintResources/StandardMacros.IsValid` NewActor
          (:`Is Valid`
            (bind _equipment (`self.GenerateEquipmentFromActor` EquipmentData NewActor))
            (return _equipment))
          (:`Is Not Valid`
            (bind _equipment_2 (`self.GenerateEquipmentFromData` EquipmentData))
            (return _equipment_2)))))
    (else
      (return null))))