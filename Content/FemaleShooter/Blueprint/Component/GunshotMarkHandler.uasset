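; Gunshot mark handler component that places bullet-mark decals on the mesh given in Setup and fades them out over time.
; ReceiveShot attaches a decal with its own dynamic material, aligned to the impact normal, then calls OnShotReceived.
; Each Tick counts down every mark's display time, fades its Alpha parameter, then destroys it.
; Map IDs are recycled through PoolList; decal components themselves are created fresh per shot.
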(event `Setup`
  (params (MeshComponent :type "PrimitiveComponent Object Reference"))
  (set `self.MeshComponent` MeshComponent))

(event `self.ReceiveTick`
  (params (DeltaSeconds :type "Float (single-precision)"))
  (`self.UpdateDecals`))

(fn `ReceiveShot`
  (params (ImpactPoint :type "Vector Structure") (HitResult :type "HitResult Structure"))
  (locals (TempIndex :type Integer))
  (bind _meshcomponent (`self.MeshComponent`))
  (bind _poollist (`self.PoolList`))
  (bind _tempindex (`local.TempIndex`))
  (bind _returnvalue (`KismetArrayLibrary.Array_LastIndex` _poollist))
  (`|ExecutionSequence`
    (:`then_0`
      (`/Engine/EditorBlueprintResources/StandardMacros.IsValid` _meshcomponent
        (:`Is Valid`
          (bind _returnvalue_2 (`KismetMaterialLibrary.CreateDynamicMaterialInstance` "/Game/FemaleShooter/Asset/GunMark/Img_GunMark_Mat.Img_GunMark_Mat"))
          (bind _returnvalue_3 (`GameplayStatics.SpawnDecalAttached` _returnvalue_2 (20.0 20.0 20.0) _meshcomponent "None" ImpactPoint (`KismetMathLibrary.Conv_VectorToRotator` (`.ImpactNormal` (`GameplayStatics.BreakHitResult` HitResult))) "KeepWorldPosition"))
          (`DecalComponent.SetFadeScreenSize` _returnvalue_3 0.0)
          (`|ExecutionSequence`
            (:`then_0`
              (if (> (`KismetArrayLibrary.Array_Length` (`self.PoolList`)) 0)
                (set `local.TempIndex` (`|GetArrayItem` _poollist _returnvalue))
                (`KismetArrayLibrary.Array_Remove` _poollist _returnvalue)
                (else
                  (set `local.TempIndex` (`self.GeneratedAmount`))
                  (`/Engine/EditorBlueprintResources/StandardMacros.IncrementInt` (`self.GeneratedAmount`)))))
            (:`then_1`
              (`BlueprintMapLibrary.Map_Add` (`self.DecalMap`) _tempindex)
              (`BlueprintMapLibrary.Map_Add` (`self.DecalMap`) _tempindex (make `/Game/FemaleShooter/Blueprint/Struct/DecalData` _tempindex))
              (`BlueprintMapLibrary.Map_Add` (`self.DecalActorMap`) _tempindex)
              (`BlueprintMapLibrary.Map_Add` (`self.DecalActorMap`) _tempindex (make `/Game/FemaleShooter/Blueprint/Struct/DecalActorData` _tempindex _returnvalue_3 _returnvalue_2)))))))
    (:`then_1`
      (`self.OnShotReceived` ImpactPoint HitResult))))

(fn `UpdateDecals`
  (locals (RemovedList :type "Array of Integer") (TempList :type "Array of Integer"))
  (bind _returnvalue (`GameplayStatics.GetWorldDeltaSeconds`))
  (`KismetArrayLibrary.Array_Clear` (`local.RemovedList`))
  (bind _keys (`BlueprintMapLibrary.Map_Keys` (`self.DecalMap`)))
  (bind _output_get (set `local.TempList` _keys))
  (`|ExecutionSequence`
    (:`then_0`
      (for _array_element _output_get
        (bind _value (`BlueprintMapLibrary.Map_Find` (`self.DecalMap`) _array_element))
        (bind (_id _appeartime _fadetime _fadecount) (break `/Game/FemaleShooter/Blueprint/Struct/DecalData` _value))
        (bind _returnvalue_2 (`KismetMathLibrary.FClamp` (- _appeartime _returnvalue) 0.0 _appeartime))
        (if (> _returnvalue_2 0.0)
          (bind _structout (setmembers `/Game/FemaleShooter/Blueprint/Struct/DecalData` :`StructRef` _value :`AppearTime` _returnvalue_2))
          (`BlueprintMapLibrary.Map_Add` (`self.DecalMap`) _array_element _structout)
          (else
            (bind _returnvalue_3 (- _fadecount _returnvalue))
            (bind _returnvalue_4 (`KismetMathLibrary.FClamp` _returnvalue_3 0.0 _returnvalue_3))
            (if (> _returnvalue_4 0.0)
              (bind _structout_2 (setmembers `/Game/FemaleShooter/Blueprint/Struct/DecalData` :`StructRef` _value :`AppearTime` 0.0 :`FadeCount` _returnvalue_4))
              (`BlueprintMapLibrary.Map_Add` (`self.DecalMap`) _array_element _structout_2)
              (bind (_id_2 _decalcomponent _decalmaterial) (break `/Game/FemaleShooter/Blueprint/Struct/DecalActorData` (`BlueprintMapLibrary.Map_Find` (`self.DecalActorMap`) _array_element)))
              (`MaterialInstanceDynamic.SetScalarParameterValue` _decalmaterial "Alpha" (`KismetMathLibrary.FClamp` (/ _returnvalue_4 _fadetime)))
              (else
                (`SceneComponent.K2_DetachFromComponent` _decalcomponent "KeepRelative" "KeepRelative" "KeepRelative" true)
                (`self.K2_DestroyComponent` _decalcomponent)
                (bind _structout_3 (setmembers `/Game/FemaleShooter/Blueprint/Struct/DecalData` :`StructRef` _value :`AppearTime` 0.0 :`FadeTime` 0.0 :`FadeCount` 1.0))
                (`BlueprintMapLibrary.Map_Add` (`self.DecalMap`) _array_element _structout_3)
                (`KismetArrayLibrary.Array_Add` (`local.RemovedList`) _array_element)))))))
    (:`then_1`
      (bind (_arrayindex _arrayelement) (`/Engine/EditorBlueprintResources/StandardMacros.ReverseForEachLoop` (`local.RemovedList`))
        (:`LoopBody`
          (bind _id_3 (break `/Game/FemaleShooter/Blueprint/Struct/DecalData` (`BlueprintMapLibrary.Map_Find` (`self.DecalMap`) _arrayelement)))
          (`KismetArrayLibrary.Array_Add` (`self.PoolList`) _id_3)
          (`BlueprintMapLibrary.Map_Remove` (`self.DecalActorMap`) _id_3)
          (`BlueprintMapLibrary.Map_Remove` (`self.DecalMap`) _id_3))))))