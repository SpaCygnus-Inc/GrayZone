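; UI controller component that drives menu navigation, panel switching and screen display settings.
; Each tick it polls mapped keyboard and gamepad keys, using press states and element-defined repeat intervals to trigger navigation, confirm, cancel and menu actions.
; A pointer stack tracks focus and parent panels for back navigation, alongside a hidden-panel stack that restores visibility.
; Focusing moves the mouse cursor to the element, and showing panels toggles game/UI input mode.
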(event `UpdateNavInterval`
  (bind (_navupinterval _navdowninterval _navleftinterval _navrightinterval) (break `/Game/FemaleShooter/Blueprint/Struct/UI/UI_NavInterval` (`self.CurrentNavInterval`)))
  ;[1 1 1] Update Navigation Delay/Interval
  (set `self.CurrentNavInterval` (make `/Game/FemaleShooter/Blueprint/Struct/UI/UI_NavInterval` (`self.FloatTimerUpdate` _navupinterval) (`self.FloatTimerUpdate` _navdowninterval) (`self.FloatTimerUpdate` _navleftinterval) (`self.FloatTimerUpdate` _navrightinterval))))

(event `SetupInput`
  ;[1 1 1] Setup Keys
  (set `self.Map_InputName` (`|MakeMap` "W" "W" "S" "S" "D" "D" "A" "A" "Up" "Up" "Down" "Down" "Left" "Left" "Right" "Right" "Gamepad_DPad_Up" "DPadUp" "Gamepad_DPad_Down" "DPadDown" "Gamepad_DPad_Left" "DPadLeft" "Gamepad_DPad_Right" "DPadRight" "Enter" "Enter" "Gamepad_FaceButton_Bottom" "GamepadConfirm" "Gamepad_FaceButton_Right" "GamepadCancel" "Escape" "Escape" "Gamepad_Special_Right" "GamepadSpecialRight" "Gamepad_LeftStick_Up" "LeftStickUp" "Gamepad_LeftStick_Down" "LeftStickDown" "Gamepad_LeftStick_Right" "LeftStickRight" "Gamepad_LeftStick_Left" "LeftStickLeft" "BackSpace" "Backspace" :!type "Key Structure" :!valuetype "Name"))
  (`self.SetupKeyStates` (`|MakeArray` "GamepadConfirm" "GamepadCancel" "Enter" "Escape" "GamepadSpecialRight" "Backspace" :!type "Name")))

(event `SetupDefaultWidget`
  (bind _defaultuserwidget (`self.DefaultUserWidget`))
  ;[1 1 1] Setup Default Widget
  (if (`KismetSystemLibrary.IsValidClass` _defaultuserwidget)
    (bind _widget (`self.RegisterPanel` "Default" _defaultuserwidget))
    (`self.SwitchWidget` _widget (`|MakeArray`) (select `/Game/FemaleShooter/Blueprint/Enum/InputMode` (`self.InputMode`) :`NewEnumerator0` true))))

(event `Internal_UpdateWidgetsVisibility`
  (params (WidgetList :type "Array of Widget Object Reference") (IsValid :type Boolean))
  ;[1 1 1] Widget Visibility
  (for _array_element WidgetList
    (`/Engine/EditorBlueprintResources/StandardMacros.IsValid` _array_element
      (:`Is Valid`
        (`Widget.SetVisibility` _array_element (select `bool` IsValid :`false` "Hidden" :`true` "Visible" :!type "ESlateVisibility Enum"))))))

(event `self.ReceiveBeginPlay`
  ;[1 1 1] Begin Play and Tick
  (if (`self.IsUIActive`)
    (`self.SetupScreenDisplay`)
    (`self.SetupInput`)
    (`self.SetupDefaultWidget`)))

(event `self.ReceiveTick`
  (params (DeltaSeconds :type "Float (single-precision)"))
  ;[1 1 1] Begin Play and Tick
  (if (`self.IsUIActive`)
    (`self.UpdateNavInterval`)
    (`self.UpdateInput`)))

(event `SetupKeyStates`
  (params (KeyList :type "Array of Name"))
  ;[1 1 1] Setup Keys
  (for _array_element KeyList
    (`BlueprintMapLibrary.Map_Add` (`self.KeyPressStatus`) _array_element (make `/Game/FemaleShooter/Blueprint/Struct/UI/KeyState` false))))

(event `HideWidgets`
  (params (WidgetList :type "Array of Widget Object Reference"))
  ;[1 1 1] Widget Visibility
  (`self.Internal_UpdateWidgetsVisibility` WidgetList))

(event `ShowWidgets`
  (params (WidgetList :type "Array of Widget Object Reference"))
  ;[1 1 1] Widget Visibility
  (`self.Internal_UpdateWidgetsVisibility` WidgetList true))

(event `UpdateWidgetsVisibility`
  (params (HiddenWidgets :type "Array of Widget Object Reference") (ShowWidgets :type "Array of Widget Object Reference"))
  ;[1 1 1] Widget Visibility
  (`self.HideWidgets` HiddenWidgets)
  (`self.ShowWidgets` ShowWidgets))

(event `ChildWidget`
  (params (Widget :type "Widget Object Reference") (HiddenWidgetList :type "Array of Widget Object Reference") (IsHUD :type Boolean))
  ;[1 1 1] ChildWidget
  (`KismetArrayLibrary.Array_Add` (`self.HiddenPanelList`) (make `/Game/FemaleShooter/Blueprint/Struct/UI/UI_HiddenPanels` HiddenWidgetList))
  (bind _pointer (`/Game/FemaleShooter/Blueprint/Misc/UILib.GetDefaultFocus` Widget))
  (`KismetArrayLibrary.Array_Add` (`self.UIPointerList`) _pointer)
  (`self.SwitchWidget` Widget HiddenWidgetList IsHUD))

(event `UpdateScreenMode`
  (params (ScreenMode :type "EWindowMode Enum" :default "Fullscreen"))
  ;[1 1 1] Display Setup
  (set `self.ScreenMode` ScreenMode)
  (`self.UpdateScreenDisplay`))

(event `UpdateScreenResolution`
  (params (ScreenResolution :type "IntPoint Structure"))
  ;[1 1 1] Display Setup
  (set `self.ScreenResolution` ScreenResolution)
  (`self.UpdateScreenDisplay`))

(event `UpdateScreenDisplay`
  ;[1 1 1] Display Setup
  (`/Game/FemaleShooter/Blueprint/Misc/ZenLib.UpdateScreenDisplay` (`self.ScreenMode`) (`self.ScreenResolution`)))

(event `UpdateCurrentPointer`
  (params (Pointer :type "/Game/FemaleShooter/Blueprint/Struct/UI/UI_Pointer Structure"))
  (bind _uipointerlist (`self.UIPointerList`))
  ;[1 1 1] Update Pointer
  (`KismetArrayLibrary.Array_Set` _uipointerlist (select `bool` (< (`KismetArrayLibrary.Array_Length` _uipointerlist) 1) :`false` (`KismetArrayLibrary.Array_LastIndex` _uipointerlist)) Pointer true))

(event `ActivateMenuInput`
  (params (IsActive :type Boolean) (FocusedWidget :type "Widget Object Reference"))
  (bind _returnvalue (`GameplayStatics.GetPlayerController` 0))
  ;[1 1 1] Activate Menu Input
  (bind _output_get (set `self.IsMenuInputActive` IsActive))
  (bind _output_get_2 (set `PlayerController.bShowMouseCursor` _output_get _returnvalue))
  (if _output_get_2
    (`WidgetBlueprintLibrary.SetInputMode_GameAndUIEx` _returnvalue FocusedWidget)
    (else
      (`WidgetBlueprintLibrary.SetInputMode_GameOnly` _returnvalue))))

(event `SetupScreenDisplay`
  (bind _screenresolution (`self.ScreenResolution`))
  ;[1 1 1] Display Setup
  (`|ExecutionSequence`
    (:`then_0`
      (bind _resolutions (`KismetSystemLibrary.GetSupportedFullscreenResolutions`))
      (set `self.ResolutionList` _resolutions))
    (:`then_1`
      (if (not (`self.IsOverwriteDisplaySettingsAtBeginning`))
        (`self.StartWithDefaultResolution`)))
    (:`then_2`
      (if (not (>= (`KismetArrayLibrary.Array_Find` (`self.ResolutionList`) _screenresolution) 0))
        (`self.AddCustomResolution` _screenresolution)))
    (:`then_3`
      (`self.UpdateScreenDisplay`))))

(event `UpdateInput`
  (bind _returnvalue (`GameplayStatics.GetPlayerController` 0))
  ;[1 1 1] Update Input
  (`/Engine/EditorBlueprintResources/StandardMacros.IsValid` _returnvalue
    (:`Is Valid`
      (bind _keys (`BlueprintMapLibrary.Map_Keys` (`self.Map_InputName`)))
      (for _array_element _keys
        (if (`PlayerController.IsInputKeyDown` _returnvalue _array_element)
          (bind _value (`BlueprintMapLibrary.Map_Find` (`self.Map_InputName`) _array_element))
          (`self.KeyDown` _array_element _value)
          (`self.TryKeyPress` _array_element _value)
          (else
            (`self.KeyUp` _array_element _value)
            (`self.TryKeyRelease` _array_element _value)))))))

(event `SwitchWidget`
  (params (Widget :type "Widget Object Reference") (HiddenWidgetList :type "Array of Widget Object Reference") (IsHUD :type Boolean))
  ;[1 1 1] SwitchWidget2
  (`|ExecutionSequence`
    (:`then_0`
      (`self.RestoreHiddenPanels`)
      (`KismetArrayLibrary.Array_Add` (`self.HiddenPanelList`) (make `/Game/FemaleShooter/Blueprint/Struct/UI/UI_HiddenPanels` HiddenWidgetList)))
    (:`then_1`
      (for _array_element HiddenWidgetList
        (`/Engine/EditorBlueprintResources/StandardMacros.IsValid` _array_element
          (:`Is Valid`
            (`Widget.SetVisibility` _array_element "Hidden")))))
    (:`then_2`
      (`Widget.SetVisibility` Widget "Visible"))
    (:`then_3`
      (`self.ActivateMenuInput` (not IsHUD) Widget))
    (:`then_4`
      (bind _pointer (`/Game/FemaleShooter/Blueprint/Misc/UILib.GetDefaultFocus` Widget))
      (bind _structout (setmembers `/Game/FemaleShooter/Blueprint/Struct/UI/UI_Pointer` :`StructRef` _pointer :`IsHUD` IsHUD))
      (`self.FocusOnElement` _structout))
    (:`then_5`
      (bind _asuser_widget (cast `UserWidget` Widget))
      (if (not (`Widget.IsInViewport` _asuser_widget))
        (`UserWidget.AddToViewport` _asuser_widget 0)))))

(event `MoveFocusLeft`
  ;[1 1 1] Move Focus
  (bind _resultpointer (`/Game/FemaleShooter/Blueprint/Misc/UILib.GetFocusLeft` (`self.ActivePointer`)))
  (`self.FocusOnElement` _resultpointer))

(event `KeyDown`
  (params (Key :type "Key Structure") (KeyName :type Name))
  (bind _keypressstatus (`self.KeyPressStatus`))
  (bind (_value _returnvalue) (`BlueprintMapLibrary.Map_Find` _keypressstatus KeyName))
  ;[1 1 1] Key Down
  (if _returnvalue
    (bind _structout (setmembers `/Game/FemaleShooter/Blueprint/Struct/UI/KeyState` :`StructRef` _value :`IsDown` true :`IsPressed` (select `bool` (`.IsDown_1_7BF6F0C34955B5A0EC587B8AC892CB8C` (break `/Game/FemaleShooter/Blueprint/Struct/UI/KeyState` _value)) :`false` true) :`IsReleased` false))
    (`BlueprintMapLibrary.Map_Add` _keypressstatus KeyName _structout)))

(event `ConfirmPressed`
  (bind (_isvalid _container _activeelement _activeindex _ishud _containerwidget _elementwidget) (break `/Game/FemaleShooter/Blueprint/Struct/UI/UI_Pointer` (`self.ActivePointer`)))
  ;[1 1 1] Confirm Pressed
  (`/Engine/EditorBlueprintResources/StandardMacros.IsValid` _elementwidget
    (:`Is Valid`
      (bind _isprocessed (`/Game/FemaleShooter/Blueprint/Interface/I_GunnerGirl_UIElement.ConfirmPressed` _activeelement))
      (if (not _isprocessed)
        (`/Game/FemaleShooter/Blueprint/Interface/I_GunnerGirl_UIContainer.ConfirmPressed` _container _activeelement _elementwidget :!label _label)))
    (:`Is Not Valid`
      (goto _label))))

(event `FocusOnElement`
  (params (UIPointer :type "/Game/FemaleShooter/Blueprint/Struct/UI/UI_Pointer Structure"))
  (bind (_isvalid _container _activeelement _activeindex _ishud _containerwidget _elementwidget) (break `/Game/FemaleShooter/Blueprint/Struct/UI/UI_Pointer` UIPointer))
  ;[1 1 1] Focus on Element
  (`|ExecutionSequence`
    (:`then_0`
      (`self.UpdateCurrentPointer` UIPointer))
    (:`then_1`
      (if _isvalid
        (`KismetSystemLibrary.Delay` 0.06)
        (`/Engine/EditorBlueprintResources/StandardMacros.IsValid` _elementwidget
          (:`Is Valid`
            (bind _widget (`/Game/FemaleShooter/Blueprint/Interface/I_GunnerGirl_UIElement.GetWidget` _activeelement))
            (`/Engine/EditorBlueprintResources/StandardMacros.IsValid` _widget
              (:`Is Valid`
                (bind _location (`/Game/FemaleShooter/Blueprint/Interface/I_GunnerGirl_UIElement.GetLocation` _activeelement))
                (bind (_x _y) (`KismetMathLibrary.BreakVector2D` _location))
                (`PlayerController.SetMouseLocation` (`GameplayStatics.GetPlayerController` 0) (`KismetMathLibrary.FTrunc` _x) (`KismetMathLibrary.FTrunc` _y))))))))))

(event `MoveFocusRight`
  ;[1 1 1] Move Focus
  (bind _resultpointer (`/Game/FemaleShooter/Blueprint/Misc/UILib.GetFocusRight` (`self.ActivePointer`)))
  (`self.FocusOnElement` _resultpointer))

(event `TryKeyPress`
  (params (Key :type "Key Structure") (Name :type Name))
  (bind (_isvalid _container _activeelement _activeindex _ishud _containerwidget _elementwidget) (break `/Game/FemaleShooter/Blueprint/Struct/UI/UI_Pointer` (`self.ActivePointer`)))
  (bind _returnvalue (`KismetSystemLibrary.IsValid` _elementwidget))
  ;[1 1 1] KeyPress
  (if (`self.ConfirmInputAllowed` Name)
    (`|ExecutionSequence`
      (:`then_0`
        (`self.SwitchOnKey` Name
          (:`UP`
            (if _returnvalue
              (`/Game/FemaleShooter/Blueprint/Interface/I_GunnerGirl_UIElement.NavUpPressed` _activeelement)))
          (:`DOWN`
            (if _returnvalue
              (`/Game/FemaleShooter/Blueprint/Interface/I_GunnerGirl_UIElement.NavDownPressed` _activeelement)))
          (:`LEFT`
            (if _returnvalue
              (`/Game/FemaleShooter/Blueprint/Interface/I_GunnerGirl_UIElement.NavLeftPressed` _activeelement)))
          (:`RIGHT`
            (if _returnvalue
              (`/Game/FemaleShooter/Blueprint/Interface/I_GunnerGirl_UIElement.NavRightPressed` _activeelement)))
          (:`CONFIRM`
            (`self.ConfirmPressed`))
          (:`CANCEL`
            (`self.CancelPressed`))
          (:`MENU`
            (`self.MenuPressed`))))
      (:`then_1`
        (if _returnvalue
          (bind _navinterval (`/Game/FemaleShooter/Blueprint/Interface/I_GunnerGirl_UIElement.GetNavInterval` _activeelement))
          (set `self.CurrentNavInterval` _navinterval))))))

(event `MoveFocusUp`
  ;[1 1 1] Move Focus
  (bind _resultpointer (`/Game/FemaleShooter/Blueprint/Misc/UILib.GetFocusAbove` (`self.ActivePointer`)))
  (`self.FocusOnElement` _resultpointer))

(event `KeyUp`
  (params (Key :type "Key Structure") (KeyName :type Name))
  (bind _keypressstatus (`self.KeyPressStatus`))
  (bind (_value _returnvalue) (`BlueprintMapLibrary.Map_Find` _keypressstatus KeyName))
  ;[1 1 1] Key Up
  (if _returnvalue
    (bind _structout (setmembers `/Game/FemaleShooter/Blueprint/Struct/UI/KeyState` :`StructRef` _value :`IsDown` false :`IsPressed` false :`IsReleased` (select `bool` (`.IsDown_1_7BF6F0C34955B5A0EC587B8AC892CB8C` (break `/Game/FemaleShooter/Blueprint/Struct/UI/KeyState` _value)) :`true` true)))
    (`BlueprintMapLibrary.Map_Add` _keypressstatus KeyName _structout)))

(event `MoveFocusDown`
  ;[1 1 1] Move Focus
  (bind _resultpointer (`/Game/FemaleShooter/Blueprint/Misc/UILib.GetFocusBelow` (`self.ActivePointer`)))
  (`self.FocusOnElement` _resultpointer))

(event `CancelPressed`
  (bind (_isvalid _container _activeelement _activeindex _ishud _containerwidget) (break `/Game/FemaleShooter/Blueprint/Struct/UI/UI_Pointer` (`self.ActivePointer`)))
  ;[1 1 1] Cancel Pressed
  (`/Engine/EditorBlueprintResources/StandardMacros.IsValid` _containerwidget
    (:`Is Valid`
      (bind _isprocessed (`/Game/FemaleShooter/Blueprint/Interface/I_GunnerGirl_UIContainer.BackPressed` _container))
      (if (not _isprocessed)
        (`self.ParentWidget` :!label _label_2)))
    (:`Is Not Valid`
      (goto _label_2))))

(event `MenuPressed`
  ;[1 1 1] Menu Pressed
  (`self.CancelPressed`))

(event `TryKeyRelease`
  (params (Key :type "Key Structure") (KeyName :type Name))
  ;[1 1 1] KeyRelease (Not Implemented Yet)
)

(fn `AddCustomResolution`
  (params (Resolution :type "IntPoint Structure"))
  (locals (IsAdded :type Boolean))
  (bind (_x _y) (break `IntPoint` Resolution))
  (bind _resolutionlist (`self.ResolutionList`))
  (`|ExecutionSequence`
    (:`then_0`
      (for (_array_element _array_index) _resolutionlist
        (bind (_x_2 _y_2) (break `IntPoint` _array_element))
        (if (== _x _x_2)
          (if (< _y _y_2)
            (`KismetArrayLibrary.Array_Insert` _resolutionlist Resolution _array_index :!label _label)
            (set `local.IsAdded` true)
            (break))
          (elif (< _x _x_2)
            (goto _label)))))
    (:`then_1`
      (if (not (`local.IsAdded`))
        (`KismetArrayLibrary.Array_Add` (`self.ResolutionList`) Resolution)))))

(fn `GetResolutionList`
  (returns (ResolutionList :type "Array of IntPoint Structure"))
  (return (`self.ResolutionList`)))

(fn `ParentWidget`
  (bind _pointer (`self.ActivePointer`))
  (bind _uipointerlist (`self.UIPointerList`))
  (bind (_isvalid _container _activeelement _activeindex _ishud _containerwidget) (break `/Game/FemaleShooter/Blueprint/Struct/UI/UI_Pointer` _pointer))
  (bind _returnvalue (`KismetArrayLibrary.Array_LastIndex` _uipointerlist))
  (if (>= _returnvalue 1)
    (`|ExecutionSequence`
      (:`then_0`
        (`self.RestoreHiddenPanels`))
      (:`then_1`
        (`Widget.SetVisibility` (`.ContainerWidget_22_FE51D65B4DC11E116C9EFC8525BC7754` (break `/Game/FemaleShooter/Blueprint/Struct/UI/UI_Pointer` (`self.ActivePointer`))) "Hidden"))
      (:`then_2`
        (`KismetArrayLibrary.Array_Remove` _uipointerlist _returnvalue))
      (:`then_3`
        (`|ExecutionSequence`
          (:`then_0`
            (`Widget.SetVisibility` _containerwidget "Visible"))
          (:`then_1`
            (`self.ActivateMenuInput` (not _ishud) _containerwidget))
          (:`then_2`
            (`self.FocusOnElement` _pointer))
          (:`then_3`
            (bind _asuser_widget (cast `UserWidget` _containerwidget))
            (if (not (`Widget.IsInViewport` _asuser_widget))
              (`UserWidget.AddToViewport` _asuser_widget 0))))))))

(fn `RegisterPanel`
  (params (PanelName :type String) (WidgetClass :type "UserWidget Class Reference") (IsOverwrite :type Boolean))
  (returns (Widget :type "Widget Object Reference"))
  (bind _registeredpanellist (`self.RegisteredPanelList`))
  (bind (_value _returnvalue) (`BlueprintMapLibrary.Map_Find` _registeredpanellist PanelName))
  (`|ExecutionSequence`
    (:`then_0`
      (if _returnvalue
        (if IsOverwrite
          (`Widget.RemoveFromParent` _value)
          (`BlueprintMapLibrary.Map_Remove` _registeredpanellist PanelName)
          (bind _returnvalue_2 (`|CreateWidget` WidgetClass :!label _label))
          (`BlueprintMapLibrary.Map_Add` (`self.RegisteredPanelList`) PanelName _returnvalue_2))
        (else
          (goto _label))))
    (:`then_1`
      (return _value))))

(fn `RestoreHiddenPanels`
  (bind _hiddenpanellist (`self.HiddenPanelList`))
  (bind _returnvalue (`KismetArrayLibrary.Array_LastIndex` _hiddenpanellist))
  (bind _hiddenlist (break `/Game/FemaleShooter/Blueprint/Struct/UI/UI_HiddenPanels` (`|GetArrayItem` _hiddenpanellist _returnvalue)))
  (if (> (`KismetArrayLibrary.Array_Length` _hiddenpanellist) 0)
    (for _array_element _hiddenlist
      (`/Engine/EditorBlueprintResources/StandardMacros.IsValid` _array_element
        (:`Is Valid`
          (`Widget.SetVisibility` _array_element "Visible"))))
    (`KismetArrayLibrary.Array_Clear` _hiddenlist)
    (`KismetArrayLibrary.Array_Remove` _hiddenpanellist _returnvalue)))

(fn `StartWithDefaultResolution`
  (bind _returnvalue (`WidgetLayoutLibrary.GetViewportSize`))
  (bind (_x _y) (`KismetMathLibrary.BreakVector2D` _returnvalue))
  (bind _returnvalue_2 (`GameUserSettings.GetGameUserSettings`))
  (set `self.ScreenMode` "Windowed")
  (set `self.ScreenResolution` (select `bool` (> (`KismetMathLibrary.VSize2D` _returnvalue) 0.0) :`false` (`GameUserSettings.GetDesktopResolution` _returnvalue_2) :`true` (make `IntPoint` (`KismetMathLibrary.FTrunc` _x) (`KismetMathLibrary.FTrunc` _y)))))