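; Blueprint interface for GunnerGirl UI elements, defining a shared contract for identifying them and handling menu navigation input.
; Query functions expose an element's location, widget, type enum and navigation interval.
; Input functions for confirm, back and the four navigation directions each return a boolean.
; The file holds only signatures with default returns, leaving behavior to implementers.
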(fn `BackPressed`
  (returns (IsProcessed :type Boolean))
  (return false))

(fn `ConfirmPressed`
  (returns (IsProcessed :type Boolean))
  (return false))

(fn `GetLocation`
  (returns (Location :type "Vector2D Structure"))
  (return (0.0 0.0)))

(fn `GetNavInterval`
  (returns (NavInterval :type "/Game/FemaleShooter/Blueprint/Struct/UI/UI_NavInterval Structure"))
  (return))

(fn `GetType`
  (returns (ElementType :type "/Game/FemaleShooter/Blueprint/Enum/GunnerGirl_UIElementType Enum"))
  (return "NewEnumerator0"))

(fn `GetWidget`
  (returns (Widget :type "Widget Object Reference"))
  (return null))

(fn `NavDownPressed`
  (returns (IsProcessed :type Boolean))
  (return false))

(fn `NavLeftPressed`
  (returns (IsProcessed :type Boolean))
  (return false))

(fn `NavRightPressed`
  (returns (IsProcessed :type Boolean))
  (return false))

(fn `NavUpPressed`
  (returns (IsProcessed :type Boolean))
  (return false))