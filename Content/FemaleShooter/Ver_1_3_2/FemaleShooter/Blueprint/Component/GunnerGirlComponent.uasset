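; Character component for the GunnerGirl shooter character, handling networked walk/run, crouch, roll, jump, somersault double jump, strafing, camera turning and flashlight toggling.
; Inputs route through Server events to Multicasts, while server Tick updates shared movement state and strafe-aware rotation, which remote instances apply.
; GetAnimData exposes that state plus animation assets with optional default fallback.
; Anim notify messages lock movement, switch flight mode and end rolls or somersaults, starting short cooldowns.
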(event `Server_UpdateCrouch`
  ;[1 1 1] Updater - Crouch Status
  (`self.Server_UpdateCrouch_1`)
  (`self.Server_UpdateCrouch_2`))

(event `self.ReceiveBeginPlay`
  ;[1 1 1] Event Tick and BeginPlay
  (bind _ascharacter (cast `Character` (`self.GetOwner`)))
  (set `self.Character` _ascharacter)
  (`self.SetupFlashlight`))

(event `LockMovement`
  (params (IsLocked :type Boolean))
  ;[1 1 1] Enable/Disable Movement
  (`self.Server_LockMovement` IsLocked))

(event `Server_UpdateVelocity`
  (bind _character (`self.Character`))
  (bind _returnvalue (`Actor.GetVelocity` _character))
  (bind (_returnvalue_x _returnvalue_y) (`KismetMathLibrary.BreakVector` (`KismetMathLibrary.LessLess_VectorRotator` _returnvalue (`Actor.K2_GetActorRotation` _character))))
  ;[1 1 1] Updater - Velocity
  (set `self.Velocity` _returnvalue)
  (setmembers `/Game/FemaleShooter/Ver_1_3_2/FemaleShooter/Blueprint/Struct/GunnerGirlSharedData` :`StructRef` (`self.SharedData`) :`Speed` (`self.SpeedThreshold` (`KismetMathLibrary.VSize` _returnvalue) 0.1) :`ForwardSpeed` (`self.SpeedThreshold` _returnvalue_x 0.1) :`SidewardSpeed` (`self.SpeedThreshold` _returnvalue_y 0.1)))

(event `Server_Sync_ActorRotation`
  ;[1 1 1] Network Synchronization - Actor Rotation
  (bind _output_get (set `self.CharacterActiveRotation` (`self.CalculateCharacterActiveRotation`)))
  (`Actor.K2_SetActorRotation` (`self.Character`) _output_get false))

(event `GunnerGirlNotifyEvent`
  (params (Message :type Name))
  ;[1 1 1] Custom Anim Event
  (switch `name` Message
    (:`MovementEnabled`
      (`self.LockMovement` false))
    (:`MovementDisabled`
      (`self.LockMovement` true))
    (:`FlyModeEnabled`
      (`self.UpdateMovementMode` "MOVE_Flying"))
    (:`FlyModeDisabled`
      (`self.UpdateMovementMode` "MOVE_Falling"))
    (:`SomersaultComplete`
      (`self.DoubleJumpComplete`))
    (:`RollComplete`
      (`self.RollComplete`))))

(event `Server_LockMovement`
  (params (IsLocked :type Boolean))
  ;[1 1 1] Enable/Disable Movement
  (set `self.IsMovementEnabled` (not IsLocked)))

(event `Server_UpdateCrouch_1`
  ;[1 1 1] Updater - Crouch Status
  (if (`self.IsCrouchPressed`)
    (if (`.IsInAir_9_B05389734D0D3EFB792181BDCBD9601E` (break `/Game/FemaleShooter/Ver_1_3_2/FemaleShooter/Blueprint/Struct/GunnerGirlSharedData` (`self.SharedData`)))
      (`self.Multicast_UnCrouch`)
      (else
        (`self.Multicast_Crouch`)))
    (else
      (`self.Multicast_UnCrouch`))))

(event `self.ReceiveTick`
  (params (DeltaSeconds :type "Float (single-precision)"))
  ;[1 1 1] Event Tick and BeginPlay
  (`self.CharacterHasAuthority`
    (:`Authority`
      (`self.Server_Sync`)
      (`self.Server_Update`))
    (:`Remote`
      (`self.Client_Sync`))))

(event `Client_Sync_ActorRotation`
  ;[1 1 1] Network Synchronization - Actor Rotation
  (`Actor.K2_SetActorRotation` (`self.Character`) (`self.CharacterActiveRotation`) false))

(event `Server_UpdateCrouch_2`
  ;[1 1 1] Updater - Crouch Status
  (setmembers `/Game/FemaleShooter/Ver_1_3_2/FemaleShooter/Blueprint/Struct/GunnerGirlSharedData` :`StructRef` (`self.SharedData`) :`IsCrouching` (`NavMovementComponent.IsCrouching` (`Character.CharacterMovement` (`self.Character`)))))

(event `Server_Sync`
  ;[1 1 1] Event Tick and BeginPlay
  (`self.Server_Sync_ActorRotation`))

(event `Server_UpdateAirStatus`
  (bind _returnvalue (`NavMovementComponent.IsFalling` (`Character.CharacterMovement` (`self.Character`))))
  ;[1 1 1] Updater - Airborne Status
  (if (not (== (`.IsInAir_9_B05389734D0D3EFB792181BDCBD9601E` (break `/Game/FemaleShooter/Ver_1_3_2/FemaleShooter/Blueprint/Struct/GunnerGirlSharedData` (`self.SharedData`))) _returnvalue))
    (setmembers `/Game/FemaleShooter/Ver_1_3_2/FemaleShooter/Blueprint/Struct/GunnerGirlSharedData` :`StructRef` (`self.SharedData`) :`IsInAir` _returnvalue)))

(event `Server_Update`
  ;[1 1 1] Event Tick and BeginPlay
  (`|ExecutionSequence`
    (:`then_0`
      (`self.Server_UpdateVelocity`)
      (`self.Server_UpdateAirStatus`)
      (`self.Server_UpdateCrouch`))))

(event `UpdateMovementMode`
  (params (MovementMode :type "EMovementMode Enum" :default "MOVE_None"))
  ;[1 1 1] Update Movement Mode
  (`self.Server_UpdateMovementMode` MovementMode))

(event `Multicast_Crouch`
  ;[1 1 1] Updater - Crouch Status
  (if (not (`NavMovementComponent.IsCrouching` (`Character.CharacterMovement` (`self.Character`))))
    (`Character.Crouch` (`self.Character`))))

(event `Client_Sync`
  ;[1 1 1] Event Tick and BeginPlay
  (`self.Client_Sync_ActorRotation`))

(event `Server_UpdateMovementMode`
  (params (MovementMode :type "EMovementMode Enum" :default "MOVE_None"))
  ;[1 1 1] Update Movement Mode
  (`self.Multicast_UpdateMovementMode` MovementMode))

(event `Multicast_UnCrouch`
  ;[1 1 1] Updater - Crouch Status
  (if (`NavMovementComponent.IsCrouching` (`Character.CharacterMovement` (`self.Character`)))
    (`Character.UnCrouch` (`self.Character`))))

(event `Multicast_UpdateMovementMode`
  (params (MovementMode :type "EMovementMode Enum" :default "MOVE_None"))
  (bind _charactermovement (`Character.CharacterMovement` (`self.Character`)))
  ;[1 1 1] Update Movement Mode
  (if (`|EnumInequality` (`CharacterMovementComponent.MovementMode` _charactermovement) MovementMode)
    (`CharacterMovementComponent.SetMovementMode` _charactermovement MovementMode 0)))

(event `Server_ActivateStrafeMode`
  (params (isActive :type Boolean))
  ;[1 1 1] Strafe Mode - Activation
  (setmembers `/Game/FemaleShooter/Ver_1_3_2/FemaleShooter/Blueprint/Struct/GunnerGirlSharedData` :`StructRef` (`self.SharedData`) :`IsStrafing` isActive)
  (`self.Multicast_ActivateStrafeMode` isActive)
  (`self.OnStrafeModeChanged` isActive))

(event `Multicast_ActivateStrafeMode`
  (params (IsActive :type Boolean))
  ;[1 1 1] Strafe Mode - Activation
)

(event `Crouch`
  ;[1 1 1] Crouch
  (`self.CharacterIsLocallyControlled`
    (:`True`
      (`self.Server_AssignCrouch` true))))

(event `Roll`
  ;[1 1 1] Roll
  (`self.CharacterIsLocallyControlled`
    (:`True`
      (`self.Server_Roll`))))

(event `Walk`
  ;[1 1 1] Walk
  (`self.CharacterIsLocallyControlled`
    (:`True`
      (`self.Server_AssignWalk` true))))

(event `Server_AssignWalk`
  (params (IsWalkPressed :type Boolean))
  ;[1 1 1] Walk
  (set `self.IsWalkPressed_Keyboard` IsWalkPressed))

(event `TriggerJump`
  (params (IsAllowSomersault :type Boolean :default true))
  ;[1 1 1] Jump - Normal/Double Jump Trigger
  (`self.CharacterIsLocallyControlled`
    (:`True`
      (`self.Server_TriggerJump` IsAllowSomersault))))

(event `Server_Roll`
  ;[1 1 1] Roll
  (if (`self.ConfirmRollPossible`)
    (`self.Server_LockMovement` true)
    (`self.Multicast_Roll` (`self.CalculateActiveDirection`))))

(event `UnCrouch`
  ;[1 1 1] Crouch
  (`self.CharacterIsLocallyControlled`
    (:`True`
      (`self.Server_AssignCrouch` false))))

(event `UnWalk`
  ;[1 1 1] Walk
  (`self.CharacterIsLocallyControlled`
    (:`True`
      (`self.Server_AssignWalk` false))))

(event `ActivateStrafeMode`
  (params (IsActivated :type Boolean))
  ;[1 1 1] Strafe Mode - Toggle
  (`self.Server_ActivateStrafeMode` IsActivated))

(event `ToggleStrafeMode`
  ;[1 1 1] Strafe Mode - Toggle
  (`self.Server_ToggleStrafeMode`))

(event `Multicast_Roll`
  (params (RollDirection :type "Vector2D Structure"))
  ;[1 1 1] Roll
  (`self.BeginRoll` RollDirection))

(event `Server_TriggerJump`
  (params (IsAllowSomersault :type Boolean))
  ;[1 1 1] Jump - Normal/Double Jump Trigger
  (if (`self.IsMovementEnabled`)
    (if IsAllowSomersault
      (if (`self.ConfirmNormalJumpPossible`)
        (`self.Multicast_Jump` :!label _label)
        (elif (`self.ConfirmDoubleJumpPossible`)
          (`self.Server_LockMovement` true)
          (`self.Multicast_DoubleJump` (`self.CalculateActiveDirection`))))
      (else
        (goto _label)))))

(event `Server_AssignCrouch`
  (params (IsCrouchPressed :type Boolean))
  ;[1 1 1] Crouch
  (set `self.IsCrouchPressed` IsCrouchPressed))

(event `Server_ToggleStrafeMode`
  ;[1 1 1] Strafe Mode - Toggle
  (`self.Server_ActivateStrafeMode` (not (`.IsStrafing_13_E0ECDA8F447441892EC461AA5290E25B` (break `/Game/FemaleShooter/Ver_1_3_2/FemaleShooter/Blueprint/Struct/GunnerGirlSharedData` (`self.SharedData`))))))

(event `MoveSideward`
  (params (`Axis Value` :type "Float (double-precision)"))
  ;[1 1 1] Walk/Run - Add Movement X
  (`self.Server_MoveSideward` `Axis Value`))

(event `BeginRoll`
  (params (RollDirection :type "Vector2D Structure" :default (0.0 1.0)))
  ;[1 1 1] Roll
  (setmembers `/Game/FemaleShooter/Ver_1_3_2/FemaleShooter/Blueprint/Struct/GunnerGirlSharedData` :`StructRef` (`self.SharedData`) :`IsRolling` true :`RollDirection` RollDirection)
  (set `self.IsRollingReady` false))

(event `MoveForward`
  (params (`Axis Value` :type "Float (double-precision)"))
  ;[1 1 1] Walk/Run - Add Movement Y
  (`self.Server_MoveForward` `Axis Value`))

(event `Server_MoveSideward`
  (params (AxisValue :type "Float (double-precision)"))
  ;[1 1 1] Walk/Run - Add Movement X
  (bind _outputvalue (`self.Update_Movement_AxisX` AxisValue)
    (:`Output`
      (`self.Multicast_MoveSideward` _outputvalue (`.RightVector` (`self.CalculateControlDirection`))))))

(event `Server_MoveForward`
  (params (AxisValue :type "Float (double-precision)"))
  ;[1 1 1] Walk/Run - Add Movement Y
  (bind _outputvalue (`self.Update_Movement_AxisY` AxisValue)
    (:`Output`
      (`self.Multicast_MoveForward` _outputvalue (`self.CalculateControlDirection`)))))

(event `RollComplete`
  ;[1 1 1] Roll
  (`self.CharacterHasAuthority`
    (:`Authority`
      (`self.Server_RollComplete`))))

(event `Server_RollComplete`
  ;[1 1 1] Roll
  (`self.Server_LockMovement` false)
  (`self.Multicast_RollComplete`))

(event `Multicast_MoveSideward`
  (params (AxisValue :type "Float (double-precision)") (Direction :type "Vector Structure"))
  ;[1 1 1] Walk/Run - Add Movement X
  (`Pawn.AddMovementInput` (`self.Character`) (`.RightVector` (`self.CalculateControlDirection`)) AxisValue false))

(event `Multicast_MoveForward`
  (params (AxisValue :type "Float (double-precision)") (Direction :type "Vector Structure"))
  ;[1 1 1] Walk/Run - Add Movement Y
  (`Pawn.AddMovementInput` (`self.Character`) (`self.CalculateControlDirection`) AxisValue true))

(event `Camera_TurnHorizontal`
  (params (AxisValue :type "Float (double-precision)") (TurnRatePerSecond :type "Float (double-precision)" :default 45.0) (Multiplier :type "Float (double-precision)" :default 1.0) (IsInverted :type Boolean))
  ;[1 1 1] Camera Control
  (`Pawn.AddControllerYawInput` (`self.Character`) (* AxisValue TurnRatePerSecond Multiplier (`GameplayStatics.GetWorldDeltaSeconds`) (select `bool` IsInverted :`false` 1.0 :`true` -1.0 :!type "Float (single-precision)"))))

(event `Multicast_Jump`
  ;[1 1 1] Jump - Normal Jump
  (`Character.Jump` (`self.Character`)))

(event `Multicast_DoubleJump`
  (params (DoubleJumpDirection :type "Vector2D Structure"))
  ;[1 1 1] Jump - Double Jump
  (`self.StartDoubleJump` DoubleJumpDirection))

(event `Multicast_RollComplete`
  ;[1 1 1] Roll
  (`self.ClearRoll` 0.2))

(event `StartDoubleJump`
  (params (JumpDirection :type "Vector2D Structure"))
  ;[1 1 1] Jump - Double Jump
  (setmembers `/Game/FemaleShooter/Ver_1_3_2/FemaleShooter/Blueprint/Struct/GunnerGirlSharedData` :`StructRef` (`self.SharedData`) :`IsDoubleJumpReady` false :`IsDoubleJump` true :`DoubleJumpDirection` JumpDirection))

(event `ClearJump`
  ;[1 1 1] Jump - Normal Jump Clearance
  (`self.Server_ClearJump`))

(event `ClearRoll`
  (params (CooldownDuration :type "Float (double-precision)"))
  ;[1 1 1] Roll
  (setmembers `/Game/FemaleShooter/Ver_1_3_2/FemaleShooter/Blueprint/Struct/GunnerGirlSharedData` :`StructRef` (`self.SharedData`) :`IsRolling` false :`RollDirection` (0.0 0.0))
  (if (> CooldownDuration 0.0)
    (`self.CooldownRoll` CooldownDuration)
    (else
      (set `self.IsRollingReady` true))))

(event `DoubleJumpComplete`
  ;[1 1 1] Jump - Double Jump
  (`self.CharacterHasAuthority`
    (:`Authority`
      (`self.Server_DoubleJumpComplete`))))

(event `Camera_TurnVertical`
  (params (AxisValue :type "Float (double-precision)") (TurnRatePerSecond :type "Float (double-precision)" :default 45.0) (Multiplier :type "Float (double-precision)" :default 1.0) (IsInverted :type Boolean))
  ;[1 1 1] Camera Control
  (`Pawn.AddControllerPitchInput` (`self.Character`) (* AxisValue TurnRatePerSecond Multiplier (`GameplayStatics.GetWorldDeltaSeconds`) (select `bool` IsInverted :`false` 1.0 :`true` -1.0 :!type "Float (single-precision)"))))

(event `Server_ClearJump`
  ;[1 1 1] Jump - Normal Jump Clearance
  (`self.Multicast_ClearJump`))

(event `Server_DoubleJumpComplete`
  ;[1 1 1] Jump - Double Jump
  (`self.Server_LockMovement` false)
  (`self.MultiCast_DoubleJumpComplete`))

(event `CooldownRoll`
  (params (CooldownDuration :type "Float (double-precision)"))
  ;[1 1 1] Roll
  (`KismetSystemLibrary.K2_ClearAndInvalidateTimerHandle` (`self.RollCooldown`))
  (bind _returnvalue (`KismetSystemLibrary.K2_SetTimerDelegate` (delegate `ReactivateRoll`) CooldownDuration))
  (set `self.RollCooldown` _returnvalue))

(event `EquipFlashlight`
  (params (IsFlashlightOn :type Boolean))
  ;[1 1 1] Flashlight
  (set `self.IsFlashlightEquipped` true)
  (`self.ActivateFlashlight` IsFlashlightOn))

(event `SetupFlashlight`
  ;[1 1 1] Flashlight
  (if (`self.IsFlashlightEquipped`)
    (`self.ActivateFlashlight_Body` (`self.IsFlashlightOn`))))

(event `Multicast_ClearJump`
  ;[1 1 1] Jump - Normal Jump Clearance
  (`Character.StopJumping` (`self.Character`)))

(event `MultiCast_DoubleJumpComplete`
  ;[1 1 1] Jump - Double Jump
  (`self.Multicast_UpdateMovementMode` "MOVE_Falling")
  (`self.ClearDoubleJump`))

(event `UnequipFlashlight`
  ;[1 1 1] Flashlight
  (`self.ActivateFlashlight` false)
  (set `self.IsFlashlightEquipped` false))

(event `ReactivateRoll`
  ;[1 1 1] Roll
  (`KismetSystemLibrary.K2_ClearAndInvalidateTimerHandle` (`self.RollCooldown`))
  (set `self.RollCooldown` (struct))
  (set `self.IsRollingReady` true))

(event `ToggleFlashLight`
  ;[1 1 1] Flashlight
  (`self.ActivateFlashlight` (not (`self.IsFlashlightOn`))))

(event `ActivateFlashlight`
  (params (IsFlashlightOn :type Boolean))
  ;[1 1 1] Flashlight
  (if (`self.IsFlashlightEquipped`)
    (set `self.IsFlashlightOn` IsFlashlightOn)
    (`|ExecutionSequence`
      (:`then_0`
        (`self.ActivateFlashlight_Body` IsFlashlightOn))
      (:`then_2`
        (`self.OnFlashlightUpdated` (`self.IsFlashlightEquipped`) (`self.IsFlashlightOn`))))))

(event `ClearDoubleJump`
  ;[1 1 1] Jump - Double Jump
  (setmembers `/Game/FemaleShooter/Ver_1_3_2/FemaleShooter/Blueprint/Struct/GunnerGirlSharedData` :`StructRef` (`self.SharedData`) :`IsDoubleJump` false :`DoubleJumpDirection` (0.0 0.0))
  (`self.CooldownDoubleJump`))

(event `CooldownDoubleJump`
  ;[1 1 1] Jump - Double Jump
  (`KismetSystemLibrary.K2_ClearAndInvalidateTimerHandle` (`self.DoubleJumpCooldown`))
  (bind _returnvalue (`KismetSystemLibrary.K2_SetTimerDelegate` (delegate `ReactivateDoubleJump`) 0.2))
  (set `self.DoubleJumpCooldown` _returnvalue))

(event `ReactivateDoubleJump`
  ;[1 1 1] Jump - Double Jump
  (`KismetSystemLibrary.K2_ClearAndInvalidateTimerHandle` (`self.DoubleJumpCooldown`))
  (setmembers `/Game/FemaleShooter/Ver_1_3_2/FemaleShooter/Blueprint/Struct/GunnerGirlSharedData` :`StructRef` (`self.SharedData`) :`IsDoubleJumpReady` true))

(event `ActivateFlashlight_Body`
  (params (IsActivated :type Boolean))
  ;[1 1 1] Flashlight
  (if (`self.IsFlashlightEquipped`)
    (for _array_element (`Actor.K2_GetComponentsByClass` (`self.Character`) "/Game/FemaleShooter/Ver_1_3_2/FemaleShooter/Blueprint/Component/FlashlightComponent.FlashlightComponent_C")
      (`/Game/FemaleShooter/Ver_1_3_2/FemaleShooter/Blueprint/Component/FlashlightComponent.UpdateLightIntensityModifier` _array_element 4.0)
      (`/Game/FemaleShooter/Ver_1_3_2/FemaleShooter/Blueprint/Component/FlashlightComponent.ActivateFlashLight` _array_element IsActivated))))

(fn `GetAnimData`
  (params (DefaultAnimData :type "/Game/FemaleShooter/Ver_1_3_2/FemaleShooter/Blueprint/Struct/GunnerGirlAnimData Structure"))
  (returns (SharedData :type "/Game/FemaleShooter/Ver_1_3_2/FemaleShooter/Blueprint/Struct/GunnerGirlSharedData Structure") (AnimData :type "/Game/FemaleShooter/Ver_1_3_2/FemaleShooter/Blueprint/Struct/GunnerGirlAnimData Structure"))
  (`|ExecutionSequence`
    (:`then_0`
      (if (and (`self.IsFallbackToDefaultAnimation`) (not (`self.IsAnimAllSetup`)))
        (`self.UpdateAnimDataValues` DefaultAnimData)))
    (:`then_1`
      (return (`self.SharedData`) (`self.AnimData`)))))

(fn `UpdateAnimDataValues`
  (params (DefaultAnimData :type "/Game/FemaleShooter/Ver_1_3_2/FemaleShooter/Blueprint/Struct/GunnerGirlAnimData Structure"))
  (bind _blend_jumploop (`self.Blend_JumpLoop`))
  (bind _blend_somersault (`self.Blend_Somersault`))
  (bind _anim_jumplanding (`self.Anim_JumpLanding`))
  (bind _blend_roll (`self.Blend_Roll`))
  (bind _blend_jumpstart (`self.Blend_JumpStart`))
  (bind _blend_walkrun (`self.Blend_WalkRun`))
  (bind _blend_crouch (`self.Blend_Crouch`))
  (bind _returnvalue (`KismetSystemLibrary.IsValid` _blend_roll))
  (bind _returnvalue_2 (`KismetSystemLibrary.IsValid` _blend_jumpstart))
  (bind _returnvalue_3 (`KismetSystemLibrary.IsValid` _blend_jumploop))
  (bind _returnvalue_4 (`KismetSystemLibrary.IsValid` _blend_somersault))
  (bind _returnvalue_5 (`KismetSystemLibrary.IsValid` _anim_jumplanding))
  (bind _returnvalue_6 (`KismetSystemLibrary.IsValid` _blend_walkrun))
  (bind _returnvalue_7 (`KismetSystemLibrary.IsValid` _blend_crouch))
  (bind (_blend_walkrun_2 _blend_crouch_2 _blend_roll_2 _blend_jumpstart_2 _blend_jumploop_2 _anim_jumplanding_2 _blend_somersault_2) (break `/Game/FemaleShooter/Ver_1_3_2/FemaleShooter/Blueprint/Struct/GunnerGirlAnimData` (select `bool` (`self.IsFallbackToDefaultAnimation`) :`true` DefaultAnimData)))
  (setmembers `/Game/FemaleShooter/Ver_1_3_2/FemaleShooter/Blueprint/Struct/GunnerGirlAnimData` :`StructRef` (`self.AnimData`) :`Blend_WalkRun` (select `bool` _returnvalue_6 :`false` _blend_walkrun_2 :`true` _blend_walkrun) :`Blend_Crouch` (select `bool` _returnvalue_7 :`false` _blend_crouch_2 :`true` _blend_crouch) :`Blend_Roll` (select `bool` _returnvalue :`false` _blend_roll_2 :`true` _blend_roll) :`Blend_JumpStart` (select `bool` _returnvalue_2 :`false` _blend_jumpstart_2 :`true` _blend_jumpstart) :`Blend_JumpLoop` (select `bool` _returnvalue_3 :`false` _blend_jumploop_2 :`true` _blend_jumploop) :`Anim_JumpLanding` (select `bool` _returnvalue_5 :`false` _anim_jumplanding_2 :`true` _anim_jumplanding) :`Blend_Somersault` (select `bool` _returnvalue_4 :`false` _blend_somersault_2 :`true` _blend_somersault))
  (set `self.IsAnimAllSetup` (and _returnvalue_6 _returnvalue_7 _returnvalue _returnvalue_2 _returnvalue_3 _returnvalue_4 _returnvalue_5)))