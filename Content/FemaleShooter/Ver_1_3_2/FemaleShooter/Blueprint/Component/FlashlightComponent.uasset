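; A flashlight component that spawns a Flashlight actor and attaches it to itself, giving its owner a controllable light.
; Setup runs on BeginPlay and before each control event, spawning and snapping the actor in place only if none is valid.
; Events forward on/off toggling, target location adjustment and light intensity modifier updates to the spawned actor.
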(event `Setup`
  (`/Engine/EditorBlueprintResources/StandardMacros.IsValid` (`self.FlashLight`)
    (:`Is Not Valid`
      (bind _returnvalue (`|SpawnActorFromClass` "/Game/FemaleShooter/Ver_1_3_2/FemaleShooter/Blueprint/Misc/Flashlight.Flashlight_C" (`KismetMathLibrary.MakeTransform` (0.0 0.0 0.0)) "Undefined" "OverrideRootScale" null null))
      (set `self.FlashLight` _returnvalue)
      (`Actor.K2_AttachToComponent` _returnvalue self "None" "SnapToTarget" "SnapToTarget" "SnapToTarget" true))))

(event `self.ReceiveBeginPlay`
  (`self.Setup`))

(event `ActivateFlashLight`
  (params (IsActive :type Boolean))
  (bind _flashlight (`self.FlashLight`))
  (`self.Setup`)
  (if IsActive
    (`/Game/FemaleShooter/Ver_1_3_2/FemaleShooter/Blueprint/Misc/Flashlight.Activate` _flashlight)
    (else
      (`/Game/FemaleShooter/Ver_1_3_2/FemaleShooter/Blueprint/Misc/Flashlight.Deactivate` _flashlight))))

(event `AdjustTargetLocation`
  (params (IsAdjustTargetLocation :type Boolean) (TargetLocation :type "Vector Structure"))
  (`self.Setup`)
  (`/Game/FemaleShooter/Ver_1_3_2/FemaleShooter/Blueprint/Misc/Flashlight.AdjustTargetLocation` (`self.FlashLight`) IsAdjustTargetLocation TargetLocation))

(event `UpdateLightIntensityModifier`
  (params (LightIntensityModifier :type "Float (double-precision)" :default 1.0))
  (`self.Setup`)
  (`/Game/FemaleShooter/Ver_1_3_2/FemaleShooter/Blueprint/Misc/Flashlight.UpdateLightintensity` (`self.FlashLight`) LightIntensityModifier))