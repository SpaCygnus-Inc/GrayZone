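; Handgun actor component that fires bullets with muzzle effects from a socket on a gun mesh supplied through Setup.
; PerformShot takes ammo data, attaches a muzzle flash emitter and spawns a Bullet configured from that data, optionally rotated toward an adjusted target.
; An optional muzzle light shows the owner's PointLightComponent until a short timer hides it.
; Gun spin events only toggle a state flag.
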(event `Setup`
  (params (GunMeshComponent :type "SkeletalMeshComponent Object Reference") (MuzzleSocket :type Name :default "MuzzleSocket"))
  (set `self.GunMeshComponent` GunMeshComponent)
  (set `self.MuzzleSocketName` MuzzleSocket))

(event `GenerateMuzzleLight`
  (params (IsGenerateMuzzleLight :type Boolean))
  (set `self.IsGenerateMuzzleLight` IsGenerateMuzzleLight)
  (if (`self.IsGenerateMuzzleLight`)
    (`KismetSystemLibrary.K2_ClearAndInvalidateTimerHandle` (`self.MuzzleLightTimer`))
    (set `self.MuzzleLightTimer` (struct))
    (`SceneComponent.SetVisibility` (`Actor.GetComponentByClass` (`self.GetOwner`) "/Script/Engine.PointLightComponent") true false)
    (bind _returnvalue (`KismetSystemLibrary.K2_SetTimerDelegate` (delegate `EndMuzzleLight`) 0.05))
    (set `self.MuzzleLightTimer` _returnvalue)))

(event `ShowMuzzleFlash`
  (params (MuzzleFlashEffect :type "ParticleSystem Object Reference") (isGenerateMuzzleLight :type Boolean))
  (`GameplayStatics.SpawnEmitterAttached` MuzzleFlashEffect (`self.GunMeshComponent`) (`self.MuzzleSocketName`))
  (`self.GenerateMuzzleLight` isGenerateMuzzleLight))

(event `EndMuzzleLight`
  (`KismetSystemLibrary.K2_ClearAndInvalidateTimerHandle` (`self.MuzzleLightTimer`))
  (set `self.MuzzleLightTimer` (struct))
  (`SceneComponent.SetVisibility` (`Actor.GetComponentByClass` (`self.GetOwner`) "/Script/Engine.PointLightComponent") false false))

(event `StartGunSpin`
  (set `self.IsGunSpinning` true))

(event `ActivateGunSpin`
  (params (IsActive :type Boolean))
  (if IsActive
    (`self.StartGunSpin`)
    (else
      (`self.StopGunSpin`))))

(event `StopGunSpin`
  (set `self.IsGunSpinning` false))

(event `PerformShot`
  (params (AmmoData :type "/Game/FemaleShooter/Ver_1_3_2/FemaleShooter/Blueprint/Data/Ammo/AmmoData Object Reference") (IsAdjustedTarget :type Boolean) (AdjustedTargetLocation :type "Vector Structure") (IsGenerateMuzzleLight :type Boolean))
  (`|ExecutionSequence`
    (:`then_0`
      (`self.ShowMuzzleFlash` (`/Game/FemaleShooter/Ver_1_3_2/FemaleShooter/Blueprint/Data/Ammo/AmmoData.MuzzleFlashEffect` AmmoData) IsGenerateMuzzleLight))
    (:`then_1`
      (`self.ShootBullet` IsAdjustedTarget AdjustedTargetLocation (`/Game/FemaleShooter/Ver_1_3_2/FemaleShooter/Blueprint/Data/Ammo/AmmoData.BulletSpeed` AmmoData) (`/Game/FemaleShooter/Ver_1_3_2/FemaleShooter/Blueprint/Data/Ammo/AmmoData.Gravity` AmmoData) (`/Game/FemaleShooter/Ver_1_3_2/FemaleShooter/Blueprint/Data/Ammo/AmmoData.ImpactModifier` AmmoData) (`/Game/FemaleShooter/Ver_1_3_2/FemaleShooter/Blueprint/Data/Ammo/AmmoData.Lifetime` AmmoData) (`/Game/FemaleShooter/Ver_1_3_2/FemaleShooter/Blueprint/Data/Ammo/AmmoData.BulletMesh` AmmoData) (`/Game/FemaleShooter/Ver_1_3_2/FemaleShooter/Blueprint/Data/Ammo/AmmoData.TrailEffect` AmmoData) (`/Game/FemaleShooter/Ver_1_3_2/FemaleShooter/Blueprint/Data/Ammo/AmmoData.ImpactEffect` AmmoData)))))

(event `ShootBullet`
  (params (IsAdjustedTarget :type Boolean) (AdjustedTargetLocation :type "Vector Structure") (BulletSpeed :type "Float (double-precision)") (Gravity :type "Float (double-precision)") (BulletImpactModifier :type "Float (double-precision)" :default 1.0) (Lifetime :type "Float (double-precision)") (BulletMesh :type "StaticMesh Object Reference") (TrailEffect :type "ParticleSystem Object Reference") (ImpactEffect :type "ParticleSystem Object Reference"))
  (bind _returnvalue (`SceneComponent.GetSocketTransform` (`self.GunMeshComponent`) (`self.MuzzleSocketName`) "RTS_World"))
  (bind _location (.location _returnvalue))
  (`|SpawnActorFromClass` "/Game/FemaleShooter/Ver_1_3_2/FemaleShooter/Asset/Bullet/Bullet.Bullet_C" (select `bool` IsAdjustedTarget :`false` _returnvalue :`true` (`KismetMathLibrary.MakeTransform` _location (`KismetMathLibrary.FindLookAtRotation` _location AdjustedTargetLocation) (.scale _returnvalue))) "AlwaysSpawn" "OverrideRootScale" null BulletMesh TrailEffect ImpactEffect BulletSpeed Gravity BulletImpactModifier Lifetime null))