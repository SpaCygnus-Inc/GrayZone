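; Actor component that tracks items registered with it and lets its owner pick up the nearest one.
; Register and Unregister maintain a map used as a set, whose keys are scanned for the valid actor closest to the owner.
; RetrieveSimpleItem reports that actor if it is a SimpleItem, while FindSimpleItem broadcasts it through OnSimpleItemFound and then calls ItemConsumed on it.
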(event `Register`
  (params (Actor :type "Actor Object Reference"))
  (if (not (`.ReturnValue` (`BlueprintMapLibrary.Map_Find` (`self.ItemMap`) Actor)))
    (`BlueprintMapLibrary.Map_Add` (`self.ItemMap`) Actor)))

(event `Unregister`
  (params (Actor :type "Actor Object Reference"))
  (if (`.ReturnValue` (`BlueprintMapLibrary.Map_Find` (`self.ItemMap`) Actor))
    (`BlueprintMapLibrary.Map_Remove` (`self.ItemMap`) Actor)))

(fn `FindSimpleItem`
  (bind _nearestactor (`self.RetrieveNearestActor`))
  (`/Engine/EditorBlueprintResources/StandardMacros.IsValid` _nearestactor
    (:`Is Valid`
      (bind _assimple_item (cast `/Game/FemaleShooter/Ver_1_3_2/FemaleShooter/Additional/SimpleItem/SimpleItem` _nearestactor))
      (`self.OnSimpleItemFound` _assimple_item (`/Game/FemaleShooter/Ver_1_3_2/FemaleShooter/Additional/SimpleItem/SimpleItem.ItemType` _assimple_item))
      (`/Game/FemaleShooter/Ver_1_3_2/FemaleShooter/Additional/SimpleItem/SimpleItem.ItemConsumed` _assimple_item))))

(fn `RetrieveList`
  (returns (List :type "Array of Actor Object Reference"))
  (bind _keys (`BlueprintMapLibrary.Map_Keys` (`self.ItemMap`)))
  (return _keys))

(fn `RetrieveNearestActor`
  (returns (NearestActor :type "Actor Object Reference"))
  (locals (CurrentResult :type "Actor Object Reference") (CurrentDistance :type "Float (double-precision)"))
  (bind _list (`self.RetrieveList`))
  (for _array_element _list
    (`/Engine/EditorBlueprintResources/StandardMacros.IsValid` _array_element
      (:`Is Valid`
        (`/Engine/EditorBlueprintResources/StandardMacros.IsValid` (`local.CurrentResult`)
          (:`Is Valid`
            (bind _returnvalue (`KismetMathLibrary.VSize` (- (`Actor.K2_GetActorLocation` _array_element) (`Actor.K2_GetActorLocation` (`self.GetOwner`)))))
            (if (< _returnvalue (`local.CurrentDistance`))
              (set `local.CurrentResult` _array_element :!label _label)
              (set `local.CurrentDistance` _returnvalue)))
          (:`Is Not Valid`
            (goto _label))))))
  (return (`local.CurrentResult`)))

(fn `RetrieveSimpleItem`
  (returns (IsFound :type Boolean) (SimpleItem :type "/Game/FemaleShooter/Ver_1_3_2/FemaleShooter/Additional/SimpleItem/SimpleItem Object Reference") (ItemType :type Name))
  (bind _nearestactor (`self.RetrieveNearestActor`))
  (`/Engine/EditorBlueprintResources/StandardMacros.IsValid` _nearestactor
    (:`Is Valid`
      (bind _assimple_item (cast `/Game/FemaleShooter/Ver_1_3_2/FemaleShooter/Additional/SimpleItem/SimpleItem` _nearestactor)
        (:`then`
          (return true _assimple_item (`/Game/FemaleShooter/Ver_1_3_2/FemaleShooter/Additional/SimpleItem/SimpleItem.ItemType` _assimple_item)))
        (:`CastFailed`
          _)))
    (:`Is Not Valid`
      _))
  (return false null "None"))