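; KeyPressHandler is a component that reports held keys for the player controlling its owning pawn.
; Setup stores a map of keys to input names.
; Each tick it gets the owner's PlayerController, polls every mapped key and fires OnKeyDown with the key and name.
; Because it polls state rather than binding input events, OnKeyDown repeats every frame a key stays down.
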(event `self.ReceiveTick`
  (params (DeltaSeconds :type "Float (single-precision)"))
  (`self.UpdateInput`))

(event `UpdateInput`
  (bind _playercontroller (`self.RetrievePlayerController`))
  (`/Engine/EditorBlueprintResources/StandardMacros.IsValid` _playercontroller
    (:`Is Valid`
      (bind _keys (`BlueprintMapLibrary.Map_Keys` (`self.Map_InputName`)))
      (for _array_element _keys
        (if (`PlayerController.IsInputKeyDown` _playercontroller _array_element)
          (`self.OnKeyDown` _array_element (`BlueprintMapLibrary.Map_Find` (`self.Map_InputName`) _array_element)))))))

(event `Setup`
  (params (KeyMap :type "Map of Key Structure to Name"))
  (set `self.Map_InputName` KeyMap))

(fn `RetrievePlayerController`
  (returns (PlayerController :type "PlayerController Object Reference"))
  (bind _aspawn (cast `Pawn` (`self.GetOwner`)))
  (bind _asplayer_controller (cast `PlayerController` (`Pawn.GetController` _aspawn)))
  (return _asplayer_controller))