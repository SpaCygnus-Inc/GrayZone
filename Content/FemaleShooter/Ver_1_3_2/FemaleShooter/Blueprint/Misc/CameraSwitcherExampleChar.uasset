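; Example character that demonstrates the CameraSwitcher component, letting the player change between several attached cameras.
; On BeginPlay it sets up the switcher with FollowCamera as the starting camera.
; C and Z cycle to the next and previous camera, while number keys jump directly to the follow, wide or above camera.
; Every switch uses the same transition mode and a custom interpolation speed.
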(event `self.ReceiveBeginPlay`
  (`self.Setup`))

(event `Setup`
  ;[1 1 1] Setup - Camera Switcher
  (`/Game/FemaleShooter/Ver_1_3_2/FemaleShooter/Blueprint/Component/CameraSwitcher.Setup` (`self.CameraSwitcher`) (`self.FollowCamera`)))

(event `Key|C`
  (params (Key :type "Key Structure"))
  ;[1 1 1] Input - Camera Switcher
  (:`Pressed`
    (`/Game/FemaleShooter/Ver_1_3_2/FemaleShooter/Blueprint/Component/CameraSwitcher.SwitchToNextCamera` (`self.CameraSwitcher`) "NewEnumerator2" 8.0)))

(event `Key|Z`
  (params (Key :type "Key Structure"))
  ;[1 1 1] Input - Camera Switcher
  (:`Pressed`
    (`/Game/FemaleShooter/Ver_1_3_2/FemaleShooter/Blueprint/Component/CameraSwitcher.SwitchToPrevCamera` (`self.CameraSwitcher`) "NewEnumerator2" 8.0)))

(event `Key|One`
  (params (Key :type "Key Structure"))
  ;[1 1 1] Input - Camera Switcher
  (:`Pressed`
    (`/Game/FemaleShooter/Ver_1_3_2/FemaleShooter/Blueprint/Component/CameraSwitcher.SwitchToCamera` (`self.CameraSwitcher`) (`self.FollowCamera`) "NewEnumerator2" 8.0)))

(event `Key|Two`
  (params (Key :type "Key Structure"))
  ;[1 1 1] Input - Camera Switcher
  (:`Pressed`
    (`/Game/FemaleShooter/Ver_1_3_2/FemaleShooter/Blueprint/Component/CameraSwitcher.SwitchToCamera` (`self.CameraSwitcher`) (`self.WideCamera`) "NewEnumerator2" 8.0)))

(event `Key|Three`
  (params (Key :type "Key Structure"))
  ;[1 1 1] Input - Camera Switcher
  (:`Pressed`
    (`/Game/FemaleShooter/Ver_1_3_2/FemaleShooter/Blueprint/Component/CameraSwitcher.SwitchToCamera` (`self.CameraSwitcher`) (`self.AboveCamera`) "NewEnumerator2" 8.0)))

(fn `UserConstructionScript`)