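; Player character Blueprint for the GunnerGirl demo, a dual-gun shooter with camera switching, item pickups and demo UI.
; Keyboard, mouse and gamepad input forwards to GunnerGirlComponent for movement, TwinGunHandler for guns and CameraSwitcher for aiming, with KeyPressHandler supplying held WASD keys.
; BeginPlay binds component events, linking aim, gun pose cameras, strafe and flashlight state, and updating the UI.
; ItemCollector finds items that grant ammo, flashlight or weapons, press triggers or cycle shooting patterns.
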(event `Key|Gamepad_Special_Right`
  (params (Key :type "Key Structure"))
  ;[1 0.4538 0.404] Input - Toggle Demo UI
  (:`Pressed`
    (`self.Toggle_UI_Help` :!label _label)))

(event `Setup_ComponentsInteraction`
  ;[1 1 1] Setup Interaction
  (`self.Setup_GunnerGirl_TwinGun`)
  (`self.Setup_Camera_TwinGun`))

(event `self.ReceiveBeginPlay`
  ;[1 1 1] Event BeginPlay, Event Tick, and Basic Setup
  (`KismetSystemLibrary.Delay` 0.2)
  (`|ExecutionSequence`
    (:`then_0`
      (if true
        (`self.SetupInput_KeyPressHandler`)))
    (:`then_1`
      (if true
        (`self.SetupDemoUI`)))
    (:`then_2`
      (`self.SetupCameraHandler`)
      (`self.Setup_ComponentsInteraction`)
      (`self.SetupItemCollector`))
    (:`then_3`
      (`/Game/FemaleShooter/Ver_1_3_2/FemaleShooter/Blueprint/Component/TwinGunHandler.EquipGun` (`self.TwinGunHandler`) true))))

(event `Key|Enter`
  (params (Key :type "Key Structure"))
  ;[1 0.4538 0.404] Input - Toggle Demo UI
  (:`Pressed`
    (goto _label)))

(event `Setup_UI_Help`
  ;[1 0.4538 0.404] Setup - Demo UI
  (`/Engine/EditorBlueprintResources/StandardMacros.IsValid` (`self.UI_Demo`)
    (:`Is Not Valid`
      (bind _returnvalue (`|CreateWidget` "/Game/FemaleShooter/Ver_1_3_2/FemaleShooter/Blueprint/UI/UI_Demo.UI_Demo_C"))
      (set `self.UI_Demo` _returnvalue)
      (`UserWidget.AddToViewport` (`self.UI_Demo`) 0))))

(event `self.ReceiveTick`
  (params (DeltaSeconds :type "Float (single-precision)"))
  ;[1 1 1] Event BeginPlay, Event Tick, and Basic Setup
)

(event `Toggle_UI_Help`
  ;[1 0.4538 0.404] Input - Toggle Demo UI
  (`/Engine/EditorBlueprintResources/StandardMacros.IsValid` (`self.UI_Demo`)
    (:`Is Valid`
      (`/Game/FemaleShooter/Ver_1_3_2/FemaleShooter/Blueprint/UI/UI_Demo.ToggleUIPanel` (`self.UI_Demo`)))))

(event `SetupDemoUI`
  ;[1 0.4538 0.404] Setup - Demo UI
  (`|ExecutionSequence`
    (:`then_0`
      (`self.Setup_UI_Help`))
    (:`then_1`
      (add `/Game/FemaleShooter/Ver_1_3_2/FemaleShooter/Blueprint/Component/TwinGunHandler.OnShootingPatternChanged` (`self.TwinGunHandler`) (delegate `OnShootingPatternChanged_Event_0`)))
    (:`then_2`
      (add `/Game/FemaleShooter/Ver_1_3_2/FemaleShooter/Blueprint/Component/TwinGunHandler.OnGunModeChanged` (`self.TwinGunHandler`) (delegate `OnGunModeChanged_Event_0`)))
    (:`then_3`
      (add `/Game/FemaleShooter/Ver_1_3_2/FemaleShooter/Blueprint/Component/TwinGunHandler.OnShootingHandChanged` (`self.TwinGunHandler`) (delegate `OnShootingHandChanged_Event_0`)))
    (:`then_4`
      (add `/Game/FemaleShooter/Ver_1_3_2/FemaleShooter/Blueprint/Component/GunnerGirlComponent.OnStrafeModeChanged` (`self.GunnerGirlComponent`) (delegate `OnStrafeModeChanged_Event_0`)))
    (:`then_5`
      (add `/Game/FemaleShooter/Ver_1_3_2/FemaleShooter/Blueprint/Component/GunnerGirlComponent.OnFlashlightUpdated` (`self.GunnerGirlComponent`) (delegate `OnFlashlightEquipped_Event_0`)))))

(event `Setup_Camera_TwinGun`
  ;[1 1 1] Setup Interaction - Camera - TwinGun
  (`|ExecutionSequence`
    (:`then_0`
      (add `/Game/FemaleShooter/Ver_1_3_2/FemaleShooter/Blueprint/Component/CameraSwitcher.OnAimActivated` (`self.CameraSwitcher`) (delegate `OnAimActivated_Event_0`)))
    (:`then_1`
      (add `/Game/FemaleShooter/Ver_1_3_2/FemaleShooter/Blueprint/Component/TwinGunHandler.OnGunPoseUpdated` (`self.TwinGunHandler`) (delegate `OnGunPoseUpdated_Event_0`)))))

(event `Key|Three`
  (params (Key :type "Key Structure"))
  ;[1 1 1] Switch mesh during gameplay
  (:`Pressed`
    (`SkinnedMeshComponent.SetSkinnedAssetAndUpdate` (`self.Mesh`) "/Game/FemaleShooter/Ver_1_3_2/FemaleShooter/Asset/GunnerGirl/Mesh/SK_GunnerGirl.SK_GunnerGirl" true)))

(event `Setup_GunnerGirl_TwinGun`
  ;[1 1 1] Setup Interaction - GunnerGirl - TwinGun
  (`|ExecutionSequence`
    (:`then_0`
      (add `/Game/FemaleShooter/Ver_1_3_2/FemaleShooter/Blueprint/Component/TwinGunHandler.OnStrafeModeUpdated` (`self.TwinGunHandler`) (delegate `OnStrafeModeUpdated_Event_0`)))
    (:`then_1`
      (add `/Game/FemaleShooter/Ver_1_3_2/FemaleShooter/Blueprint/Component/GunnerGirlComponent.OnFlashlightUpdated` (`self.GunnerGirlComponent`) (delegate `OnFlashlightEquipped_Event_1`)))))

(event `OnStrafeModeUpdated_Event_0`
  (params (IsActivated :type Boolean))
  ;[1 1 1] Setup Interaction - GunnerGirl - TwinGun
  (`/Game/FemaleShooter/Ver_1_3_2/FemaleShooter/Blueprint/Component/GunnerGirlComponent.ActivateStrafeMode` (`self.GunnerGirlComponent`) IsActivated))

(event `OnAimActivated_Event_0`
  (params (IsActivated :type Boolean))
  ;[1 1 1] Setup Interaction - Camera - TwinGun
  (if IsActivated
    (`/Game/FemaleShooter/Ver_1_3_2/FemaleShooter/Blueprint/Component/TwinGunHandler.StartAim` (`self.TwinGunHandler`))
    (else
      (`/Game/FemaleShooter/Ver_1_3_2/FemaleShooter/Blueprint/Component/TwinGunHandler.StopAim` (`self.TwinGunHandler`)))))

(event `OnShootingPatternChanged_Event_0`
  (params (ShootingPattern :type "/Game/FemaleShooter/Ver_1_3_2/FemaleShooter/Blueprint/Data/ShootingPattern/ShootingPattern Object Reference"))
  ;[1 0.4538 0.404] Setup - Demo UI
  (`/Game/FemaleShooter/Ver_1_3_2/FemaleShooter/Blueprint/UI/UI_Demo.UpdateShootingPattern` (`self.UI_Demo`) ShootingPattern))

(event `Key|Four`
  (params (Key :type "Key Structure"))
  ;[1 1 1] Switch mesh during gameplay
  (:`Pressed`
    (`SkinnedMeshComponent.SetSkinnedAssetAndUpdate` (`self.Mesh`) "/Game/FemaleShooter/Ver_1_3_2/FemaleShooter/Asset/GunnerGirl/Mesh/SK_Mannequin.SK_Mannequin" true)))

(event `Key|Escape`
  (params (Key :type "Key Structure"))
  ;[1 0.4538 0.404] Input - Quit Program
  (:`Pressed`
    (`KismetSystemLibrary.QuitGame` null "Quit" :!label _label_2)))

(event `OnFlashlightEquipped_Event_1`
  (params (IsEquipped :type Boolean) (IsActivated :type Boolean))
  ;[1 1 1] Setup Interaction - GunnerGirl - TwinGun
  (`/Game/FemaleShooter/Ver_1_3_2/FemaleShooter/Blueprint/Component/TwinGunHandler.UpdateFlashlightStatus` (`self.TwinGunHandler`) IsEquipped IsActivated))

(event `Key|Five`
  (params (Key :type "Key Structure"))
  ;[1 1 1] Switch mesh during gameplay
  (:`Pressed`
    (`SkinnedMeshComponent.SetSkinnedAssetAndUpdate` (`self.Mesh`) "/Game/FemaleShooter/Ver_1_3_2/FemaleShooter/Asset/GunnerGirl/Mesh/SK_Mannequin_Female.SK_Mannequin_Female" true)))

(event `OnGunPoseUpdated_Event_0`
  (params (GunPose :type "/Game/FemaleShooter/Ver_1_3_2/FemaleShooter/Blueprint/Enum/GunPoseStatus Enum" :default "NewEnumerator0") (IsGunPoseActivated :type Boolean))
  ;[1 1 1] Setup Interaction - Camera - TwinGun
  (if IsGunPoseActivated
    (`/Game/FemaleShooter/Ver_1_3_2/FemaleShooter/Blueprint/Component/CameraSwitcher.SwitchToCamera` (`self.CameraSwitcher`) (`self.GunCamera`) "NewEnumerator2" 8.0)
    (else
      (`/Game/FemaleShooter/Ver_1_3_2/FemaleShooter/Blueprint/Component/CameraSwitcher.SwitchToCamera` (`self.CameraSwitcher`) (`self.FollowCamera`) "NewEnumerator2" 8.0))))

(event `Key|Gamepad_Special_Left`
  (params (Key :type "Key Structure"))
  ;[1 0.4538 0.404] Input - Quit Program
  (:`Pressed`
    (goto _label_2)))

(event `OnGunModeChanged_Event_0`
  (params (IsActive :type Boolean))
  ;[1 0.4538 0.404] Setup - Demo UI
  (if IsActive
    (`/Game/FemaleShooter/Ver_1_3_2/FemaleShooter/Blueprint/UI/UI_Demo.GunModeEnabled` (`self.UI_Demo`))
    (else
      (`/Game/FemaleShooter/Ver_1_3_2/FemaleShooter/Blueprint/UI/UI_Demo.GunModeDisabled` (`self.UI_Demo`)))))

(event `OnShootingHandChanged_Event_0`
  (params (ShootingHand :type "/Game/FemaleShooter/Ver_1_3_2/FemaleShooter/Blueprint/Enum/ShootingHand Enum" :default "NewEnumerator3"))
  ;[1 0.4538 0.404] Setup - Demo UI
  (`/Game/FemaleShooter/Ver_1_3_2/FemaleShooter/Blueprint/UI/UI_Demo.UpdateShootingHand` (`self.UI_Demo`) ShootingHand))

(event `OnStrafeModeChanged_Event_0`
  (params (IsActive :type Boolean))
  ;[1 0.4538 0.404] Setup - Demo UI
  (if IsActive
    (`/Game/FemaleShooter/Ver_1_3_2/FemaleShooter/Blueprint/UI/UI_Demo.StrafeModeEnabled` (`self.UI_Demo`))
    (else
      (`/Game/FemaleShooter/Ver_1_3_2/FemaleShooter/Blueprint/UI/UI_Demo.StrafeModeDisabled` (`self.UI_Demo`)))))

(event `Key|RightMouseButton`
  (params (Key :type "Key Structure"))
  ;[1 0.7231 0.3613] Input - Aim (Keyboard)
  (:`Pressed`
    (`/Game/FemaleShooter/Ver_1_3_2/FemaleShooter/Blueprint/Component/CameraSwitcher.StartAim` (`self.CameraSwitcher`)))
  (:`Released`
    (`/Game/FemaleShooter/Ver_1_3_2/FemaleShooter/Blueprint/Component/CameraSwitcher.StopAim` (`self.CameraSwitcher`))))

(event `Key|Gamepad_RightThumbstick`
  (params (Key :type "Key Structure"))
  ;[1 0.72 0.3615] Input - Switch Camera
  (:`Pressed`
    (`/Game/FemaleShooter/Ver_1_3_2/FemaleShooter/Blueprint/Component/CameraSwitcher.SwitchToNextCamera` (`self.CameraSwitcher`) "NewEnumerator2" 8.0 :!label _label_3)))

(event `SetupCameraHandler`
  (bind _cameraswitcher (`self.CameraSwitcher`))
  ;[1 0.7231 0.3613] Setup - Camera Handler
  (`/Game/FemaleShooter/Ver_1_3_2/FemaleShooter/Blueprint/Component/CameraSwitcher.Setup` _cameraswitcher (`self.FollowCamera`))
  (`/Game/FemaleShooter/Ver_1_3_2/FemaleShooter/Blueprint/Component/CameraSwitcher.RegisterAimCamera` _cameraswitcher (`|MakeArray` (`self.GunCamera`))))

(event `Key|V`
  (params (Key :type "Key Structure"))
  ;[1 0.72 0.3615] Input - Switch Camera
  (:`Pressed`
    (goto _label_3)))

(event `InputAxisKey|Gamepad_LeftTriggerAxis`
  (params (AxisValue :type "Float (single-precision)"))
  ;[1 0.7231 0.3613] Input - Aim (Gamepad)
  (`/Game/FemaleShooter/Ver_1_3_2/FemaleShooter/Blueprint/Component/CameraSwitcher.DynamicAim` (`self.CameraSwitcher`) AxisValue))

(event `OnFlashlightEquipped_Event_0`
  (params (IsEquipped :type Boolean) (IsActivated :type Boolean))
  ;[1 0.4538 0.404] Setup - Demo UI
  (`/Game/FemaleShooter/Ver_1_3_2/FemaleShooter/Blueprint/UI/UI_Demo.FlashlightEquipped` (`self.UI_Demo`) IsEquipped IsActivated))

(event `Key|Gamepad_FaceButton_Top`
  (params (Key :type "Key Structure"))
  ;[0 0.6445 1] Input - Examine/Interact
  (:`Pressed`
    (`/Game/FemaleShooter/Ver_1_3_2/FemaleShooter/Blueprint/Component/ItemCollector.FindSimpleItem` (`self.ItemCollector`) :!label _label_4)))

(event `Key|Gamepad_LeftThumbstick`
  (params (Key :type "Key Structure"))
  ;[0.3569 1 0.3843] Input - Strafe Mode
  (:`Pressed`
    (`/Game/FemaleShooter/Ver_1_3_2/FemaleShooter/Blueprint/Component/GunnerGirlComponent.ToggleStrafeMode` (`self.GunnerGirlComponent`) :!label _label_5)))

(event `Key|Gamepad_DPad_Left`
  (params (Key :type "Key Structure"))
  ;[0.8714 0.2016 1] Input - Left Gun Shot Only
  (:`Pressed`
    (`/Game/FemaleShooter/Ver_1_3_2/FemaleShooter/Blueprint/Component/TwinGunHandler.LeftGunShotOnly` (`self.TwinGunHandler`) true :!label _label_6))
  (:`Released`
    (`/Game/FemaleShooter/Ver_1_3_2/FemaleShooter/Blueprint/Component/TwinGunHandler.LeftGunShotOnly` (`self.TwinGunHandler`) false :!label _label_7)))

(event `InputAxisKey|Gamepad_RightX`
  (params (AxisValue :type "Float (single-precision)"))
  ;[0.3569 1 0.3843] Input - Camera Control
  (`/Game/FemaleShooter/Ver_1_3_2/FemaleShooter/Blueprint/Component/GunnerGirlComponent.Camera_TurnHorizontal` (`self.GunnerGirlComponent`) AxisValue 45.0 2.0 false))

(event `Key|Gamepad_LeftShoulder`
  (params (Key :type "Key Structure"))
  ;[0.8714 0.2016 1] Input - Gun Equip + Unequip (Normal) (Gamepad)
  (:`Pressed`
    (`/Game/FemaleShooter/Ver_1_3_2/FemaleShooter/Blueprint/Component/TwinGunHandler.ToggleEquipGun` (`self.TwinGunHandler`) false)))

(event `InputAxisKey|Gamepad_LeftY`
  (params (AxisValue :type "Float (single-precision)"))
  ;[0.3569 1 0.3843] Input - Movement (Gamepad)
  (`/Game/FemaleShooter/Ver_1_3_2/FemaleShooter/Blueprint/Component/GunnerGirlComponent.MoveForward` (`self.GunnerGirlComponent`) AxisValue))

(event `SetupItemCollector`
  ;[0 0.6445 1] Item Collector
  (add `/Game/FemaleShooter/Ver_1_3_2/FemaleShooter/Blueprint/Component/ItemCollector.OnSimpleItemFound` (`self.ItemCollector`) (delegate `OnSimpleItemFound_Event_0`)))

(event `Key|LeftShift`
  (params (Key :type "Key Structure"))
  ;[0.3569 1 0.3843] Input - Walk
  (:`Pressed`
    (`/Game/FemaleShooter/Ver_1_3_2/FemaleShooter/Blueprint/Component/GunnerGirlComponent.Walk` (`self.GunnerGirlComponent`)))
  (:`Released`
    (`/Game/FemaleShooter/Ver_1_3_2/FemaleShooter/Blueprint/Component/GunnerGirlComponent.UnWalk` (`self.GunnerGirlComponent`))))

(event `Key|F`
  (params (Key :type "Key Structure"))
  ;[0 0.6445 1] Input - Examine/Interact
  (:`Pressed`
    (goto _label_4)))

(event `Key|Y`
  (params (Key :type "Key Structure"))
  ;[0.3569 1 0.3843] Input - Strafe Mode
  (:`Pressed`
    (goto _label_5)))

(event `Key|Z`
  (params (Key :type "Key Structure"))
  ;[0.8714 0.2016 1] Input - Left Gun Shot Only
  (:`Pressed`
    (goto _label_6))
  (:`Released`
    (goto _label_7)))

(event `OnSimpleItemFound_Event_0`
  (params (SimpleItem :type "/Game/FemaleShooter/Ver_1_3_2/FemaleShooter/Additional/SimpleItem/SimpleItem Object Reference") (ItemType :type Name))
  ;[0 0.6445 1] Item Collector
  (switch `name` ItemType
    (:`Ammo`
      (`self.ExamineAmmo` SimpleItem))
    (:`Trigger`
      (`self.ExamineTrigger` SimpleItem))
    (:`Flashlight`
      (`self.PickupFlashlight` SimpleItem))
    (:`WeaponSet`
      (`self.PickupWeaponSet` SimpleItem))
    (:`ShootingPatternChange`
      (`self.ChangeShootingPattern`))))

(event `InputAxisKey|Gamepad_LeftX`
  (params (AxisValue :type "Float (single-precision)"))
  ;[0.3569 1 0.3843] Input - Movement (Gamepad)
  (`/Game/FemaleShooter/Ver_1_3_2/FemaleShooter/Blueprint/Component/GunnerGirlComponent.MoveSideward` (`self.GunnerGirlComponent`) AxisValue))

(event `InputAxisKey|Gamepad_RightY`
  (params (AxisValue :type "Float (single-precision)"))
  ;[0.3569 1 0.3843] Input - Camera Control
  (`/Game/FemaleShooter/Ver_1_3_2/FemaleShooter/Blueprint/Component/GunnerGirlComponent.Camera_TurnVertical` (`self.GunnerGirlComponent`) AxisValue 45.0 2.0 true))

(event `InputAxisKey|MouseX`
  (params (AxisValue :type "Float (single-precision)"))
  ;[0.3569 1 0.3843] Input - Camera Control
  (`/Game/FemaleShooter/Ver_1_3_2/FemaleShooter/Blueprint/Component/GunnerGirlComponent.Camera_TurnHorizontal` (`self.GunnerGirlComponent`) AxisValue 45.0 1.5 false))

(event `Key|Gamepad_RightShoulder`
  (params (Key :type "Key Structure"))
  ;[0.3569 1 0.3843] Input - Crouch
  (:`Pressed`
    (`/Game/FemaleShooter/Ver_1_3_2/FemaleShooter/Blueprint/Component/GunnerGirlComponent.Crouch` (`self.GunnerGirlComponent`) :!label _label_8))
  (:`Released`
    (`/Game/FemaleShooter/Ver_1_3_2/FemaleShooter/Blueprint/Component/GunnerGirlComponent.UnCrouch` (`self.GunnerGirlComponent`) :!label _label_9)))

(event `Key|Gamepad_DPad_Up`
  (params (Key :type "Key Structure"))
  ;[0.8714 0.2016 1] Input - Gun Equip + Unequip (Gunspinning) (Gamepad)
  (:`Pressed`
    (`/Game/FemaleShooter/Ver_1_3_2/FemaleShooter/Blueprint/Component/TwinGunHandler.ToggleEquipGun` (`self.TwinGunHandler`) true)))

(event `ExamineAmmo`
  (params (Item :type "/Game/FemaleShooter/Ver_1_3_2/FemaleShooter/Additional/SimpleItem/SimpleItem Object Reference"))
  ;[0 0.6445 1] Item Collector
  (bind _asammo_data (cast `/Game/FemaleShooter/Ver_1_3_2/FemaleShooter/Blueprint/Data/Ammo/AmmoData` (`/Game/FemaleShooter/Ver_1_3_2/FemaleShooter/Additional/SimpleItem/SimpleItem.ItemData` Item)))
  (`/Game/FemaleShooter/Ver_1_3_2/FemaleShooter/Blueprint/Component/TwinGunHandler.AssignAmmo` (`self.TwinGunHandler`) _asammo_data))

(event `Key|Gamepad_DPad_Right`
  (params (Key :type "Key Structure"))
  ;[0.8714 0.2016 1] Input - Right Gun Shot Only
  (:`Pressed`
    (`/Game/FemaleShooter/Ver_1_3_2/FemaleShooter/Blueprint/Component/TwinGunHandler.RightGunShotOnly` (`self.TwinGunHandler`) true :!label _label_10))
  (:`Released`
    (`/Game/FemaleShooter/Ver_1_3_2/FemaleShooter/Blueprint/Component/TwinGunHandler.RightGunShotOnly` (`self.TwinGunHandler`) false :!label _label_11)))

(event `Key|LeftAlt`
  (params (Key :type "Key Structure"))
  ;[0.3569 1 0.3843] Input - Crouch
  (:`Pressed`
    (goto _label_8))
  (:`Released`
    (goto _label_9)))

(event `Key|C`
  (params (Key :type "Key Structure"))
  ;[0.8714 0.2016 1] Input - Right Gun Shot Only
  (:`Pressed`
    (goto _label_10))
  (:`Released`
    (goto _label_11)))

(event `SetupInput_KeyPressHandler`
  ;[0.3569 1 0.3843] Input - Movement (Keyboard)
  (`/Game/FemaleShooter/Ver_1_3_2/FemaleShooter/Blueprint/Component/KeyPressHandler.Setup` (`self.KeyPressHandler`) (`|MakeMap` "W" "W" "S" "S" "D" "D" "A" "A" :!type "Key Structure" :!valuetype "Name"))
  (add `/Game/FemaleShooter/Ver_1_3_2/FemaleShooter/Blueprint/Component/KeyPressHandler.OnKeyDown` (`self.KeyPressHandler`) (delegate `OnKeyDown`)))

(event `Key|LeftControl`
  (params (Key :type "Key Structure"))
  ;[0.3569 1 0.3843] Input - Crouch
  (:`Pressed`
    (goto _label_8))
  (:`Released`
    (goto _label_9)))

(event `InputAxisKey|MouseY`
  (params (AxisValue :type "Float (single-precision)"))
  ;[0.3569 1 0.3843] Input - Camera Control
  (`/Game/FemaleShooter/Ver_1_3_2/FemaleShooter/Blueprint/Component/GunnerGirlComponent.Camera_TurnVertical` (`self.GunnerGirlComponent`) AxisValue 45.0 2.0 true))

(event `ExamineTrigger`
  (params (Item :type "/Game/FemaleShooter/Ver_1_3_2/FemaleShooter/Additional/SimpleItem/SimpleItem Object Reference"))
  (bind _itemtrigger (`/Game/FemaleShooter/Ver_1_3_2/FemaleShooter/Additional/SimpleItem/SimpleItem.ItemTrigger` Item))
  ;[0 0.6445 1] Item Collector
  (`/Engine/EditorBlueprintResources/StandardMacros.IsValid` _itemtrigger
    (:`Is Valid`
      (`/Game/FemaleShooter/Ver_1_3_2/FemaleShooter/Additional/SimpleItem/ItemTrigger.PressTrigger` _itemtrigger))))

(event `PickupFlashlight`
  (params (Item :type "/Game/FemaleShooter/Ver_1_3_2/FemaleShooter/Additional/SimpleItem/SimpleItem Object Reference"))
  ;[0 0.6445 1] Item Collector
  (`/Game/FemaleShooter/Ver_1_3_2/FemaleShooter/Blueprint/Component/GunnerGirlComponent.EquipFlashlight` (`self.GunnerGirlComponent`) true))

(event `Key|One`
  (params (Key :type "Key Structure"))
  ;[0.8714 0.2016 1] Gun Equip / Unequip (Keyboard)
  (:`Pressed`
    (`/Game/FemaleShooter/Ver_1_3_2/FemaleShooter/Blueprint/Component/TwinGunHandler.ToggleEquipGun` (`self.TwinGunHandler`) false)))

(event `Key|Gamepad_FaceButton_Right`
  (params (Key :type "Key Structure"))
  ;[0.3569 1 0.3843] Input - Roll
  (:`Pressed`
    (`/Game/FemaleShooter/Ver_1_3_2/FemaleShooter/Blueprint/Component/GunnerGirlComponent.Roll` (`self.GunnerGirlComponent`) :!label _label_12)))

(event `Key|E`
  (params (Key :type "Key Structure"))
  ;[0.3569 1 0.3843] Input - Roll
  (:`Pressed`
    (goto _label_12)))

(event `Key|Two`
  (params (Key :type "Key Structure"))
  ;[0.8714 0.2016 1] Gun Equip / Unequip (Keyboard)
  (:`Pressed`
    (`/Game/FemaleShooter/Ver_1_3_2/FemaleShooter/Blueprint/Component/TwinGunHandler.ToggleEquipGun` (`self.TwinGunHandler`) true)))

(event `PickupWeaponSet`
  (params (Item :type "/Game/FemaleShooter/Ver_1_3_2/FemaleShooter/Additional/SimpleItem/SimpleItem Object Reference"))
  ;[0 0.6445 1] Item Collector
  (bind _asequipment_set (cast `/Game/FemaleShooter/Ver_1_3_2/FemaleShooter/Blueprint/Data/Equipment/EquipmentSet` (`/Game/FemaleShooter/Ver_1_3_2/FemaleShooter/Additional/SimpleItem/SimpleItem.ItemData` Item)))
  (`/Game/FemaleShooter/Ver_1_3_2/FemaleShooter/Blueprint/Component/TwinGunHandler.LoadEquipmentSet` (`self.TwinGunHandler`) _asequipment_set true))

(event `OnKeyDown`
  (params (Key :type "Key Structure") (KeyName :type Name))
  ;[0.3569 1 0.3843] Input - Movement (Keyboard)
  (switch `name` KeyName
    (:`W`
      (`/Game/FemaleShooter/Ver_1_3_2/FemaleShooter/Blueprint/Component/GunnerGirlComponent.MoveForward` (`self.GunnerGirlComponent`) 1.0))
    (:`S`
      (`/Game/FemaleShooter/Ver_1_3_2/FemaleShooter/Blueprint/Component/GunnerGirlComponent.MoveForward` (`self.GunnerGirlComponent`) -1.0))
    (:`A`
      (`/Game/FemaleShooter/Ver_1_3_2/FemaleShooter/Blueprint/Component/GunnerGirlComponent.MoveSideward` (`self.GunnerGirlComponent`) -1.0))
    (:`D`
      (`/Game/FemaleShooter/Ver_1_3_2/FemaleShooter/Blueprint/Component/GunnerGirlComponent.MoveSideward` (`self.GunnerGirlComponent`) 1.0))))

(event `ChangeShootingPattern`
  (bind _array (`|MakeArray` "/Game/FemaleShooter/Ver_1_3_2/FemaleShooter/Blueprint/Data/ShootingPattern/Shooting_Frantic.Shooting_Frantic" "/Game/FemaleShooter/Ver_1_3_2/FemaleShooter/Blueprint/Data/ShootingPattern/Shooting_OneTwo.Shooting_OneTwo" "/Game/FemaleShooter/Ver_1_3_2/FemaleShooter/Blueprint/Data/ShootingPattern/Shooting_OneTwoThree.Shooting_OneTwoThree" "/Game/FemaleShooter/Ver_1_3_2/FemaleShooter/Blueprint/Data/ShootingPattern/Shooting_SevenShots.Shooting_SevenShots" :!type "/Game/FemaleShooter/Ver_1_3_2/FemaleShooter/Blueprint/Data/ShootingPattern/ShootingPattern Object Reference"))
  ;[0 0.6445 1] Item Collector
  (bind _output_get (set `self.ShootingPatternCount` (mod (+ (`self.ShootingPatternCount`) 1) (`KismetArrayLibrary.Array_Length` _array))))
  (`/Game/FemaleShooter/Ver_1_3_2/FemaleShooter/Blueprint/Component/TwinGunHandler.AssignShootingPattern` (`self.TwinGunHandler`) (`|GetArrayItem` _array _output_get)))

(event `Key|Gamepad_RightTrigger`
  (params (Key :type "Key Structure"))
  ;[0.8714 0.2016 1] Input - Shoot
  (:`Pressed`
    (`/Game/FemaleShooter/Ver_1_3_2/FemaleShooter/Blueprint/Component/TwinGunHandler.StartShooting` (`self.TwinGunHandler`) :!label _label_13))
  (:`Released`
    (`/Game/FemaleShooter/Ver_1_3_2/FemaleShooter/Blueprint/Component/TwinGunHandler.StopShooting` (`self.TwinGunHandler`) :!label _label_14)))

(event `Key|SpaceBar`
  (params (Key :type "Key Structure"))
  ;[0.3564 1 0.3864] Input - Jump/Double Jump/Somersault
  (:`Pressed`
    (`/Game/FemaleShooter/Ver_1_3_2/FemaleShooter/Blueprint/Component/GunnerGirlComponent.TriggerJump` (`self.GunnerGirlComponent`) true :!label _label_15))
  (:`Released`
    (`/Game/FemaleShooter/Ver_1_3_2/FemaleShooter/Blueprint/Component/GunnerGirlComponent.ClearJump` (`self.GunnerGirlComponent`) :!label _label_16)))

(event `Key|LeftMouseButton`
  (params (Key :type "Key Structure"))
  ;[0.8714 0.2016 1] Input - Shoot
  (:`Pressed`
    (goto _label_13))
  (:`Released`
    (goto _label_14)))

(event `Key|Gamepad_FaceButton_Bottom`
  (params (Key :type "Key Structure"))
  ;[0.3564 1 0.3864] Input - Jump/Double Jump/Somersault
  (:`Pressed`
    (goto _label_15))
  (:`Released`
    (goto _label_16)))

(event `Key|Gamepad_DPad_Down`
  (params (Key :type "Key Structure"))
  ;[0.3564 1 0.3864] Input - Toggle Flashlight
  (:`Pressed`
    (`/Game/FemaleShooter/Ver_1_3_2/FemaleShooter/Blueprint/Component/GunnerGirlComponent.ToggleFlashLight` (`self.GunnerGirlComponent`) :!label _label_17)))

(event `Key|Q`
  (params (Key :type "Key Structure"))
  ;[0.3564 1 0.3864] Input - Toggle Flashlight
  (:`Pressed`
    (goto _label_17)))

(fn `UserConstructionScript`)